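; Test actor that highlights its mesh color on overlap and shows a bounding box while the right trigger is pressed.
; Construction creates a dynamic material, caches its floor color and randomizes glow color.
; When selection is enabled, authority-side Tick interpolates NewColor between highlight and original colors, and its OnRep applies it to the material.
; BeginPlay fits the box to actor bounds, and trigger events toggle its visibility, counting displays.
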(event Custom|ServerSetColor
  (params (Color :type Linear%20Color%20Structure))
  (Variables|Default|SetNewColor Color))

(event EventBeginPlay
  (bind (_origin _boxextent) (Collision|GetActorBounds false))
  (Transformation|SetWorldTransform (Variables|Default|GetBoundingBox) (Math|Transform|MakeTransform _origin "0, 0, 0" (/ _boxextent 2e+01)) false false))

(event EventRTriggerReleased
  (params (Other%20Data :type Object%20Object%20Reference))
  (bind _boundingbox (Variables|Default|GetBoundingBox))
  ;[1 1 1] If a controller is pointing at this object and the trigger is pressed, activate/deactivate the bounding box
  (Development|SetHiddeninGame _boundingbox true true)
  (Rendering|SetActorHiddenInGame (Variables|/Script/Engine.ChildActorComponent|GetChildActor _boundingbox) true))

(event EventRTriggerPressed
  (params (Other%20Data :type Object%20Object%20Reference))
  (bind _boundingbox (Variables|Default|GetBoundingBox))
  ;[1 1 1] If a controller is pointing at this object and the trigger is pressed, activate/deactivate the bounding box
  (Development|SetHiddeninGame _boundingbox false true)
  (Rendering|SetActorHiddenInGame (Variables|/Script/Engine.ChildActorComponent|GetChildActor _boundingbox) false)
  (Math|Integer|IncrementInt (Variables|Default|GetBBTimesDisplayed)))

(event EventTick
  (params (DeltaSeconds :type Float%20%28single-precision%29))
  (Networking|SwitchHasAuthority
    (:Authority
      ;[1 1 1] If selected, animate color highlighting
      (if (Variables|Default|GetIsSelectionEnabled)
        (bind _returnvalue (Rendering|Material|GetVectorParameterValue (Variables|Default|GetMaterial) "FloorColor" :!class /Script/Engine.MaterialInstanceDynamic))
        (Variables|Default|SetCurrentColor _returnvalue)
        (if (Variables|Default|GetIsOverlapping)
          (Variables|Default|SetNewColor (Class|KismetMathLibrary|CInterpto (Variables|Default|GetCurrentColor) (Variables|Default|GetHighlightColor) DeltaSeconds 2.0))
          (else
            (Variables|Default|SetNewColor (Class|KismetMathLibrary|CInterpto (Variables|Default|GetCurrentColor) (Variables|Default|GetFloorColor) DeltaSeconds 2.0))))))))

(event Collision|EventActorEndOverlap
  (params (OtherActor :type Actor%20Object%20Reference))
  (Variables|Default|SetIsOverlapping false))

(event Collision|EventActorBeginOverlap
  (params (OtherActor :type Actor%20Object%20Reference))
  (Variables|Default|SetIsOverlapping true))

(fn ConstructionScript
  (bind _targetmesh (Variables|Default|GetTargetMesh))
  (Utilities|FlowControl|Sequence
    (:then_0
      (bind _returnvalue (Rendering|Material|CreateDynamicMaterialInstance (Utilities|Array|Get(acopy) (Rendering|Material|GetMaterials _targetmesh)) :!class /Script/Engine.KismetMaterialLibrary))
      (bind _output_get (Variables|Default|SetMaterial _returnvalue))
      (Rendering|Material|SetMaterial _targetmesh 0 _output_get)
      (Utilities|FlowControl|Sequence
        (:then_0
          (bind _returnvalue_2 (Rendering|Material|GetVectorParameterValue _output_get "FloorColor" :!class /Script/Engine.MaterialInstanceDynamic))
          (Variables|Default|SetFloorColor _returnvalue_2))
        (:then_1
          (Rendering|Material|SetVectorParameterValue _output_get "GlowColor" (Utilities|Struct|MakeLinearColor (Math|Random|RandomFloatinRange 0.0 1.0) (Math|Random|RandomFloatinRange 0.0 1.0) (Math|Random|RandomFloatinRange 0.0 1.0) 1.0) :!class /Script/Engine.MaterialInstanceDynamic))))))

(fn OnRepNewColor
  (Rendering|Material|SetVectorParameterValue (Variables|Default|GetMaterial) "FloorColor" (Variables|Default|GetNewColor) :!class /Script/Engine.MaterialInstanceDynamic))