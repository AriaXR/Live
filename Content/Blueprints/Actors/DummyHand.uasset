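; DummyHand is a scripted hand actor that grabs and throws the first ThrowableActor tagged "Animation".
; Each Tick, the Grip flag switches the RightHand_AnimBP grip state and toggles the object's physics.
; ApplyForce runs a while loop adding a fixed force until accumulated delta time reaches ForceDuration, all within one tick.
; The hand then hides, and after a delay every ThrowableActor calls ReturnState.
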(event EventBeginPlay)

(event Collision|EventActorBeginOverlap
  (params (OtherActor :type Actor%20Object%20Reference)))

(event EventTick
  (params (DeltaSeconds :type Float%20%28single-precision%29))
  (bind _asright_hand_anim_bp (Utilities|Casting|CastToRightHand_AnimBP (Components|SkeletalMesh|GetAnimInstance (Variables|Default|GetHand))))
  (Utilities|FlowControl|Sequence
    (:then_0
      (if (Variables|Default|GetbGrip)
        (if (Utilities|Enum|Equal(Enum) (Variables|/Game/Assets/Mannequin/Animations/RightHand_AnimBP.RightHand_AnimBP_C|GetGripState _asright_hand_anim_bp) "NewEnumerator0")
          (Variables|/Game/Assets/Mannequin/Animations/RightHand_AnimBP.RightHand_AnimBP_C|SetGripState _asright_hand_anim_bp "NewEnumerator2")
          (bind _outactors (Actor|GetAllActorswithTag "Animation"))
          (Variables|Default|SetThrowable (.AsThrowable%20Actor (Utilities|Casting|CastToThrowableActor (Utilities|Array|Get(acopy) _outactors))))
          (Physics|SetSimulatePhysics (Variables|/Game/Blueprints/Actors/ThrowableActor.ThrowableActor_C|GetTargetMesh (.AsThrowable%20Actor (Utilities|Casting|CastToThrowableActor (Utilities|Array|Get(acopy) _outactors)))) false))
        (elif (Utilities|Enum|Equal(Enum) (Variables|/Game/Assets/Mannequin/Animations/RightHand_AnimBP.RightHand_AnimBP_C|GetGripState _asright_hand_anim_bp) "NewEnumerator2")
          (Variables|/Game/Assets/Mannequin/Animations/RightHand_AnimBP.RightHand_AnimBP_C|SetGripState _asright_hand_anim_bp "NewEnumerator0")
          (Physics|SetSimulatePhysics (Variables|/Game/Blueprints/Actors/ThrowableActor.ThrowableActor_C|GetTargetMesh (.AsThrowable%20Actor (Utilities|Casting|CastToThrowableActor (Variables|Default|GetThrowable)))) true))))
    (:then_1
      (while (and (Variables|Default|GetbApplyForce) (< (Variables|Default|GetElapsed) (Variables|Default|GetForceDuration)))
        (Physics|AddForce (Variables|/Game/Blueprints/Actors/ThrowableActor.ThrowableActor_C|GetTargetMesh (.AsThrowable%20Actor (Utilities|Casting|CastToThrowableActor (Variables|Default|GetThrowable)))) "0.000000,-1000.000000,200.000000" "None" false)
        (Variables|Default|SetElapsed (+ (Variables|Default|GetElapsed) DeltaSeconds))))
    (:then_2
      (if (>= (Variables|Default|GetElapsed) (Variables|Default|GetForceDuration))
        (Utilities|FlowControl|Sequence
          (:then_0
            (Variables|Default|SetbApplyForce false)
            (Variables|Default|SetElapsed 0.0))
          (:then_1
            (Utilities|FlowControl|Delay 3.0)
            (bind _outactors_2 (Actor|GetAllActorsOfClass "/Game/Blueprints/Actors/ThrowableActor.ThrowableActor_C"))
            (for _array_element _outactors_2
              (Default|ReturnState _array_element)))
          (:then_2
            (Rendering|SetActorHiddenInGame true)))))))

(fn ConstructionScript)