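; Actor that fakes a radial shape menu, automatically cycling its selection through Cube, Pyramid and Sphere while Animate is on.
; On Tick, an elapsed timer and a Changed flag advance the selection once every two seconds.
; Each step moves a SpotLight to an offset from the selected shape component and passes the shape name to the ContextualMenuActor through ChangeShape.
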(event EventBeginPlay)

(event Collision|EventActorBeginOverlap
  (params (OtherActor :type Actor%20Object%20Reference)))

(event EventTick
  (params (DeltaSeconds :type Float%20%28single-precision%29))
  (|CallParentFunction DeltaSeconds)
  (if (Variables|Default|GetbAnimate)
    (Utilities|FlowControl|Sequence
      (:then_0
        (Variables|Default|SetElapsed (+ (Variables|Default|GetElapsed) DeltaSeconds)))
      (:then_1
        (if (not (Variables|Default|GetbChanged))
          (Utilities|FlowControl|Sequence
            (:then_0
              (CallFunction|SelectShape (Variables|Default|GetSelectedShape))
              (bind _actor (CallFunction|GetActorOfType "/Game/Blueprints/Actors/ContextualMenuActor.ContextualMenuActor_C"))
              (switch int (Variables|Default|GetSelectedShape)
                (:0
                  (Default|ChangeShape (.AsContextual%20Menu%20Actor (Utilities|Casting|CastToContextualMenuActor _actor)) "Cube"))
                (:1
                  (Default|ChangeShape (.AsContextual%20Menu%20Actor (Utilities|Casting|CastToContextualMenuActor _actor)) "Pyramid"))
                (:2
                  (Default|ChangeShape (.AsContextual%20Menu%20Actor (Utilities|Casting|CastToContextualMenuActor _actor)) "Sphere"))))
            (:then_1
              (bind _result (Math|Integer|IncrementInt (Variables|Default|GetSelectedShape))
                (:%20%20
                  (Variables|Default|SetSelectedShape (Math|Integer|%(Integer) _result 3))
                  (Variables|Default|SetbChanged true)))))))
      (:then_2
        (if (>= (Variables|Default|GetElapsed) 2.0)
          (Variables|Default|SetElapsed 0.0)
          (Variables|Default|SetbChanged false))))))

(fn ConstructionScript
  (|CallParentFunction))

(fn SelectShape
  (params (Selection :type Integer))
  (switch int Selection
    (:0
      (Variables|Default|SetSelectedActor (Variables|Default|GetCube)))
    (:1
      (Variables|Default|SetSelectedActor (Variables|Default|GetPyramid)))
    (:2
      (Variables|Default|SetSelectedActor (Variables|Default|GetSphere))))
  (Transformation|SetRelativeLocation (Variables|Default|GetSpotLight) (+ (Variables|/Script/Engine.SceneComponent|GetRelativeLocation (Variables|Default|GetSelectedActor)) "-100.000000, 0, 0") false false))