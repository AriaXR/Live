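; BrickActor is a physics-simulated brick that can be picked up and dropped.
; BeginPlay applies its configured mesh and material, enables physics and stops characters stepping up on it.
; Pickup disables physics and attaches the root to a given component, keeping its world transform.
; Drop re-enables physics, detaches the actor in place and sets InteractedWith to true.
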(event EventBeginPlay
  (bind _staticmesh (Variables|Default|GetStaticMesh))
  (bind _staticmesh_2 (Variables|Default|GetStaticMesh))
  (Components|StaticMesh|SetStaticMesh _staticmesh_2 (Variables|Default|GetMesh))
  (Rendering|Material|SetMaterial _staticmesh_2 0 (Variables|Default|GetMaterial))
  (Physics|SetSimulatePhysics _staticmesh true)
  (Variables|/Script/Engine.PrimitiveComponent|SetCanCharacterStepUpOn _staticmesh "ECB_No"))

(event Collision|EventActorBeginOverlap
  (params (OtherActor :type Actor%20Object%20Reference)))

(event EventPickup
  (params (AttachTo :type Scene%20Component%20Object%20Reference))
  ;[1 1 1] Pickup & Drop
  (Physics|SetSimulatePhysics (Variables|Default|GetStaticMesh) false)
  (Transformation|AttachComponentToComponent (VehicleSound|GetRootComponent) AttachTo "None" "KeepWorld" "KeepWorld" "KeepWorld" false))

(event EventTick
  (params (DeltaSeconds :type Float%20%28single-precision%29)))

(event EventDrop
  ;[1 1 1] Pickup & Drop
  (Physics|SetSimulatePhysics (Variables|Default|GetStaticMesh) true)
  (Transformation|DetachFromActor "KeepWorld" "KeepWorld" "KeepWorld")
  (Variables|Default|SetbInteractedWith true))

(fn ConstructionScript)