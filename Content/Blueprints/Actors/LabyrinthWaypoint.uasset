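; Labyrinth waypoint actor that marks a step on a route and guides the player onward to the next waypoint.
; While active, it spins its scene component every tick until reached.
; Overlap by a Teleporter or WorldInMiniature actor points the player pawn's arrow at NextWaypoint through IPawn, stops the spin, flags it reached and turns both meshes green.
; Reset reactivates it, clears the reached state and restores the orange material.
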(event Custom|Reset
  (Variables|Default|SetbActive true)
  (Variables|Default|SetbStopSpinning false)
  (Variables|Default|SetbIsReached false)
  (Rendering|Material|SetMaterial (Variables|Default|GetStaticMesh1) 0 "/Game/Assets/Abstract/Materials/M_Orange_Shiny.M_Orange_Shiny"))

(event EventBeginPlay)

(event Collision|EventActorBeginOverlap
  (params (OtherActor :type Actor%20Object%20Reference))
  (Utilities|Casting|CastToTeleporter OtherActor
    (:then
      _)
    (:CastFailed
      (Utilities|Casting|CastToWorldInMiniature OtherActor)))
  (if (Variables|Default|GetbActive)
    (bind _asipawn (Utilities|Casting|CastToIPawn (Game|Player|GetPlayerPawn 0)))
    (bind _arrow (Default|GetArrow _asipawn))
    (Default|PointTowards _arrow (Variables|Default|GetNextWaypoint))
    (Variables|Default|SetbStopSpinning true)
    (Variables|Default|SetbIsReached true)
    (Rendering|Material|SetMaterial (Variables|Default|GetStaticMesh1) 0 "/Game/Assets/Abstract/Materials/Green.Green")))

(event EventTick
  (params (DeltaSeconds :type Float%20%28single-precision%29))
  (if (Variables|Default|GetbActive)
    (if (not (Variables|Default|GetbStopSpinning))
      (Transformation|AddRelativeRotation (Variables|Default|GetScene) (Math|Rotator|MakeRotator 0.0 0.0 (* DeltaSeconds 1.8e+02)) false false))))

(fn ConstructionScript)