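; Stand-in UI controller actor that simulates pointer input on world-space widgets through a WidgetInteraction component.
; Tick syncs debug display to Activate, turns the Click flag into timed left-button press/release and, with Animate set, periodically cycles ContextualMenuActor through three colors.
; Hover changes track the current widget and send PointerLeave through IWidget, while RaiseClick releases the pointer and notifies the hovered IControllerReactive owner.
; Construction gives the controller mesh a dynamic material.
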(event OnHoveredWidgetChanged(WidgetInteraction)
  (params (WidgetComponent :type Widget%20Component%20Object%20Reference) (PreviousWidgetComponent :type Widget%20Component%20Object%20Reference))
  ;[1 1 1] Forward pointer enter/leave to widget
  (Utilities|IsValid WidgetComponent
    (:Is%20Valid
      (if (!= WidgetComponent PreviousWidgetComponent)
        (Utilities|IsValid (Variables|Default|GetCurrentWidget)
          (:Is%20Valid
            (Utilities|IsValid (Utilities|ToObject(Interface) (.AsIWidget (Utilities|Casting|CastToIWidget (Variables|Default|GetCurrentWidget))))
              (:Is%20Valid
                (Default|PointerLeave (.AsIWidget (Utilities|Casting|CastToIWidget (Variables|Default|GetCurrentWidget)))))))
          (:Is%20Not%20Valid
            _))
        (Variables|Default|SetPreviousWidget (Variables|Default|GetCurrentWidget))
        (Variables|Default|SetCurrentWidget (UserInterface|GetUserWidgetObject WidgetComponent))
        (Utilities|IsValid (Utilities|ToObject(Interface) (.AsIWidget (Utilities|Casting|CastToIWidget (Variables|Default|GetCurrentWidget)))))))))

(event Custom|RaiseClick
  (Class|WidgetInteractionComponent|ReleasePointerKey (Variables|Default|GetWidgetInteraction) "LeftMouseButton")
  (bind _asicontroller_reactive (Utilities|Casting|CastToIControllerReactive (Components|GetOwner (Class|WidgetInteractionComponent|GetHoveredWidgetComponent (Variables|Default|GetWidgetInteraction)))))
  (Default|RTriggerReleased _asicontroller_reactive (Variables|Default|GetCurrentWidget)))

(event EventBeginPlay)

(event Collision|EventActorBeginOverlap
  (params (OtherActor :type Actor%20Object%20Reference)))

(event EventTick
  (params (DeltaSeconds :type Float%20%28single-precision%29))
  (bind _widgetinteraction (Variables|Default|GetWidgetInteraction))
  (Utilities|FlowControl|Sequence
    (:then_0
      (Variables|/Script/UMG.WidgetInteractionComponent|SetbShowDebug (Variables|Default|GetWidgetInteraction) (Variables|Default|GetbActivate)))
    (:then_1
      (if (Variables|Default|GetbClick)
        (Utilities|FlowControl|DoOnce false :!label _label
          (:Completed
            (Class|WidgetInteractionComponent|PressPointerKey _widgetinteraction "LeftMouseButton")
            (Utilities|FlowControl|Delay 0.3)
            (Class|WidgetInteractionComponent|ReleasePointerKey _widgetinteraction "LeftMouseButton")
            (goto _label Reset)))))
    (:then_2
      (if (Variables|Default|GetbAnimate)
        (Utilities|FlowControl|Sequence
          (:then_0
            (Variables|Default|SetElapsed (+ (Variables|Default|GetElapsed) DeltaSeconds)))
          (:then_1
            (if (not (Variables|Default|GetbChanged))
              (Utilities|FlowControl|Sequence
                (:then_0
                  (bind _actor (CallFunction|GetActorOfType "/Game/Blueprints/Actors/ContextualMenuActor.ContextualMenuActor_C"))
                  (switch int (Variables|Default|GetSelectedColor)
                    (:0
                      (Default|ChangeColor (.AsContextual%20Menu%20Actor (Utilities|Casting|CastToContextualMenuActor _actor)) "Blue"))
                    (:1
                      (Default|ChangeColor (.AsContextual%20Menu%20Actor (Utilities|Casting|CastToContextualMenuActor _actor)) "Red"))
                    (:2
                      (Default|ChangeColor (.AsContextual%20Menu%20Actor (Utilities|Casting|CastToContextualMenuActor _actor)) "Green"))))
                (:then_1
                  (bind _result (Math|Integer|IncrementInt (Variables|Default|GetSelectedColor))
                    (:%20%20
                      (Variables|Default|SetSelectedColor (Math|Integer|%(Integer) _result 3))
                      (Variables|Default|SetbChanged true)))))))
          (:then_2
            (if (>= (Variables|Default|GetElapsed) 3.0)
              (Variables|Default|SetElapsed 0.0)
              (Variables|Default|SetbChanged false))))))))

(fn ConstructionScript
  (bind _returnvalue (Rendering|Material|CreateDynamicMaterialInstance (Rendering|Material|GetMaterial (Variables|Default|GetController) 0) :!class /Script/Engine.KismetMaterialLibrary))
  (bind _output_get (Variables|Default|SetControllerMaterial _returnvalue))
  (Rendering|Material|SetMaterial (Variables|Default|GetController) 0 _output_get))