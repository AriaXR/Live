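; Actor with a changeable mesh and a contextual menu of Red, Green and Blue widget buttons for recoloring it.
; While the menu is active, controller overlap reveals the buttons and enables their UI collision; leaving hides them after a delay unless re-entered.
; Trigger release passes the button's label to ChangeColor, which sets a parameter on a dynamic material created at construction.
; ChangeShape separately swaps between cube, sphere and pyramid meshes.
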(event Custom|SetMenuVisibility
  (params (Hidden :type Boolean))
  (Development|SetHiddeninGame (Variables|Default|GetWidgetBlue) Hidden false))

(event Custom|ChangeColor
  (params (ColorName :type String))
  ;[1 1 1] Change Color
  (switch string ColorName
    (:Red
      (Variables|Default|SetColor (Utilities|Struct|MakeLinearColor 0.6 0.0 0.0 1.0)))
    (:Green
      (Variables|Default|SetColor (Utilities|Struct|MakeLinearColor 0.0 0.6 0.0 1.0)))
    (:Blue
      (Variables|Default|SetColor (Utilities|Struct|MakeLinearColor 0.0 0.0 0.6 1.0)))
    (:Black
      (Variables|Default|SetColor "")))
  (Rendering|Material|SetVectorParameterValue (Variables|Default|GetMaterial) "FloorColor" (Variables|Default|GetColor) :!class /Script/Engine.MaterialInstanceDynamic))

(event Custom|HideMenu
  (if (Variables|Default|GetbShouldHide)
    (CallFunction|SetMenuVisibility true)
    (Collision|SetCollisionProfileName (Variables|Default|GetWidgetBlue) "NoCollision" :!class /Script/Engine.PrimitiveComponent)))

(event Custom|ChangeShape
  (params (Shape%20Name :type String))
  (bind _staticmesh (Variables|Default|GetStaticMesh))
  ;[1 1 1] Change Shape
  (switch string Shape%20Name
    (:Cube
      (Variables|Default|SetMesh "/Game/Assets/Abstract/SM_Cube_01.SM_Cube_01")
      (Variables|Default|SetMeshTransform (Math|Transform|MakeTransform "0, 0, 0")))
    (:Sphere
      (Variables|Default|SetMesh "/Game/Assets/Abstract/SM_Ball_01.SM_Ball_01")
      (Variables|Default|SetMeshTransform (Math|Transform|MakeTransform "0, 0,3.000000" "0, 0, 0" "0.400000,0.400000,0.400000")))
    (:Pyramid
      (Variables|Default|SetMesh "/Game/Assets/Abstract/SM_Pyramid_01.SM_Pyramid_01")
      (Variables|Default|SetMeshTransform (Math|Transform|MakeTransform "0, 0,-5.000000" "0, 0, 0" "0.500000,0.500000,0.500000"))))
  (Components|StaticMesh|SetStaticMesh _staticmesh (Variables|Default|GetMesh))
  (Transformation|SetRelativeTransform _staticmesh (Variables|Default|GetMeshTransform) false false))

(event Custom|HideMenuAfter
  (params (Wait%20Delay :type Float%20%28single-precision%29))
  (Variables|Default|SetbShouldHide true)
  (Utilities|Time|SetTimerbyEvent (delegate Custom|HideMenu) Wait%20Delay))

(event EventBeginPlay
  (Utilities|FlowControl|Sequence
    (:then_0
      (Utilities|SetTextLabel (Variables|Default|GetWidgetGreen) "Green" 80))
    (:then_1
      (Utilities|SetTextLabel (Variables|Default|GetWidgetRed) "Red" 80))
    (:then_2
      (Utilities|SetTextLabel (Variables|Default|GetWidgetBlue) "Blue" 80))))

(event EventControllerBeginOverlap
  (if (Variables|Default|GetbMenuActive)
    (CallFunction|SetMenuVisibility false)
    (Collision|SetCollisionProfileName (Variables|Default|GetWidgetBlue) "UI" :!class /Script/Engine.PrimitiveComponent)
    (Variables|Default|SetbShouldHide false)))

(event EventControllerEndOverlap
  (if (Variables|Default|GetbMenuActive)
    (CallFunction|HideMenuAfter 2.0)))

(event EventTick
  (params (DeltaSeconds :type Float%20%28single-precision%29)))

(event EventRTriggerReleased
  (params (Other%20Data :type Object%20Object%20Reference))
  (bind _asradial_button (Utilities|Casting|CastToRadialButton Other%20Data))
  (Utilities|IsValid _asradial_button
    (:Is%20Valid
      (CallFunction|ChangeColor (Utilities|String|ToString(Text) (Class|TextBlock|GetText (Variables|/Game/Blueprints/UserInterface/RadialButton.RadialButton_C|GetTextBlock_Label _asradial_button))))
      (Variables|Default|SetbHasBeenUsed true))))

(fn ConstructionScript
  (bind _staticmesh (Variables|Default|GetStaticMesh))
  (bind _returnvalue (Rendering|Material|CreateDynamicMaterialInstance (Utilities|Array|Get(acopy) (Rendering|Material|GetMaterials _staticmesh)) :!class /Script/Engine.KismetMaterialLibrary))
  (bind _output_get (Variables|Default|SetMaterial _returnvalue))
  (Rendering|Material|SetMaterial _staticmesh 0 _output_get))