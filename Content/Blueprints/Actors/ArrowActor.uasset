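; Arrow actor that stores a target via PointTowards and sets its scene rotation each Tick from RotateTowardsTarget while the target is valid.
; RotateTowardsTarget holds a yaw-only look-at calculation toward the target, though those nodes appear unconnected to any output.
; CheckRotation separately tests whether the arrow's forward is within a fixed angle of the live pawn camera's horizontally projected forward; nothing here calls it.
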(event Custom|PointTowards
  (params (Target%20Actor :type Actor%20Object%20Reference))
  (Variables|Default|SetTarget Target%20Actor))

(event EventBeginPlay)

(event Collision|EventActorBeginOverlap
  (params (OtherActor :type Actor%20Object%20Reference)))

(event EventTick
  (params (DeltaSeconds :type Float%20%28single-precision%29))
  (bind _returnvalue (|RotateTowardsTarget))
  (Utilities|IsValid (Variables|Default|GetTarget)
    (:Is%20Valid
      (Transformation|SetWorldRotation (Variables|Default|GetScene) _returnvalue false false)
      (Variables|Default|SetCurrentRotation _returnvalue))))

(fn ConstructionScript)

(fn CheckRotation
  (bind _camera (Default|GetCamera (Utilities|LivePawn)))
  (bind _angle (CallFunction|AngleBetweenVectors (Math|Vector|GetForwardVector (Variables|Default|GetScene)) (Math|Vector|ProjectVectorontoPlane (Math|Vector|GetForwardVector _camera) "0, 0,1.000000")))
  (return (<= (Math|Float|Absolute(Float) (Math|Trig|RadiansToDegrees _angle)) 3e+01)))