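; Dummy hand actor that holds a 2x2 brick and plate, posing the hand and releasing the pieces in response to flags.
; Each tick, the Grip flag toggles the GripState of the hand's RightHand_AnimBP between two states.
; The DropBrick and DropPlate flags each enable physics simulation on their piece once, through a DoOnce.
; Nothing in this Blueprint sets the flags.
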(event EventBeginPlay)

(event Collision|EventActorBeginOverlap
  (params (OtherActor :type Actor%20Object%20Reference)))

(event EventTick
  (params (DeltaSeconds :type Float%20%28single-precision%29))
  (bind _asright_hand_anim_bp (Utilities|Casting|CastToRightHand_AnimBP (Components|SkeletalMesh|GetAnimInstance (Variables|Default|GetHand))))
  (Utilities|FlowControl|Sequence
    (:then_0
      (if (Variables|Default|GetbGrip)
        (if (Utilities|Enum|Equal(Enum) (Variables|/Game/Assets/Mannequin/Animations/RightHand_AnimBP.RightHand_AnimBP_C|GetGripState _asright_hand_anim_bp) "NewEnumerator0")
          (Variables|/Game/Assets/Mannequin/Animations/RightHand_AnimBP.RightHand_AnimBP_C|SetGripState _asright_hand_anim_bp "NewEnumerator2"))
        (elif (Utilities|Enum|Equal(Enum) (Variables|/Game/Assets/Mannequin/Animations/RightHand_AnimBP.RightHand_AnimBP_C|GetGripState _asright_hand_anim_bp) "NewEnumerator2")
          (Variables|/Game/Assets/Mannequin/Animations/RightHand_AnimBP.RightHand_AnimBP_C|SetGripState _asright_hand_anim_bp "NewEnumerator0"))))
    (:then_1
      (if (Variables|Default|GetbDropBrick)
        (Utilities|FlowControl|DoOnce false
          (:Completed
            (Physics|SetSimulatePhysics (Variables|Default|GetBrick2x2) true)))))
    (:then_2
      (if (Variables|Default|GetbDropPlate)
        (Utilities|FlowControl|DoOnce false
          (:Completed
            (Physics|SetSimulatePhysics (Variables|Default|GetPlate2x2) true)))))))

(fn ConstructionScript)