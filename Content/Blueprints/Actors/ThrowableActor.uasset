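; Throwable prop that floats around, can be picked up and dropped, and returns to its original transform after a drop if tagged "Throwables".
; It spawns near the "indicator" actor, and events set a state (ToStart, Wander, Return, MoveTo) that server-side Tick runs as timed transform lerps.
; Physics is off while moving or held; MoveTo hides the actor on arrival.
; A dynamic material gets a random glow, and an OnRep updates its floor color.
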(event Custom|RandomState
  ;[1 1 1] Move to random location
  (Variables|Default|SetDuration 5.0)
  (Variables|Default|SetState "ToStart")
  (Variables|Default|SetElapsed 0.0)
  (Variables|Default|SetbIsMoving true)
  (Physics|SetSimulatePhysics (Variables|Default|GetTargetMesh) false))

(event Custom|MoveTo
  (params (Start :type Transform) (Target :type Transform))
  (CallFunction|MoveTowards self (Variables|Default|GetElapsed) (Variables|Default|GetDuration) Start Target))

(event Custom|RandomWanderPoint
  (bind _returnvalue (Transformation|GetActorTransform))
  (bind (_location _rotation _scale) (Math|Transform|BreakTransform _returnvalue))
  ;[1 1 1] Get a Random wander location
  (Variables|Default|SetInitialTransform _returnvalue)
  (Variables|Default|SetTargetTransform (Math|Transform|MakeTransform (Math|Random|RandomPointinBoundingBox _location (Math|Vector|MakeVector 1e+01 1e+01 1e+01)) (* (Math|Random|RandomRotator true) 0.25) _scale)))

(event Custom|WanderState
  ;[1 1 1] Wander
  (Utilities|FlowControl|Sequence
    (:then_0
      (Variables|Default|SetInitialTransform (Transformation|GetActorTransform)))
    (:then_1
      (Variables|Default|SetDuration 1.0))
    (:then_2
      (Variables|Default|SetState "Wander"))
    (:then_3
      ;[1 1 1] Move to random location
      (Variables|Default|SetElapsed 0.0)
      (Variables|Default|SetbIsMoving true)
      (Physics|SetSimulatePhysics (Variables|Default|GetTargetMesh) false))))

(event Custom|ReturnState
  ;[1 1 1] Return to original locations
  (Utilities|FlowControl|Sequence
    (:then_0
      (Variables|Default|SetInitialTransform (Transformation|GetActorTransform)))
    (:then_1
      (Variables|Default|SetDuration 2.0))
    (:then_2
      (Variables|Default|SetState "Return"))
    (:then_3
      ;[1 1 1] Move to random location
      (Variables|Default|SetElapsed 0.0)
      (Variables|Default|SetbIsMoving true)
      (Physics|SetSimulatePhysics (Variables|Default|GetTargetMesh) false))))

(event Custom|MoveToState
  (params (Target :type Transform) (Duration :type Float%20%28single-precision%29))
  (Utilities|FlowControl|Sequence
    (:then_0
      (Variables|Default|SetInitialTransform (Transformation|GetActorTransform))
      (Variables|Default|SetTargetTransform Target))
    (:then_1
      (Variables|Default|SetDuration Duration))
    (:then_2
      (Variables|Default|SetState "MoveTo"))
    (:then_3
      ;[1 1 1] Move to random location
      (Variables|Default|SetElapsed 0.0)
      (Variables|Default|SetbIsMoving true)
      (Physics|SetSimulatePhysics (Variables|Default|GetTargetMesh) false))))

(event EventBeginPlay
  (bind _outactors (Actor|GetAllActorswithTag "indicator"))
  (Transformation|SetActorLocation (Math|Random|RandomPointinBoundingBox (+ (Transformation|GetActorLocation (Utilities|Array|Get(acopy) _outactors)) "0, 0,200.000000") (Math|Vector|MakeVector 1e+02 25.0 25.0)) false false)
  (Variables|Default|SetInitialTransform (Transformation|GetActorTransform))
  (Variables|Default|SetTargetTransform (Math|Transform|MakeTransform (Math|Random|RandomPointinBoundingBox (Transformation|GetActorLocation (Utilities|Array|Get(acopy) _outactors)) (Math|Vector|MakeVector 1e+02 1e+02 1e+02)) (Math|Random|RandomRotator true) (Transformation|GetActorScale3D))))

(event EventPickup
  (params (AttachTo :type Scene%20Component%20Object%20Reference))
  ;[1 1 1] Pickup & Drop
  (Physics|SetSimulatePhysics (Variables|Default|GetTargetMesh) false)
  (Transformation|AttachComponentToComponent (VehicleSound|GetRootComponent) AttachTo "None" "KeepWorld" "KeepWorld" "KeepWorld" false)
  (Variables|Default|SetbInteractedWith true))

(event EventTick
  (params (DeltaSeconds :type Float%20%28single-precision%29))
  (bind _returnvalue (Transformation|GetActorLocation))
  (bind (_x _y _z) (Math|Vector|BreakVector _returnvalue))
  (Networking|SwitchHasAuthority
    (:Authority
      ;[1 1 1] If "Reset targets" is invoked, make object move towards their original place
      (if (Variables|Default|GetbIsMoving)
        (Utilities|FlowControl|Sequence
          (:then_0
            (switch string (Variables|Default|GetState)
              (:ToStart
                (Utilities|FlowControl|Sequence
                  (:then_0
                    (CallFunction|Moveto (Variables|Default|GetInitialTransform) (Variables|Default|GetTargetTransform) :!label _label))
                  (:then_1
                    (if (>= (Variables|Default|GetElapsed) (Variables|Default|GetDuration))
                      (CallFunction|WanderState)
                      (CallFunction|RandomWanderPoint)))))
              (:Wander
                (CallFunction|Moveto (Variables|Default|GetInitialTransform) (Variables|Default|GetTargetTransform))
                (if (> (Variables|Default|GetElapsed) (Variables|Default|GetDuration))
                  (CallFunction|RandomWanderPoint)
                  (Variables|Default|SetElapsed 0.0)))
              (:Return
                (CallFunction|Moveto (Variables|Default|GetInitialTransform) (Variables|Default|GetOriginalTransform))
                (if (> (Variables|Default|GetElapsed) (Variables|Default|GetDuration))
                  (Variables|Default|SetbIsMoving false)
                  (Utilities|FlowControl|Delay 1.0)
                  (Physics|SetSimulatePhysics (Variables|Default|GetTargetMesh) true)))
              (:MoveTo
                (Utilities|FlowControl|Sequence
                  (:then_0
                    (goto _label))
                  (:then_1
                    (if (> (Variables|Default|GetElapsed) (Variables|Default|GetDuration))
                      (Rendering|SetActorHiddenInGame true)))))))
          (:then_1
            (Variables|Default|SetElapsed (+ DeltaSeconds (Variables|Default|GetElapsed))))
          (:then_2
            (Transformation|SetActorLocation (Math|Vector|MakeVector _x _y (Math|Float|Clamp(Float) _z 12.5 1e+04)) false false)))))))

(event EventDrop
  ;[1 1 1] Pickup & Drop
  (Physics|SetSimulatePhysics (Variables|Default|GetTargetMesh) true)
  (Transformation|DetachFromActor "KeepWorld" "KeepWorld" "KeepWorld")
  (if (Actor|ActorHasTag "Throwables")
    (Utilities|FlowControl|Delay 3.0)
    (CallFunction|ReturnState)))

(fn ConstructionScript
  (bind _targetmesh (Variables|Default|GetTargetMesh))
  (Utilities|FlowControl|Sequence
    (:then_0
      (bind _returnvalue (Rendering|Material|CreateDynamicMaterialInstance (Utilities|Array|Get(acopy) (Rendering|Material|GetMaterials _targetmesh)) :!class /Script/Engine.KismetMaterialLibrary))
      (bind _output_get (Variables|Default|SetMaterial _returnvalue))
      (Rendering|Material|SetMaterial _targetmesh 0 _output_get)
      (Utilities|FlowControl|Sequence
        (:then_0
          (bind _returnvalue_2 (Rendering|Material|GetVectorParameterValue _output_get "FloorColor" :!class /Script/Engine.MaterialInstanceDynamic))
          (Variables|Default|SetFloorColor _returnvalue_2))
        (:then_1
          (Rendering|Material|SetVectorParameterValue _output_get "GlowColor" (Utilities|Struct|MakeLinearColor (Math|Random|RandomFloatinRange 0.0 1.0) (Math|Random|RandomFloatinRange 0.0 1.0) (Math|Random|RandomFloatinRange 0.0 1.0) 1.0) :!class /Script/Engine.MaterialInstanceDynamic))))
    (:then_1
      (Variables|Default|SetOriginalTransform (Transformation|GetActorTransform)))))

(fn OnRepNewColor
  (Rendering|Material|SetVectorParameterValue (Variables|Default|GetMaterial) "FloorColor" (Variables|Default|GetNewColor) :!class /Script/Engine.MaterialInstanceDynamic))

(fn MoveTowards
  (params (Actor :type Actor%20Object%20Reference) (Elapsed :type Float%20%28single-precision%29) (Duration :type Float%20%28single-precision%29) (Start :type Transform) (Target :type Transform))
  (bind (_location _rotation _scale) (Math|Transform|BreakTransform Target))
  (bind (_location_2 _rotation_2 _scale_2) (Math|Transform|BreakTransform Start))
  (bind _returnvalue (/ Elapsed Duration))
  (Transformation|SetActorTransform Actor (Math|Transform|MakeTransform (Math|Vector|Lerp(Vector) _location_2 _location _returnvalue) (Math|Rotator|Lerp(Rotator) _rotation_2 _rotation _returnvalue true) (Math|Vector|Lerp(Vector) _scale_2 _scale _returnvalue))))