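; Dummy controller actor whose mesh material can pulse a glow on and off, apparently to highlight buttons.
; The construction script puts a dynamic material instance on the Controller component.
; While shining, Tick eases the B2 and B4 scalar parameters up and down, reversing Direction at thresholds set just inside the interpolation targets so each swing completes.
; ToggleLight flip-flops the shining state, leaving the parameters at their current values when switched off.
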(event Custom|ToggleLight
  (Utilities|FlowControl|FlipFlop
    (:A
      (Variables|Default|SetIsShining true))
    (:B
      (Variables|Default|SetIsShining false))))

(event EventBeginPlay)

(event Collision|EventActorBeginOverlap
  (params (OtherActor :type Actor%20Object%20Reference)))

(event EventTick
  (params (DeltaSeconds :type Float%20%28single-precision%29))
  (bind _controllermaterial (Variables|Default|GetControllerMaterial))
  (if (Variables|Default|GetIsShining)
    (bind _returnvalue (Rendering|Material|GetScalarParameterValue _controllermaterial "B2" :!class /Script/Engine.MaterialInstanceDynamic))
    (if (Variables|Default|GetDirection)
      (Rendering|Material|SetScalarParameterValue _controllermaterial "B2" (Math|Interpolation|FInterpTo _returnvalue -1e+01 DeltaSeconds 2.0) :!class /Script/Engine.MaterialInstanceDynamic)
      (Rendering|Material|SetScalarParameterValue _controllermaterial "B4" (Math|Interpolation|FInterpTo _returnvalue -1e+01 DeltaSeconds 2.0) :!class /Script/Engine.MaterialInstanceDynamic)
      (if (<= (Math|Interpolation|FInterpTo _returnvalue -1e+01 DeltaSeconds 2.0) 0.0)
        (Variables|Default|SetDirection false))
      (else
        (Rendering|Material|SetScalarParameterValue _controllermaterial "B2" (Math|Interpolation|FInterpTo _returnvalue 2.1e+02 DeltaSeconds 2.0) :!class /Script/Engine.MaterialInstanceDynamic)
        (Rendering|Material|SetScalarParameterValue _controllermaterial "B4" (Math|Interpolation|FInterpTo _returnvalue 2.1e+02 DeltaSeconds 2.0) :!class /Script/Engine.MaterialInstanceDynamic)
        (if (>= (Math|Interpolation|FInterpTo _returnvalue 2.1e+02 DeltaSeconds 2.0) 2e+02)
          (Variables|Default|SetDirection true))))))

(fn ConstructionScript
  (bind _returnvalue (Rendering|Material|CreateDynamicMaterialInstance (Rendering|Material|GetMaterial (Variables|Default|GetController) 0) :!class /Script/Engine.KismetMaterialLibrary))
  (bind _output_get (Variables|Default|SetControllerMaterial _returnvalue))
  (Rendering|Material|SetMaterial (Variables|Default|GetController) 0 _output_get))