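; Target actor that grows when a Ray-type technique points at or overlaps it, and shrinks back afterwards.
; Overlap events and Enter/Leave events play or reverse a timeline, whose updates interpolate the mesh scale toward 1.5x or its original size, cached at construction.
; On BeginPlay the mesh eases to a random location and rotation within a box, then simulates physics.
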(event Custom|Enter
  ;[1 1 1] Restore dimensions
  (if (not (Variables|Default|GetIsOverlapping))
    ;[1 1 1] Animation
    (bind _direction (Timeline|Timeline_0 Play)
      (:Update
        (switch Utilities|FlowControl|Switch|SwitchonETimelineDirection _direction
          (:Forward
            (Variables|Default|SetCurrentTarget (Variables|Default|GetTargetScale)))
          (:Backward
            (Variables|Default|SetCurrentTarget (Variables|Default|GetInitialScale))))
        (Transformation|SetRelativeScale3D (Variables|Default|GetTargetMesh) (Math|Interpolation|VInterpTo (Variables|Default|GetCurrentScale) (Variables|Default|GetCurrentTarget) (Utilities|Time|GetWorldDeltaSeconds) 2.0))
        (Variables|Default|SetCurrentScale (Math|Interpolation|VInterpTo (Variables|Default|GetCurrentScale) (Variables|Default|GetCurrentTarget) (Utilities|Time|GetWorldDeltaSeconds) 2.0))))))

(event Custom|Leave
  ;[1 1 1] Restore dimensions
  (if (Variables|Default|GetIsOverlapping)
    ;[1 1 1] Animation
    (bind _direction (Timeline|Timeline_0 Reverse)
      (:Update
        (switch Utilities|FlowControl|Switch|SwitchonETimelineDirection _direction
          (:Forward
            (Variables|Default|SetCurrentTarget (Variables|Default|GetTargetScale)))
          (:Backward
            (Variables|Default|SetCurrentTarget (Variables|Default|GetInitialScale))))
        (Transformation|SetRelativeScale3D (Variables|Default|GetTargetMesh) (Math|Interpolation|VInterpTo (Variables|Default|GetCurrentScale) (Variables|Default|GetCurrentTarget) (Utilities|Time|GetWorldDeltaSeconds) 2.0))
        (Variables|Default|SetCurrentScale (Math|Interpolation|VInterpTo (Variables|Default|GetCurrentScale) (Variables|Default|GetCurrentTarget) (Utilities|Time|GetWorldDeltaSeconds) 2.0))))))

(event EventBeginPlay
  (bind _boxextent (Variables|Default|GetBoxExtent))
  (bind _returnvalue (/ _boxextent 2.0))
  ;[1 1 1] Spawn Animation
  (Components|MoveComponentTo (Variables|Default|GetTargetMesh) (Math|Random|RandomPointinBoundingBox (Math|Vector|MakeVector _returnvalue _returnvalue _returnvalue) (Math|Vector|MakeVector _boxextent _boxextent _returnvalue)) (Math|Random|RandomRotator true) true false 5.0 false)
  (Physics|SetSimulatePhysics (Variables|Default|GetTargetMesh) true))

(event Collision|EventActorEndOverlap
  (params (OtherActor :type Actor%20Object%20Reference))
  ;[1 1 1] Restore dimensions
  (Utilities|Casting|CastToITechnique OtherActor)
  ;[1 1 1] Animation
  (bind _direction (Timeline|Timeline_0 Reverse)
    (:Update
      (switch Utilities|FlowControl|Switch|SwitchonETimelineDirection _direction
        (:Forward
          (Variables|Default|SetCurrentTarget (Variables|Default|GetTargetScale)))
        (:Backward
          (Variables|Default|SetCurrentTarget (Variables|Default|GetInitialScale))))
      (Transformation|SetRelativeScale3D (Variables|Default|GetTargetMesh) (Math|Interpolation|VInterpTo (Variables|Default|GetCurrentScale) (Variables|Default|GetCurrentTarget) (Utilities|Time|GetWorldDeltaSeconds) 2.0))
      (Variables|Default|SetCurrentScale (Math|Interpolation|VInterpTo (Variables|Default|GetCurrentScale) (Variables|Default|GetCurrentTarget) (Utilities|Time|GetWorldDeltaSeconds) 2.0)))))

(event Collision|EventActorBeginOverlap
  (params (OtherActor :type Actor%20Object%20Reference))
  ;[1 1 1] Enlarge Actor when overlapped
  (bind _asitechnique (Utilities|Casting|CastToITechnique OtherActor))
  (bind _output_get (Variables|Default|SetTechniquePointer _asitechnique))
  (bind _techniquetype (Default|GetTechniqueType _output_get))
  (switch Utilities|FlowControl|Switch|SwitchonSelectionTechniqueEnum _techniquetype
    (:NewEnumerator0
      ;[1 1 1] Animation
      (bind _direction (Timeline|Timeline_0 Play)
        (:Update
          (switch Utilities|FlowControl|Switch|SwitchonETimelineDirection _direction
            (:Forward
              (Variables|Default|SetCurrentTarget (Variables|Default|GetTargetScale)))
            (:Backward
              (Variables|Default|SetCurrentTarget (Variables|Default|GetInitialScale))))
          (Transformation|SetRelativeScale3D (Variables|Default|GetTargetMesh) (Math|Interpolation|VInterpTo (Variables|Default|GetCurrentScale) (Variables|Default|GetCurrentTarget) (Utilities|Time|GetWorldDeltaSeconds) 2.0))
          (Variables|Default|SetCurrentScale (Math|Interpolation|VInterpTo (Variables|Default|GetCurrentScale) (Variables|Default|GetCurrentTarget) (Utilities|Time|GetWorldDeltaSeconds) 2.0)))))))

(fn ConstructionScript
  (bind _output_get (Variables|Default|SetCurrentScale (Variables|/Script/Engine.SceneComponent|GetRelativeScale3D (Variables|Default|GetTargetMesh))))
  (bind _output_get_2 (Variables|Default|SetInitialScale _output_get))
  (Variables|Default|SetTargetScale (* _output_get_2 1.5)))