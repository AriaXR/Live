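; UFONavigator flies the player along a spline route in a UFO that faces along the path.
; On BeginPlay it takes the first SplinePath's duration, attaches itself to the player pawn and hides the actor tagged "UFOstatic".
; Tick teleports the pawn by elapsed time at constant velocity and turns the UFO component to the spline rotation with a yaw offset.
; When the duration elapses, navigation stops and the navigator hides.
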(event EventBeginPlay
  (bind _returnvalue (Game|Player|GetPlayerPawn 0))
  (Utilities|FlowControl|Sequence
    (:then_0
      (bind _outactors (Actor|GetAllActorsOfClass "/Game/Blueprints/Actors/SplinePath.SplinePath_C"))
      (Variables|Default|SetSplinePath (Utilities|Array|Get(acopy) _outactors)))
    (:then_1
      (Variables|Default|SetDuration (Variables|/Script/Engine.SplineComponent|GetDuration (Variables|/Game/Blueprints/Actors/SplinePath.SplinePath_C|GetPath (Variables|Default|GetSplinePath)))))
    (:then_2
      (Utilities|Casting|CastToIPawn _returnvalue)
      (Transformation|AttachActorToActor _returnvalue "None" "KeepRelative" "KeepRelative" "KeepRelative" true))
    (:then_3
      (bind _outactors_2 (Actor|GetAllActorswithTag "UFOstatic"))
      (Rendering|SetActorHiddenInGame (Utilities|Array|Get(acopy) _outactors_2) true))))

(event Collision|EventActorBeginOverlap
  (params (OtherActor :type Actor%20Object%20Reference)))

(event EventTick
  (params (DeltaSeconds :type Float%20%28single-precision%29))
  (bind _returnvalue (Game|Player|GetPlayerPawn 0))
  (bind _splinepath (Variables|Default|GetSplinePath))
  (bind _path (Variables|/Game/Blueprints/Actors/SplinePath.SplinePath_C|GetPath _splinepath))
  ;[1 1 1] Move UFO along route and make it face forward along the path
  (if (not (Variables|Default|GetIsComplete))
    (if (>= (Variables|Default|GetElapsedTime) (Variables|Default|GetDuration))
      ;[1 1 1] Stop navigation once complete
      (Variables|Default|SetIsComplete true)
      (Rendering|SetActorHiddenInGame true)
      (else
        (Variables|Default|SetElapsedTime (+ (Variables|Default|GetElapsedTime) DeltaSeconds))
        (bind _asipawn (Utilities|Casting|CastToIPawn _returnvalue))
        (bind _camera (Default|GetCamera _asipawn))
        (Transformation|Teleport _returnvalue (Spline|GetLocationatTime _path (Variables|Default|GetElapsedTime) "World" true) "0, 0, 0")
        (Transformation|SetRelativeRotation (Variables|Default|GetUFO) (Math|Rotator|CombineRotators (Class|SplineComponent|GetRotationatTime _path (Variables|Default|GetElapsedTime) "Local" true) (Math|Rotator|MakeRotator 0.0 0.0 -9e+01)) false false)))))

(fn ConstructionScript)