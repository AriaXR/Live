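; ButtonActor is a button that changes color when another actor overlaps it.
; Begin and end overlap events swap both button meshes between shiny red while overlapped and shiny orange afterward, without filtering which actor overlaps.
; Separately, Tick sets IsCloseEnough each frame from the player pawn's distance against a short threshold; nothing in this Blueprint reads that flag.
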(event EventBeginPlay)

(event Collision|EventActorBeginOverlap
  (params (OtherActor :type Actor%20Object%20Reference))
  (Rendering|Material|SetMaterial (Variables|Default|GetButtonMesh) 0 "/Game/Assets/Abstract/Materials/M_Red_Shiny.M_Red_Shiny")
  (Rendering|Material|SetMaterial (Variables|Default|GetButtonMesh2) 0 "/Game/Assets/Abstract/Materials/M_Red_Shiny.M_Red_Shiny"))

(event EventTick
  (params (DeltaSeconds :type Float%20%28single-precision%29))
  (Variables|Default|SetbIsCloseEnough! (< (Transformation|GetDistanceTo (Game|Player|GetPlayerPawn 0)) 5e+01)))

(event Collision|EventActorEndOverlap
  (params (OtherActor :type Actor%20Object%20Reference))
  (Rendering|Material|SetMaterial (Variables|Default|GetButtonMesh) 0 "/Game/Assets/Abstract/Materials/M_Orange_Shiny.M_Orange_Shiny")
  (Rendering|Material|SetMaterial (Variables|Default|GetButtonMesh2) 0 "/Game/Assets/Abstract/Materials/M_Orange_Shiny.M_Orange_Shiny"))

(fn ConstructionScript)