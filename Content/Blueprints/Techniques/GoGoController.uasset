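; VR hand controller implementing the Go-Go technique, stretching the virtual hand's reach non-linearly as the real hand moves away from the body.
; On authority, Tick measures the controller in spherical coordinates around a point below the parent pawn's camera.
; Beyond LinearDistance, it adds a K-scaled squared excess to the radius and moves HandMesh through ClientUpdate.
; Within that distance, it only stores the initial hand offset, without moving the mesh.
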(event Custom|ClientUpdate
  (params (NewLocation :type Vector))
  (Transformation|SetWorldLocation (Variables|Default|GetHandMesh) NewLocation false false))

(event EventBeginPlay)

(event Collision|EventActorBeginOverlap
  (params (OtherActor :type Actor%20Object%20Reference)))

(event EventTick
  (params (DeltaSeconds :type Float%20%28single-precision%29))
  (|CallParentFunction DeltaSeconds)
  (Networking|SwitchHasAuthority
    (:Authority
      (bind _asipawn (Utilities|Casting|CastToIPawn (Actor|GetAttachParentActor)))
      (bind _camera (Default|GetCamera _asipawn))
      (bind (_r _inclination _azimuth) (CallFunction|CartesiantoSpherical (Math|Transform|MakeTransform (Math|Vector|MakeVector (.X (Math|Vector|BreakVector (Transformation|GetWorldLocation _camera))) (.Y (Math|Vector|BreakVector (Transformation|GetWorldLocation _camera))) (- (.Z (Math|Vector|BreakVector (Transformation|GetWorldLocation _camera))) 4e+01)) (.Rotation (Math|Transform|BreakTransform (Transformation|GetWorldTransform _camera))) (.Scale (Math|Transform|BreakTransform (Transformation|GetWorldTransform _camera)))) (Transformation|GetWorldLocation (Variables|Default|GetScene))))
      (if (<= _r (Variables|Default|GetLinearDistance))
        (Variables|Default|SetHandLocation (Variables|Default|GetInitial%20Hand%20Offset))
        (else
          (bind _location (CallFunction|SphericaltoCartesian (|(R+(coff*(pow((R-D),2)))) _r (Variables|Default|Getk) (Variables|Default|GetLinearDistance)) _inclination _azimuth))
          (bind _output_get (Variables|Default|SetHandLocation (Math|Transform|TransformLocation (Math|Transform|MakeTransform (Math|Vector|MakeVector (.X (Math|Vector|BreakVector (Transformation|GetWorldLocation _camera))) (.Y (Math|Vector|BreakVector (Transformation|GetWorldLocation _camera))) (- (.Z (Math|Vector|BreakVector (Transformation|GetWorldLocation _camera))) 4e+01)) (.Rotation (Math|Transform|BreakTransform (Transformation|GetWorldTransform _camera))) (.Scale (Math|Transform|BreakTransform (Transformation|GetWorldTransform _camera)))) _location)))
          (CallFunction|ClientUpdate _output_get))))))

(fn ConstructionScript
  (|CallParentFunction)
  (Variables|Default|SetInitial%20Hand%20Offset (Variables|/Script/Engine.SceneComponent|GetRelativeLocation (Variables|Default|GetHandMesh))))

(fn DistancetoHand
  (params (Pawn%20Location :type Vector))
  (return (Math|Vector|VectorLength (- (Transformation|GetWorldLocation (Variables|Default|GetScene)) Pawn%20Location))))