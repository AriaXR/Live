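; VR cone pointer technique that selects TargetActors, with a cone width adjustable from the trackpad.
; Each tick maps trackpad Y to the cone's XY scale, keeping the last width when Y is zero.
; It approximates the cone with multi-sphere traces along the motion controller's forward vector, sized by the cone radius at the current distance.
; Hit targets get Enter and an overlap flag, while all other TargetActors get Leave.
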(event EventBeginPlay
  (Variables|Default|SetVR%20Pawn (.AsIPawn (Utilities|Casting|CastToIPawn (Game|Player|GetPlayerPawn 0))))
  (Variables|Default|SetCurrentScale (Math|Vector|MakeVector 1.0 1.0 (.Z (Math|Vector|BreakVector (Transformation|GetWorldScale (Variables|Default|GetOffset)))))))

(event Collision|EventActorBeginOverlap
  (params (OtherActor :type Actor%20Object%20Reference)))

(event EventTick
  (params (DeltaSeconds :type Float%20%28single-precision%29))
  (bind _offset (Variables|Default|GetOffset))
  ;[1 1 1] Use Trackpad Y position for Scale
  (bind _trackpadposition (Default|GetTrackpadPosition (Variables|Default|GetVR%20Pawn) "NewEnumerator0"))
  (bind _output_get (Variables|Default|SetTrackpadPosition _trackpadposition))
  (if (Math|Float|NearlyEqual(Float) (.Y (Math|Vector2D|BreakVector2D _output_get)) 0.0 1e-06)
    (Variables|Default|SetNewScale (Variables|Default|GetCurrentScale))
    (else
      ;[1 1 1] Assign value to XY scale
      (Variables|Default|SetNewScale (Math|Vector|MakeVector (Math|Float|MapRangeClamped (* (Class|KismetMathLibrary|VSize2DSquared (Math|Vector2D|MakeVector2D 0.0 (- (.Y (Math|Vector2D|BreakVector2D _output_get)) 1.0))) (Variables|Default|GetScaleFactor) DeltaSeconds) 0.0 2.0 1.0 1e+01) (Math|Float|MapRangeClamped (* (Class|KismetMathLibrary|VSize2DSquared (Math|Vector2D|MakeVector2D 0.0 (- (.Y (Math|Vector2D|BreakVector2D _output_get)) 1.0))) (Variables|Default|GetScaleFactor) DeltaSeconds) 0.0 2.0 1.0 1e+01) (.Z (Math|Vector|BreakVector (Transformation|GetWorldScale _offset)))))))
  (Transformation|SetRelativeScale3D _offset (Variables|Default|GetNewScale))
  (Variables|Default|SetCurrentScale (Variables|Default|GetNewScale))
  (CallFunction|ConeIntersectsObject))

(fn ConstructionScript)

(fn GetAngle
  (bind _currentscale (Variables|Default|GetCurrentScale))
  (bind (_x _y _z) (Math|Vector|BreakVector _currentscale))
  (bind _angleradians (CallFunction|ConeAngle (/ _x 2.0) _z))
  (return _angleradians))

(fn ConeIntersectsObject
  (bind _motioncontroller (Default|GetMotionController (.AsIPawn (Utilities|Casting|CastToIPawn (Game|Player|GetPlayerPawn 0))) "NewEnumerator1"))
  (bind _output_get (LocalVariables|SetConeVertex (Transformation|GetWorldLocation _motioncontroller)))
  (bind _output_get_2 (LocalVariables|SetConeDirection (Math|Vector|GetForwardVector _motioncontroller)))
  (bind (_radius _height) (CallFunction|GetRadiusandHeight))
  (for _index (range 1 20)
    (CallFunction|PointAlongDirection _output_get _output_get_2 (LocalVariables|GetDistance))
    (bind _newradius (CallFunction|ConeRadiusatHeight _radius _height (LocalVariables|GetDistance)))
    (bind _point (CallFunction|PointAlongDirection (LocalVariables|GetConeVertex) (LocalVariables|GetConeDirection) (LocalVariables|GetDistance)))
    (bind _point_2 (CallFunction|PointAlongDirection (LocalVariables|GetConeVertex) (LocalVariables|GetConeDirection) 1e+03))
    (LocalVariables|SetDistance (+ (* _newradius 2.0) (LocalVariables|GetDistance)))
    (bind _outhits (Collision|MultiSphereTraceForObjects _point _point_2 _newradius (Utilities|Array|MakeArray "ObjectTypeQuery2") false 0 "None"))
    (for _array_element _outhits
      (bind _astarget_actor (Utilities|Casting|CastToTargetActor (.HitActor (Collision|BreakHitResult _array_element))))
      (Default|Enter _astarget_actor)
      (Variables|/Game/Blueprints/Actors/TargetActor.TargetActor_C|SetIsOverlapping _astarget_actor true)
      (Utilities|Array|AddUnique (LocalVariables|GetOverlappedActors) _astarget_actor))
    (bind _outactors (Actor|GetAllActorsOfClass "/Game/Blueprints/Actors/TargetActor.TargetActor_C"))
    (for _array_element_2 _outactors
      (if (not (Utilities|Array|ContainsItem (LocalVariables|GetOverlappedActors) _array_element_2))
        (Default|Leave _array_element_2)
        (Variables|/Game/Blueprints/Actors/TargetActor.TargetActor_C|SetIsOverlapping _array_element_2 false)))
    (Utilities|Array|Clear (LocalVariables|GetOverlappedActors))
    (return false))
  (return false))

(fn GetRadiusandHeight
  (bind _currentscale (Variables|Default|GetCurrentScale))
  (bind (_x _y _z) (Math|Vector|BreakVector _currentscale))
  (return (/ _x 2.0) _z))

(fn GetTechniqueType
  (return "NewEnumerator1"))