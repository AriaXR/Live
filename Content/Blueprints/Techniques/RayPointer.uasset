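; RayPointer is a controller ray-pointing technique that forwards trigger input to the reactive object it points at.
; A trigger press traces from SceneRoot, stores the hit actor or its attach parent implementing IControllerReactive, and presses it; release goes to that stored actor.
; The trace ignores the bounding box, itself and the player pawn.
; Grip release toggles ray mesh visibility; trackpad push/pull movement code is disconnected.
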(event Custom|OnRelease
  (params (Actor :type Actor%20Object%20Reference))
  (Default|RTriggerReleased (.AsIController%20Reactive (Utilities|Casting|CastToIControllerReactive Actor))))

(event Custom|ServerToggleRayVisibility
  (bind _raymesh (Variables|Default|GetRayMesh))
  (Utilities|FlowControl|FlipFlop
    (:A
      (Development|SetHiddeninGame _raymesh false false))
    (:B
      (Development|SetHiddeninGame _raymesh true false))))

(event Custom|RayTrace
  (params (Location :type Vector) (Forward :type Vector))
  ;[1 1 1] RayTrace
  (bind _firsthit (CallFunction|RayTrace Location Forward (Variables|Default|GetRayTraceObjectTypes) (Variables|Default|GetActors%20to%20Ignore)))
  (Utilities|IsValid (.HitActor (Collision|BreakHitResult _firsthit))
    (:Is%20Valid
      (bind _asicontroller_reactive (Utilities|Casting|CastToIControllerReactive (.HitActor (Collision|BreakHitResult _firsthit)))
        (:then
          (Variables|Default|SetHitActor _asicontroller_reactive))
        (:CastFailed
          (bind _asicontroller_reactive_2 (Utilities|Casting|CastToIControllerReactive (Actor|GetAttachParentActor (.HitActor (Collision|BreakHitResult _firsthit)))))
          (Variables|Default|SetHitActor _asicontroller_reactive_2)))
      (Default|RTriggerPressed (Variables|Default|GetHitActor)))))

(event Custom|ServerRelease
  (CallFunction|OnRelease (.AsActor (Utilities|Casting|CastToActor (Variables|Default|GetHitActor)))))

(event EventBeginPlay
  (Utilities|Array|Add (Variables|Default|GetActors%20to%20Ignore) (Game|Player|GetPlayerPawn 0)))

(event Collision|EventActorBeginOverlap
  (params (OtherActor :type Actor%20Object%20Reference)))

(event EventRTriggerPressed
  (bind _sceneroot (Variables|Default|GetSceneRoot))
  (Variables|Default|SetbTriggerPressed true)
  (CallFunction|RayTrace (Transformation|GetWorldLocation _sceneroot) (Math|Vector|GetForwardVector _sceneroot)))

(event EventRTriggerReleased
  (CallFunction|ServerRelease))

(event EventTick
  (params (DeltaSeconds :type Float%20%28single-precision%29))
  (if false
    _))

(event EventRGripReleased
  (CallFunction|ServerToggleRayVisibility))

(fn ConstructionScript
  (bind _outactors (Actor|GetAllActorsOfClass "/Game/Blueprints/Actors/BoundingBox.BoundingBox_C"))
  (Utilities|IsValid (Utilities|Array|Get(acopy) _outactors)
    (:Is%20Valid
      (bind _output_get (Variables|Default|SetBoundingBox (Utilities|Array|Get(acopy) _outactors)))
      (Variables|Default|SetActors%20to%20Ignore (Utilities|Array|MakeArray _output_get self)))))

(fn GetTechniqueType
  (return "NewEnumerator0"))

(fn ReturnFirstRaytraceHit
  (params (Pointer :type Scene%20Component%20Object%20Reference))
  (bind _firsthit (CallFunction|RayTrace (Transformation|GetWorldLocation Pointer) (Math|Vector|GetForwardVector Pointer) (Variables|Default|GetRayTraceObjectTypes) (Variables|Default|GetActors%20to%20Ignore)))
  (return (.HitActor (Collision|BreakHitResult _firsthit))))