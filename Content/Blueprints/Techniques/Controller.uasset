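; Controller technique Blueprint that animates a right Vive controller model to mirror trackpad and trigger input, reporting its own technique type enum.
; Trackpad updates store the thumb position and map it, with axes swapped and scaled, to a sphere's relative location on the controller.
; Trigger axis and press events share one path that passes the axis value to the controller's Animation Blueprint to drive the trigger animation.
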(event EventBeginPlay)

(event Collision|EventActorBeginOverlap
  (params (OtherActor :type Actor%20Object%20Reference)))

(event EventRTrackpadUpdate
  (params (Position :type Vector%202D%20Structure))
  ;[0.1137 0.349 1] Right Trackpad Thumb Tracking
  (bind _output_get (Variables|Default|SetTrackpadPosition Position))
  (bind _output_get_2 (Variables|Default|SetR%20ThumbX (.X (Math|Vector2D|BreakVector2D _output_get))))
  (bind _output_get_3 (Variables|Default|SetR%20ThumbY (.Y (Math|Vector2D|BreakVector2D _output_get))))
  (Transformation|SetRelativeLocation (Variables|Default|GetR%20TrackpadSphere) (Math|Vector|MakeVector (- (* _output_get_3 -1.7) 3.5) (* _output_get_2 1.7) 1.8) false false))

(event EventRTriggerPressed
  ;[0.1137 0.349 1] Right Controller w/ Trigger Animation
  (bind _asvive_controller_ab (Utilities|Casting|CastToVive_Controller_AB (Components|SkeletalMesh|GetAnimInstance (Variables|Default|GetR%20ViveController))))
  (Variables|/Game/Assets/Controller/Animations/Vive_Controller_AB.Vive_Controller_AB_C|SetTriggerAxisAmount _asvive_controller_ab (stale EventRTriggerAxis Value)))

(event EventTick
  (params (DeltaSeconds :type Float%20%28single-precision%29)))

(event EventRTriggerAxis
  (params (Value :type Float%20%28single-precision%29))
  ;[0.1137 0.349 1] Right Controller w/ Trigger Animation
  (bind _asvive_controller_ab (Utilities|Casting|CastToVive_Controller_AB (Components|SkeletalMesh|GetAnimInstance (Variables|Default|GetR%20ViveController))))
  (Variables|/Game/Assets/Controller/Animations/Vive_Controller_AB.Vive_Controller_AB_C|SetTriggerAxisAmount _asvive_controller_ab Value))

(fn ConstructionScript)

(fn GetTechniqueType
  (return "NewEnumerator4"))