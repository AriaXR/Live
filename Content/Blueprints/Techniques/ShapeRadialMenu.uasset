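; Shape selection technique that uses a right-trackpad radial menu to pick a sphere, cube or pyramid.
; Trackpad position maps to sectors that set the selected shape and move a spotlight beside it, while one sector or centre only resets the spotlight.
; Release sends the shape name to the first ContextualMenuActor, defaulting to sphere, and counts changes.
; SetupNewActor copies the selected mesh and material onto a BrickActor and enables physics.
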(event EventBeginPlay)

(event Collision|EventActorBeginOverlap
  (params (OtherActor :type Actor%20Object%20Reference)))

(event EventSetupNewActor
  (params (Actor :type Actor%20Object%20Reference))
  (bind _asbrick_actor (Utilities|Casting|CastToBrickActor Actor))
  (bind _selectedactor (Variables|Default|GetSelectedActor))
  (bind _staticmesh (Variables|/Game/Blueprints/Actors/BrickActor.BrickActor_C|GetStaticMesh _asbrick_actor))
  (Components|StaticMesh|SetStaticMesh _staticmesh (Variables|/Script/Engine.StaticMeshComponent|GetStaticMesh _selectedactor))
  (Rendering|Material|SetMaterial _staticmesh 0 (Rendering|Material|GetMaterial _selectedactor 0))
  (Physics|SetSimulatePhysics _staticmesh true))

(event EventTick
  (params (DeltaSeconds :type Float%20%28single-precision%29)))

(event EventRTrackpadUpdate
  (params (Position :type Vector%202D%20Structure))
  ;[1 1 1] Handle Trackpad selection
  (|CallParentFunction Position)
  (if (Math|Vector|NotEqual(Vector) :A Position)
    (bind _sector (CallFunction|PositiontoSector 4 Position 0.0))
    (switch int _sector
      (:0
        (Variables|Default|SetSelectedActor (Variables|Default|GetSphere) :!label _label)
        (Variables|Default|SetNewPosition (+ (Variables|/Script/Engine.SceneComponent|GetRelativeLocation (Variables|Default|GetSelectedActor)) "-100.000000, 0, 0") :!label _label_2))
      (:1
        (Variables|Default|SetNewPosition "0, 0, 0" :!label _label_3))
      (:2
        (Variables|Default|SetSelectedActor (Variables|Default|GetCube))
        (goto _label_2))
      (:3
        (Variables|Default|SetSelectedActor (Variables|Default|GetPyramid))
        (goto _label_2))
      (:4
        (goto _label)))
    (else
      (goto _label_3)))
  (Transformation|SetRelativeLocation (Variables|Default|GetSpotLight) (Variables|Default|GetNewPosition) false false))

(event EventRTrackpadReleased
  (Utilities|IsValid (Variables|Default|GetSelectedActor)
    (:Is%20Valid
      _)
    (:Is%20Not%20Valid
      (Variables|Default|SetSelectedActor (Variables|Default|GetSphere))))
  (bind _outactors (Actor|GetAllActorsOfClass "/Game/Blueprints/Actors/ContextualMenuActor.ContextualMenuActor_C"))
  (Default|ChangeShape (Utilities|Array|Get(acopy) _outactors) (Utilities|GetObjectName (Variables|Default|GetSelectedActor)))
  (Math|Integer|IncrementInt (Variables|Default|GetTimesChanged)))

(fn ConstructionScript
  (|CallParentFunction))