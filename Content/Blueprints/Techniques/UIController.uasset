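; UIController is a pointer controller that lets the player hover and click world widgets and reactive actors using a WidgetInteraction component.
; Each tick, a ray trace along the component's forward vector sends begin and end overlap calls to IControllerReactive actors.
; Hovered-widget changes forward PointerEnter and PointerLeave through IWidget.
; Right-trigger events simulate left mouse press and release, with release also notifying the hovered widget's owning actor.
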(event OnHoveredWidgetChanged(WidgetInteraction)
  (params (WidgetComponent :type Widget%20Component%20Object%20Reference) (PreviousWidgetComponent :type Widget%20Component%20Object%20Reference))
  ;[1 1 1] Forward pointer enter/leave to widget
  (Utilities|IsValid WidgetComponent
    (:Is%20Valid
      (if (!= WidgetComponent PreviousWidgetComponent)
        (Utilities|IsValid (Variables|Default|GetCurrentWidget)
          (:Is%20Valid
            (Utilities|IsValid (Utilities|ToObject(Interface) (.AsIWidget (Utilities|Casting|CastToIWidget (Variables|Default|GetCurrentWidget))))
              (:Is%20Valid
                (Default|PointerLeave (.AsIWidget (Utilities|Casting|CastToIWidget (Variables|Default|GetCurrentWidget)))))
              (:Is%20Not%20Valid
                _)))
          (:Is%20Not%20Valid
            _))
        (Variables|Default|SetPreviousWidget (Variables|Default|GetCurrentWidget))
        (Variables|Default|SetCurrentWidget (UserInterface|GetUserWidgetObject WidgetComponent))
        (Utilities|IsValid (Utilities|ToObject(Interface) (.AsIWidget (Utilities|Casting|CastToIWidget (Variables|Default|GetCurrentWidget))))
          (:Is%20Valid
            (Default|PointerEnter (.AsIWidget (Utilities|Casting|CastToIWidget (Variables|Default|GetCurrentWidget))))))))))

(event Custom|RaisePress
  (Class|WidgetInteractionComponent|PressPointerKey (Variables|Default|GetWidgetInteraction) "LeftMouseButton"))

(event Custom|RaiseRelease
  (bind _widgetinteraction (Variables|Default|GetWidgetInteraction))
  (bind _returnvalue (Class|WidgetInteractionComponent|GetHoveredWidgetComponent _widgetinteraction))
  (bind _returnvalue_2 (Components|GetOwner _returnvalue))
  (Utilities|FlowControl|Sequence
    (:then_0
      (Class|WidgetInteractionComponent|ReleasePointerKey (Variables|Default|GetWidgetInteraction) "LeftMouseButton"))
    (:then_1
      (Utilities|IsValid _returnvalue_2
        (:Is%20Valid
          (bind _asicontroller_reactive (Utilities|Casting|CastToIControllerReactive _returnvalue_2))
          (Default|RTriggerReleased _asicontroller_reactive (Variables|Default|GetCurrentWidget)))))))

(event EventBeginPlay)

(event Collision|EventActorBeginOverlap
  (params (OtherActor :type Actor%20Object%20Reference)))

(event EventRTriggerPressed
  (CallFunction|RaisePress))

(event EventTick
  (params (DeltaSeconds :type Float%20%28single-precision%29))
  (bind _widgetinteraction (Variables|Default|GetWidgetInteraction))
  ;[1 1 1] Checks whether we are overlapping an IControllerReactive
  (bind _firsthit (CallFunction|RayTrace (Transformation|GetWorldLocation _widgetinteraction) (Math|Vector|GetForwardVector _widgetinteraction) (Utilities|Array|MakeArray "ObjectTypeQuery2") (Utilities|Array|MakeArray 0)))
  (if (!= (Variables|Default|GetHitActor) (.HitActor (Collision|BreakHitResult _firsthit)))
    (Utilities|IsValid (Variables|Default|GetHitActor)
      (:Is%20Valid
        (bind _asicontroller_reactive (Utilities|Casting|CastToIControllerReactive (Variables|Default|GetHitActor)))
        (Default|ControllerEndOverlap _asicontroller_reactive))
      (:Is%20Not%20Valid
        _))
    (bind _asicontroller_reactive_2 (Utilities|Casting|CastToIControllerReactive (.HitActor (Collision|BreakHitResult _firsthit)))
      (:then
        (Variables|Default|SetHitActor (.HitActor (Collision|BreakHitResult _firsthit)))
        (Default|ControllerBeginOverlap _asicontroller_reactive_2))
      (:CastFailed
        (Variables|Default|SetHitActor 0)))))

(event EventRTriggerReleased
  (CallFunction|RaiseRelease))

(fn ConstructionScript
  (|CallParentFunction))