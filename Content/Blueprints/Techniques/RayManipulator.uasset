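; RayManipulator is a VR interaction technique for grabbing and moving objects with a ray from the right controller.
; Pressing the trigger attaches the first ray-hit actor to the controller, keeping its world transform, and releasing it detaches the actor.
; While an actor is held, Tick uses the trackpad's Y sign to slide it at constant speed along the SceneRoot forward axis.
; The technique adds itself and the player pawn to its ignore list.
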(event EventBeginPlay
  (Utilities|Array|Add (Variables|Default|GetActors%20to%20Ignore) (Game|Player|GetPlayerPawn 0)))

(event Collision|EventActorBeginOverlap
  (params (OtherActor :type Actor%20Object%20Reference)))

(event EventRTrackpadUpdate
  (params (Position :type Vector%202D%20Structure))
  (bind _output_get (Variables|Default|SetTrackpadPosition Position)))

(event EventRTriggerPressed
  (bind _actor (CallFunction|ReturnFirstRaytraceHit (Variables|Default|GetR%20ViveController)))
  (Utilities|IsValid _actor
    (:Is%20Valid
      (if (or (!= _actor (Variables|Default|GetActor)) (not (Utilities|IsValid (Variables|Default|GetActor))))
        (Utilities|IsValid (Variables|Default|GetActor)
          (:Is%20Valid
            (Transformation|DetachFromActor (Variables|Default|GetActor) "KeepWorld" "KeepWorld" "KeepWorld"))
          (:Is%20Not%20Valid
            _))
        (bind _output_get (Variables|Default|SetActor _actor))
        (Transformation|AttachComponentToComponent _output_get (Variables|Default|GetR%20ViveController) "None" "KeepWorld" "KeepWorld" "KeepWorld" true)))
    (:Is%20Not%20Valid
      (Variables|Default|SetActor 0))))

(event EventRTriggerReleased
  (Utilities|IsValid (Variables|Default|GetActor)
    (:Is%20Valid
      (Transformation|DetachFromActor (Variables|Default|GetActor) "KeepWorld" "KeepWorld" "KeepWorld")
      (Variables|Default|SetActor 0))))

(event EventTick
  (params (DeltaSeconds :type Float%20%28single-precision%29))
  (bind _actor (Variables|Default|GetActor))
  (Utilities|IsValid _actor
    (:Is%20Valid
      (bind _point (CallFunction|PointAlongDirection (Transformation|GetActorLocation _actor) (Math|Vector|GetForwardVector (Variables|Default|GetSceneRoot)) (* DeltaSeconds (* (Math|Float|Sign(Float) (.Y (Math|Vector2D|BreakVector2D (stale EventRTrackpadUpdate _output_get)))) -3e+02))))
      (Transformation|SetActorLocation _actor _point false false))))

(event Input|KeyboardEvents|MotionControllerRightTrigger
  (params (Key :type Key%20Structure :default "AnyKey"))
  (:Pressed
    (bind _actor (CallFunction|ReturnFirstRaytraceHit (Variables|Default|GetR%20ViveController)))
    (Utilities|IsValid _actor
      (:Is%20Valid
        (if (or (!= _actor (Variables|Default|GetActor)) (not (Utilities|IsValid (Variables|Default|GetActor))))
          (Utilities|IsValid (Variables|Default|GetActor)
            (:Is%20Valid
              (Transformation|DetachFromActor (Variables|Default|GetActor) "KeepWorld" "KeepWorld" "KeepWorld"))
            (:Is%20Not%20Valid
              _))
          (bind _output_get (Variables|Default|SetActor _actor))
          (Transformation|AttachComponentToComponent _output_get (Variables|Default|GetR%20ViveController) "None" "KeepWorld" "KeepWorld" "KeepWorld" true)))
      (:Is%20Not%20Valid
        (Variables|Default|SetActor 0))))
  (:Released
    (Utilities|IsValid (Variables|Default|GetActor)
      (:Is%20Valid
        (Transformation|DetachFromActor (Variables|Default|GetActor) "KeepWorld" "KeepWorld" "KeepWorld")
        (Variables|Default|SetActor 0)))))

(fn ConstructionScript
  (Variables|Default|SetActors%20to%20Ignore (Utilities|Array|MakeArray self)))

(fn GetTechniqueType
  (return "NewEnumerator0"))