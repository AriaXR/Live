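; Maths is a set of geometry helper functions covering cones, angles, directions and coordinate conversion.
; Cone helpers derive apex angle and scaled radius, while angle helpers give the acute angle between vectors and a 0–360 degree heading from XY.
; RayTrace runs a fixed-length object-type line trace and returns the hit.
; Spherical conversion works in an origin transform's local space, using single-argument Atan for azimuth, so opposite quadrants are not distinguished.
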(fn ConeAngle
  (params (BaseRadius :type Float%20%28single-precision%29) (Height :type Float%20%28single-precision%29))
  (return (* (Math|Trig|Atan(Degrees) (/ BaseRadius Height)) 2.0)))

(fn AngleBetweenVectors
  (params (Vector1 :type Vector) (Vector2 :type Vector))
  (bind _returnvalue (Math|Vector|Normalize Vector1))
  (bind _returnvalue_2 (Math|Vector|Normalize Vector2))
  (bind _returnvalue_3 (Math|Vector|DotProduct _returnvalue _returnvalue_2))
  (bind _returnvalue_4 (Math|Float|Clamp(Float) _returnvalue_3 -1.0))
  (bind _returnvalue_5 (Math|Trig|Acos(Degrees) _returnvalue_4))
  (return (Math|Float|Min(Float) _returnvalue_5 (Math|Float|Absolute(Float) (- _returnvalue_5 (Math|Trig|GetPI))))))

(fn ConeRadiusatHeight
  (params (Radius :type Float%20%28single-precision%29) (Height :type Float%20%28single-precision%29) (NewHeight :type Float%20%28single-precision%29))
  (return (/ (* Radius NewHeight) Height)))

(fn PointAlongDirection
  (params (Origin :type Vector) (Direction :type Vector) (Distance :type Float%20%28single-precision%29))
  (return (+ Origin (* Direction Distance))))

(fn RayTrace
  (params (Location :type Vector) (Forward :type Vector) (ObjectTypes :type Array%20of%20EObjectTypeQuery%20Enums) (Actors%20to%20Ignore :type Array%20of%20Actor%20Object%20References))
  (bind _outhit (Collision|LineTraceForObjects 0 Location (+ Location (* Forward 5000)) ObjectTypes false Actors%20to%20Ignore "None"))
  (return _outhit))

(fn GetAnglefromUnitVector
  (params (Unit%20Vector :type Vector%202D%20Structure))
  (bind (_x _y) (Math|Vector2D|BreakVector2D Unit%20Vector))
  (return (Math|Float|%(Float) (+ (Class|KismetMathLibrary|DegAtan2 _y _x) 3.6e+02) 3.6e+02)))

(fn CartesiantoSpherical
  (params (Origin :type Transform) (Position :type Vector))
  (bind _returnvalue (Math|Transform|InverseTransformLocation Origin Position))
  (bind _returnvalue_2 (Math|Vector|VectorLength _returnvalue))
  (bind (_x _y _z) (Math|Vector|BreakVector _returnvalue))
  (return _returnvalue_2 (Math|Trig|Acos(Degrees) (/ _z _returnvalue_2)) (Math|Trig|Atan(Degrees) (/ _y _x))))

(fn SphericaltoCartesian
  (params (R :type Float%20%28single-precision%29) (Inclination :type Float%20%28single-precision%29) (Azimuth :type Float%20%28single-precision%29))
  (return (Math|Vector|MakeVector (|((r*(sin(Inclination)))*(cos(Azimuth))) R Inclination Azimuth) (|((r*(sin(Inclination)))*(sin(Azimuth))) R Inclination Azimuth) (|(r*(cos(Inclination))) R Inclination))))