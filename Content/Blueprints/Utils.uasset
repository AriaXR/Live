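; Utility function library for a VR app with selection, manipulation, navigation and system-control scenarios.
; Helpers convert scenario names to identifiers, supply display titles and report the selection map as non-networked, with the true result left unwired.
; Actor lookups return the first actor of a given class and search IPawn implementers by user class.
; The pawn search returns inside its loop, at the first match.
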(fn StringtoScenario
  (params (Scenario :type String))
  (switch string Scenario
    (:VRSelectionMap
      (return "NewEnumerator1"))
    (:VRManipulationMap
      (return "NewEnumerator3"))
    (:VRNavigationMap
      (return "NewEnumerator4"))
    (:VRSystemMap
      (return "NewEnumerator6"))))

(fn TitlefromScenarioEnum
  (params (Scenario :type ScenarioEnum%20Enum))
  (switch Utilities|FlowControl|Switch|SwitchonScenarioEnum Scenario
    (:NewEnumerator5
      (return "Error"))
    (:NewEnumerator1
      (return "3D Selection"))
    (:NewEnumerator3
      (return "3D Manipulation"))
    (:NewEnumerator4
      (return "3D Navigation"))
    (:NewEnumerator6
      (return "3D System Control"))))

(fn IsNetworkScenario
  (params (Scenario :type ScenarioEnum%20Enum))
  (switch Utilities|FlowControl|Switch|SwitchonScenarioEnum Scenario
    (:NewEnumerator1
      (return false))))

(fn GetActorOfType
  (params (Type :type Actor%20Class%20Reference))
  (bind _outactors (Actor|GetAllActorsOfClass 0 Type))
  (Utilities|IsValid (Utilities|Array|Get(acopy) _outactors)
    (:Is%20Valid
      (return (Utilities|Array|Get(acopy) _outactors)))
    (:Is%20Not%20Valid
      (return 0))))

(fn GetAllPawnsbyUserClass
  (params (User%20Class :type UserClassEnum%20Enum))
  (bind _outactors (Actor|GetAllActorswithInterface 0 "/Game/Blueprints/Pawns/IPawn.IPawn_C"))
  (for _array_element _outactors
    (bind _asipawn (Utilities|Casting|CastToIPawn _array_element))
    (bind _user (Default|GetUser _asipawn))
    (if (Utilities|Enum|Equal(Enum) (.UserClass (Utilities|Struct|BreakUser _user)) User%20Class)
      (Utilities|Array|AddUnique (LocalVariables|GetPawns) _asipawn)
      (return (LocalVariables|GetPawns)))))