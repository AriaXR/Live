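; Helper functions for a radial menu in a VR user interface, supplying its command labels and mapping an input position to a menu sector.
; CreateCommands picks labels by scenario and user class; all VR maps currently give "Next" to User and Observer, while unset selections return warning labels.
; PositionToSector turns a unit vector's angle, offset by an initial angle, into a rounded sector index.
; LogScreen prints text on screen.
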(fn LogScreen
  (params (Text :type Text))
  (Development|PrintText 0 Text))

(fn CreateCommands
  (params (Scenario :type ScenarioEnum%20Enum) (User%20Class :type UserClassEnum%20Enum))
  (switch Utilities|FlowControl|Switch|SwitchonScenarioEnum Scenario
    (:NewEnumerator5
      _)
    (:NewEnumerator1
      (switch Utilities|FlowControl|Switch|SwitchonUserClassEnum User%20Class :!label _label
        (:NewEnumerator0
          _)
        (:NewEnumerator1
          (return (Utilities|Array|MakeArray (Utilities|String|MakeLiteralString "Next"))))
        (:NewEnumerator2
          (return (Utilities|Array|MakeArray (Utilities|String|MakeLiteralString "Next"))))))
    (:NewEnumerator3
      (goto _label))
    (:NewEnumerator4
      (goto _label))
    (:NewEnumerator6
      (goto _label)))
  (Development|PrintString 0 "Warning, no Scenario or User selected.")
  (return (Utilities|Array|MakeArray "No" "Scenario" "or User" "Selected")))

(fn PositiontoSector
  (params (ItemCount :type Integer) (Position :type Vector%202D%20Structure) (InitialAngle :type Float%20%28single-precision%29))
  (bind _angle_degrees (CallFunction|GetAnglefromUnitVector Position))
  (return (Math|Float|Round (/ (Math|Float|%(Float) (+ _angle_degrees InitialAngle) 3.6e+02) (/ 3.6e+02 (Math|Conversions|ToFloat(Integer) ItemCount))))))