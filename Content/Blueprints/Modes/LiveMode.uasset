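; LiveMode is the game mode for a multiplayer session with User and Observer roles, spawning desktop or VR (Vive) pawns.
; BeginPlay copies persistent user data to the game state, and logout destroys the session.
; PostLogin sorts PlayerStarts by Host tag, assigns a UserId and notifies the client controller.
; Respawn replaces the pawn, placing Users at the first Host start and Observers at Id-indexed starts, then possesses and switches technique.
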(event Custom|Respawn
  (params (User :type User%20Structure) (PlayerController :type Player%20Controller%20Object%20Reference))
  (bind (_id _name _vrenabled _userclass) (Utilities|Struct|BreakUser User))
  (bind _returnvalue (Pawn|GetControlledPawn PlayerController))
  ;[1 1 1] Respawn
  (Class|GameModeBase|GetNumPlayers)
  (Utilities|IsValid _returnvalue
    (:Is%20Valid
      (Development|PrintString (Utilities|String|Append "Destroying " (Utilities|GetObjectName _returnvalue)))
      (Actor|DestroyActor _returnvalue))
    (:Is%20Not%20Valid
      _))
  (switch Utilities|FlowControl|Switch|SwitchonUserClassEnum _userclass
    (:NewEnumerator0
      (Development|PrintString "Error! No user class"))
    (:NewEnumerator1
      (Variables|Default|SetSelectedStart (Transformation|GetActorTransform (Utilities|Array|Get(acopy) (Variables|Default|GetHost))))
      (Development|PrintString (Utilities|String|Append "Spawning " (Utilities|GetObjectName PlayerController) " " (Utilities|String|EnumtoString _userclass)) :!label _label)
      (if _vrenabled
        (bind _returnvalue_2 (Game|SpawnActorfromClass "/Game/Blueprints/Pawns/VivePawn.VivePawn_C" (Variables|Default|GetSelectedStart) "AlwaysSpawn" 0 User 0))
        (Utilities|FlowControl|Delay 0.1)
        (Pawn|Possess PlayerController _returnvalue_2)
        (bind _aslive_player_controller (Utilities|Casting|CastToLivePlayerController PlayerController))
        (Default|SwitchTechnique _aslive_player_controller "Controller" _returnvalue_2)
        (else
          (bind _returnvalue_3 (Game|SpawnActorfromClass "/Game/Blueprints/Pawns/DesktopPawn.DesktopPawn_C" (Variables|Default|GetSelectedStart) "AlwaysSpawn" 0 User 0))
          (Utilities|FlowControl|Delay 0.1)
          (Pawn|Possess PlayerController _returnvalue_3)
          (bind _aslive_player_controller_2 (Utilities|Casting|CastToLivePlayerController PlayerController))
          (Default|SwitchTechnique _aslive_player_controller_2 "Controller" _returnvalue_3)))
      (Development|PrintString (Utilities|String|Append "Possessing " (Utilities|String|ToString(Text) (Default|UserInfotoString (Utilities|LiveInstance) User)) " " (Utilities|GetObjectName PlayerController))))
    (:NewEnumerator2
      (Variables|Default|SetSelectedStart (Transformation|GetActorTransform (Utilities|Array|Get(acopy) (Variables|Default|GetUser) (- _id 1))))
      (goto _label))))

(event EventTick
  (params (DeltaSeconds :type Float%20%28single-precision%29)))

(event EventOnLogout
  (params (ExitingController :type Controller%20Object%20Reference))
  (bind _liveinstance (Utilities|LiveInstance))
  (|DestroySession
    (:OnSuccess
      (Default|LogMessage _liveinstance "LIVE" "Session destroyed."))
    (:OnFailure
      (Default|LogMessage _liveinstance "LIVE" "Failed to destroy session."))))

(event EventPostLogin
  (params (NewPlayer :type Player%20Controller%20Object%20Reference))
  ;[1 1 1] Post login
  (Development|PrintString (Utilities|String|Append (Utilities|GetObjectName NewPlayer) " joined"))
  (bind _outactors (Actor|GetAllActorsOfClass "/Script/Engine.PlayerStart"))
  (for _array_element _outactors
    (if (Utilities|Name|Equal(Name) (Variables|/Script/Engine.PlayerStart|GetPlayerStartTag _array_element) "Host")
      (Utilities|Array|AddUnique (Variables|Default|GetHost) _array_element)
      (else
        (Utilities|Array|AddUnique (Variables|Default|GetUser) _array_element))))
  (bind _aslive_player_state (Utilities|Casting|CastToLivePlayerState (Variables|/Script/Engine.Controller|GetPlayerState NewPlayer)))
  (Variables|/Game/Blueprints/Modes/LivePlayerState.LivePlayerState_C|SetUserId _aslive_player_state (- (Utilities|Array|Length (Variables|/Script/Engine.GameStateBase|GetPlayerArray (Utilities|LiveGameState))) 1))
  (bind _aslive_player_controller (Utilities|Casting|CastToLivePlayerController NewPlayer))
  (Default|ClientPostLogin _aslive_player_controller))

(event EventBeginPlay
  (Variables|/Game/Blueprints/Modes/LiveGameState.LiveGameState_C|SetUsers (Utilities|LiveGameState) (Variables|/Game/Blueprints/LiveInstance.LiveInstance_C|GetPersistentUserData (Utilities|LiveInstance))))

(fn ConstructionScript)