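; Player controller for the multiplayer lobby that handles session joins, the mini lobby screen and the loading screen.
; SessionJoined gets an ID from the game state, registers the user, shows the lobby and stores the user ID in the game instance.
; Update and load requests use Server and MultiClient events to drive game instance UI.
; A helper retries the LivePlayerState cast after a delay until it succeeds; Next and Previous are empty.
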(event Custom|ClientShowLobby
  ;[1 1 1] Show Lobby
  (Default|ShowMiniLobby (Utilities|LiveInstance)))

(event Custom|ServerNotifyLoad
  ;[1 1 1] Show loading screen to clients
  (for _array_element 0
    (CallFunction|MultiClientLoading _array_element)))

(event Custom|MultiClientLoading
  ;[1 1 1] Show loading screen to clients
  (Default|ShowLoadingScreen (Utilities|LiveInstance)))

(event Custom|ServerRequestUpdate
  ;[1 1 1] Refresh Users
  (CallFunction|MultiClientUpdate))

(event Custom|Previous)

(event Custom|SessionJoined
  (params (User :type User%20Structure))
  (bind _livegamestate (Utilities|LiveGameState))
  ;[1 1 1] Session Joined
  (bind _userout (Default|AssignId _livegamestate User))
  (Default|UserConnected _livegamestate _userout)
  (CallFunction|ClientShowLobby)
  (CallFunction|ServerRequestUpdate)
  (CallFunction|WriteId (.Id (Utilities|Struct|BreakUser User))))

(event Custom|Next)

(event Custom|MultiClientUpdate
  ;[1 1 1] Refresh Users
  (CallFunction|ClientShowLobby)
  (Default|UpdateUserList (Variables|/Game/Blueprints/LiveInstance.LiveInstance_C|GetMiniLobby (Utilities|LiveInstance))))

(event Custom|WriteId
  (params (UserId :type Integer))
  ;[1 1 1] StoreUserId
  (bind _output_get (Variables|/Game/Blueprints/LiveInstance.LiveInstance_C|SetPersistentUserId (Utilities|LiveInstance) UserId))
  (Development|PrintString (Utilities|String|Append "Writing" (Utilities|String|ToString(Integer) _output_get))))

(event EventBeginPlay)

(event EventTick
  (params (DeltaSeconds :type Float%20%28single-precision%29)))

(fn ConstructionScript)