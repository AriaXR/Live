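; Lobby game mode that launches scenarios by server-traveling to a chosen map as a listen server.
; StartScenario captures the users from the live game state before issuing the travel console command, then retries on a short delay until the game state casts to LiveGameState.
; It then stores those users and the map's scenario on the live game instance and logs the user count.
; PostLogin collects each joining player controller.
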(event Custom|Start%20Scenario
  (params (MapName :type String))
  (bind _liveinstance (Utilities|LiveInstance))
  (bind _liveinstance_2 (Utilities|LiveInstance))
  ;[1 1 1] Start Scenario
  (Variables|Default|SetUsers (Variables|/Game/Blueprints/Modes/LiveGameState.LiveGameState_C|GetUsers (Utilities|LiveGameState)))
  (Development|ExecuteConsoleCommand (Utilities|String|Append (Utilities|String|Append "ServerTravel /Game/Maps/" MapName) "?listen"))
  (Utilities|Casting|CastToLiveGameState (Game|GetGameState) :!label _label
    (:then
      (Variables|/Game/Blueprints/LiveInstance.LiveInstance_C|SetPersistentUserData _liveinstance_2 (Variables|Default|GetUsers))
      (bind _result (CallFunction|StringtoScenario MapName))
      (Variables|/Game/Blueprints/LiveInstance.LiveInstance_C|SetCurrentScenario _liveinstance _result)
      (Default|LogMessage _liveinstance "!There are " (Utilities|Text|ToText(Integer) (Utilities|Array|Length (Variables|Default|GetUsers)))))
    (:CastFailed
      (Default|LogMessage _liveinstance_2 "Travel" "Waiting...")
      (Utilities|FlowControl|Delay 0.2)
      (goto _label))))

(event EventBeginPlay)

(event EventTick
  (params (DeltaSeconds :type Float%20%28single-precision%29)))

(event EventPostLogin
  (params (NewPlayer :type Player%20Controller%20Object%20Reference))
  (Utilities|Array|Add (Variables|Default|GetPlayerControllers) NewPlayer))

(fn ConstructionScript)