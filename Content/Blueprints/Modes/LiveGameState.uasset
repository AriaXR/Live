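; Live game state that keeps the list of connected users for the live instance.
; UserConnected appends each user to the array and logs its ID, name and client total through LiveInstance.
; The Users RepNotify refreshes the MiniLobby user list, only on authority.
; Helpers derive a new user's ID from the incremented array length and fetch users by using the ID as the array index.
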(event Custom|UserConnected
  (params (User :type User%20Structure))
  (bind (_id _name) (Utilities|Struct|BreakUser User))
  (Utilities|Array|Add (Variables|Default|GetUsers) User)
  (Default|LogMessage (Utilities|LiveInstance) "UserConnected" (Utilities|Text|FormatText "Registered [{Id}]:{Name} - Total clients: {Total}" _id (Utilities|Text|ToText(String) _name) (Utilities|Array|Length (Variables|Default|GetUsers)))))

(event EventBeginPlay)

(fn ConstructionScript)

(fn OnRepUsers
  (Networking|SwitchHasAuthority
    (:Authority
      (Default|UpdateUserList (Variables|/Game/Blueprints/LiveInstance.LiveInstance_C|GetMiniLobby (Utilities|LiveInstance))))))

(fn AssignId
  (params (UserIn :type User%20Structure))
  (bind _result (Math|Integer|IncrementInt (Utilities|Array|Length (Variables|Default|GetUsers)))
    (:%20%20
      (bind _structout (Utilities|Struct|SetmembersinUser UserIn _result))
      (return _structout))))

(fn GetUser
  (params (UserId :type Integer))
  (return (Utilities|Array|Get(acopy) (Variables|Default|GetUsers) UserId)))