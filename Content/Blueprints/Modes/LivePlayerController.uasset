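; VR player controller that respawns users from persistent data at login and manages their swappable interaction techniques (pointers, hands, teleporter, WIM, UI).
; Input actions request a server switch, which spawns the technique actor on a motion controller, replacing the previous one.
; Right-hand trigger, grip and trackpad input reaches it through ITechnique, via Server events when remote, though trigger axis is called directly.
; Helper events cover server spawning and destruction, spawn notification and rumble.
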(event Custom|RumbleController
  (params (Intensity :type Float%20%28single-precision%29) (Duration :type Float%20%28single-precision%29) (VibrateLeft :type Boolean))
  (bind _returnvalue (not VibrateLeft))
  (Game|Feedback|PlayDynamicForceFeedback (Game|GetPlayerController 0) Intensity Duration VibrateLeft VibrateLeft _returnvalue _returnvalue))

(event Custom|RetrieveUser
  (params (PlayerController :type Live%20Player%20Controller%20Object%20Reference))
  (bind _liveinstance (Utilities|LiveInstance))
  (bind _aslive_player_state (Utilities|Casting|CastToLivePlayerState (Variables|GetPlayerState)))
  (Development|PrintString (Utilities|String|ToString(Integer) (Variables|/Game/Blueprints/Modes/LivePlayerState.LivePlayerState_C|GetUserId _aslive_player_state)))
  (Default|Respawn (.AsLive%20Mode (Utilities|Casting|CastToLiveMode (Game|GetGameMode))) (Utilities|Array|Get(acopy) (Variables|/Game/Blueprints/LiveInstance.LiveInstance_C|GetPersistentUserData (Utilities|LiveInstance)) (Variables|/Game/Blueprints/Modes/LivePlayerState.LivePlayerState_C|GetUserId _aslive_player_state)) PlayerController)
  (Default|LogMessage _liveinstance "I am a:" (Default|UserInfotoString _liveinstance (Utilities|Array|Get(acopy) (Variables|/Game/Blueprints/LiveInstance.LiveInstance_C|GetPersistentUserData (Utilities|LiveInstance)) (Variables|/Game/Blueprints/Modes/LivePlayerState.LivePlayerState_C|GetUserId _aslive_player_state)))))

(event Custom|ServerRTrackpad
  (bind _actortechnique (Variables|Default|GetActorTechnique))
  ;[1 1 1] RTrackpad
  (Utilities|IsValid _actortechnique
    (:Is%20Valid
      (bind _asitechnique (Utilities|Casting|CastToITechnique _actortechnique))
      (Default|RTrackpadReleased _asitechnique))))

(event Custom|ClientNotifySpawn
  (params (Actor :type Actor%20Object%20Reference))
  (Default|SetupNewActor (.AsITechnique (Utilities|Casting|CastToITechnique (Variables|Default|GetActorTechnique))) Actor))

(event Custom|ServerRTriggerPress
  (Default|RTriggerPressed (.AsITechnique (Utilities|Casting|CastToITechnique (Variables|Default|GetActorTechnique)))))

(event Custom|ServerDestroyActor
  (params (Actor :type Actor%20Object%20Reference))
  (Actor|DestroyActor Actor))

(event Custom|ServerRTrackpadUpdate
  (params (Position :type Vector%202D%20Structure))
  (bind _actortechnique (Variables|Default|GetActorTechnique))
  (Utilities|IsValid _actortechnique
    (:Is%20Valid
      (bind _asitechnique (Utilities|Casting|CastToITechnique _actortechnique))
      (Default|RTrackpadUpdate _asitechnique Position))))

(event Custom|Server%20RTriggerReleased
  (Default|RTriggerReleased (.AsITechnique (Utilities|Casting|CastToITechnique (Variables|Default|GetActorTechnique)))))

(event Custom|ServerSpawnActor
  (params (Actor%20Class :type Actor%20Class%20Reference) (Transform :type Transform) (Owner :type Actor%20Object%20Reference) (Attach :type Boolean) (IsScaleRelative :type Boolean))
  (bind _returnvalue (Game|SpawnActorfromClass Actor%20Class Transform "AlwaysSpawn" Owner 0))
  (if Attach
    (if IsScaleRelative
      (Transformation|AttachActorToActor _returnvalue Owner "None" "KeepRelative" "KeepRelative" "KeepRelative" true)
      (else
        (Transformation|AttachActorToActor _returnvalue Owner "None" "KeepRelative" "KeepRelative" "KeepWorld" true)))
    (CallFunction|ClientNotifySpawn _returnvalue)))

(event Custom|ServerRequestSwitch
  (params (Command :type String))
  (CallFunction|SwitchTechnique Command (Utilities|IPawn)))

(event Custom|ClientPostLogin
  ;[1 1 1] Client PostLogin
  (CallFunction|RetrieveUser self))

(event Custom|Server%20RGripReleased
  (bind _actortechnique (Variables|Default|GetActorTechnique))
  (Utilities|IsValid _actortechnique
    (:Is%20Valid
      (bind _asitechnique (Utilities|Casting|CastToITechnique _actortechnique))
      (Default|RGripReleased _asitechnique))))

(event EventBeginPlay)

(event Input|ActionEvents|InputActionAction
  (params (Key :type Key%20Structure :default "AnyKey"))
  ;[1 1 1] TriggerAxis
  (:Released
    (bind _asitechnique (Utilities|Casting|CastToITechnique (Variables|Default|GetActorTechnique)))
    (Default|RTriggerAxis _asitechnique 0.0)))

(event Input|ActionEvents|InputActionForceAdvance
  (params (Key :type Key%20Structure :default "AnyKey"))
  (:Released
    (Default|ForceAdvance (Utilities|LivePawn))))

(event Input|ActionEvents|InputActionAction
  (params (Key :type Key%20Structure :default "AnyKey"))
  (bind _actortechnique (Variables|Default|GetActorTechnique))
  (bind _asitechnique (Utilities|Casting|CastToITechnique _actortechnique))
  ;[1 1 1] Trigger
  (:Pressed
    (Networking|SwitchHasAuthority
      (:Authority
        (Default|RTriggerPressed _asitechnique))
      (:Remote
        (CallFunction|ServerRTriggerPress))))
  (:Released
    (Networking|SwitchHasAuthority
      (:Authority
        (Default|RTriggerReleased _asitechnique))
      (:Remote
        (CallFunction|ServerRTriggerReleased)))))

(event Input|ActionEvents|InputActionRayTechnique
  (params (Key :type Key%20Structure :default "AnyKey"))
  ;[1 1 1] Switch Techniques
  (:Released
    (CallFunction|ServerRequestSwitch "Hand")))

(event Input|ActionEvents|InputActionControllerTechnique
  (params (Key :type Key%20Structure :default "AnyKey"))
  ;[1 1 1] Switch Techniques
  (:Released
    (CallFunction|ServerRequestSwitch "Controller")))

(event Input|ActionEvents|InputActionRTrackpad
  (params (Key :type Key%20Structure :default "AnyKey"))
  (bind _actortechnique (Variables|Default|GetActorTechnique))
  ;[1 1 1] RTrackpad
  (:Released
    (Networking|SwitchHasAuthority
      (:Authority
        (Utilities|IsValid _actortechnique
          (:Is%20Valid
            (bind _asitechnique (Utilities|Casting|CastToITechnique _actortechnique))
            (Default|RTrackpadReleased _asitechnique))))
      (:Remote
        (CallFunction|ServerRTrackpad)))))

(event Input|ActionEvents|InputActionRTrackpadDown
  (params (Key :type Key%20Structure :default "AnyKey"))
  (bind _actortechnique (Variables|Default|GetActorTechnique))
  ;[1 1 1] Trackpad Update
  (:Released
    (Variables|Default|SetRThumbY -1.0)
    (Networking|SwitchHasAuthority
      (:Authority
        (Utilities|IsValid _actortechnique
          (:Is%20Valid
            (bind _asitechnique (Utilities|Casting|CastToITechnique _actortechnique))
            (Default|RTrackpadUpdate _asitechnique (Math|Vector2D|MakeVector2D (Variables|Default|GetRThumbX) (Variables|Default|GetRThumbY))))))
      (:Remote
        (CallFunction|ServerRTrackpadUpdate (Math|Vector2D|MakeVector2D (Variables|Default|GetRThumbX) (Variables|Default|GetRThumbY)))))))

(event Input|ActionEvents|InputActionRTrackpadLeft
  (params (Key :type Key%20Structure :default "AnyKey"))
  (bind _actortechnique (Variables|Default|GetActorTechnique))
  ;[1 1 1] Trackpad Update
  (:Released
    (Variables|Default|SetRThumbX -1.0)
    (Networking|SwitchHasAuthority
      (:Authority
        (Utilities|IsValid _actortechnique
          (:Is%20Valid
            (bind _asitechnique (Utilities|Casting|CastToITechnique _actortechnique))
            (Default|RTrackpadUpdate _asitechnique (Math|Vector2D|MakeVector2D (Variables|Default|GetRThumbX) (Variables|Default|GetRThumbY))))))
      (:Remote
        (CallFunction|ServerRTrackpadUpdate (Math|Vector2D|MakeVector2D (Variables|Default|GetRThumbX) (Variables|Default|GetRThumbY)))))))

(event Input|ActionEvents|InputActionTeleporter
  (params (Key :type Key%20Structure :default "AnyKey"))
  ;[1 1 1] Switch Techniques
  (:Released
    (CallFunction|ServerRequestSwitch "Teleporter")))

(event Input|ActionEvents|InputActionAction
  (params (Key :type Key%20Structure :default "AnyKey"))
  ;[1 1 1] TriggerAxis
  (:Pressed
    (bind _asitechnique (Utilities|Casting|CastToITechnique (Variables|Default|GetActorTechnique)))
    (Default|RTriggerAxis _asitechnique 1.0)))

(event Input|ActionEvents|InputActionWim
  (params (Key :type Key%20Structure :default "AnyKey"))
  ;[1 1 1] Switch Techniques
  (:Released
    (CallFunction|ServerRequestSwitch "wim")))

(event Input|ActionEvents|InputActionUFONavigator
  (params (Key :type Key%20Structure :default "AnyKey"))
  ;[1 1 1] Switch Techniques
  (:Released
    (CallFunction|ServerRequestSwitch "UI")))

(event Input|ActionEvents|InputActionRTrackpadRight
  (params (Key :type Key%20Structure :default "AnyKey"))
  (bind _actortechnique (Variables|Default|GetActorTechnique))
  ;[1 1 1] Trackpad Update
  (:Released
    (Variables|Default|SetRThumbX 1.0)
    (Networking|SwitchHasAuthority
      (:Authority
        (Utilities|IsValid _actortechnique
          (:Is%20Valid
            (bind _asitechnique (Utilities|Casting|CastToITechnique _actortechnique))
            (Default|RTrackpadUpdate _asitechnique (Math|Vector2D|MakeVector2D (Variables|Default|GetRThumbX) (Variables|Default|GetRThumbY))))))
      (:Remote
        (CallFunction|ServerRTrackpadUpdate (Math|Vector2D|MakeVector2D (Variables|Default|GetRThumbX) (Variables|Default|GetRThumbY)))))))

(event Input|ActionEvents|InputActionRTrackpadUp
  (params (Key :type Key%20Structure :default "AnyKey"))
  (bind _actortechnique (Variables|Default|GetActorTechnique))
  ;[1 1 1] Trackpad Update
  (:Released
    (Variables|Default|SetRThumbY 1.0)
    (Networking|SwitchHasAuthority
      (:Authority
        (Utilities|IsValid _actortechnique
          (:Is%20Valid
            (bind _asitechnique (Utilities|Casting|CastToITechnique _actortechnique))
            (Default|RTrackpadUpdate _asitechnique (Math|Vector2D|MakeVector2D (Variables|Default|GetRThumbX) (Variables|Default|GetRThumbY))))))
      (:Remote
        (CallFunction|ServerRTrackpadUpdate (Math|Vector2D|MakeVector2D (Variables|Default|GetRThumbX) (Variables|Default|GetRThumbY)))))))

(event Input|ActionEvents|InputActionHandTechnique
  (params (Key :type Key%20Structure :default "AnyKey"))
  ;[1 1 1] Switch Techniques
  (:Released
    (CallFunction|ServerRequestSwitch "GoGo")))

(event Input|ActionEvents|InputActionRGrip
  (params (Key :type Key%20Structure :default "AnyKey"))
  (bind _actortechnique (Variables|Default|GetActorTechnique))
  (:Released
    (Networking|SwitchHasAuthority
      (:Authority
        (Utilities|IsValid _actortechnique
          (:Is%20Valid
            (bind _asitechnique (Utilities|Casting|CastToITechnique _actortechnique))
            (Default|RGripReleased _asitechnique))))
      (:Remote
        (CallFunction|ServerRGripReleased)))))

(event Input|KeyboardEvents|MotionControllerRightThumbstickX
  (params (AxisValue :type Float%20%28single-precision%29))
  (bind _actortechnique (Variables|Default|GetActorTechnique))
  ;[1 1 1] Trackpad Update
  (Variables|Default|SetRThumbX AxisValue)
  (Networking|SwitchHasAuthority
    (:Authority
      (Utilities|IsValid _actortechnique
        (:Is%20Valid
          (bind _asitechnique (Utilities|Casting|CastToITechnique _actortechnique))
          (Default|RTrackpadUpdate _asitechnique (Math|Vector2D|MakeVector2D (Variables|Default|GetRThumbX) (Variables|Default|GetRThumbY))))))
    (:Remote
      (CallFunction|ServerRTrackpadUpdate (Math|Vector2D|MakeVector2D (Variables|Default|GetRThumbX) (Variables|Default|GetRThumbY))))))

(event Input|KeyboardEvents|MotionControllerRightTriggerAxis
  (params (AxisValue :type Float%20%28single-precision%29))
  ;[1 1 1] TriggerAxis
  (Utilities|IsValid 0
    (:Is%20Valid
      (bind _asitechnique (Utilities|Casting|CastToITechnique (Variables|Default|GetActorTechnique)))
      (Default|RTriggerAxis _asitechnique AxisValue))))

(event Input|KeyboardEvents|MotionControllerRightThumbstickY
  (params (AxisValue :type Float%20%28single-precision%29))
  (bind _actortechnique (Variables|Default|GetActorTechnique))
  ;[1 1 1] Trackpad Update
  (Variables|Default|SetRThumbY AxisValue)
  (Networking|SwitchHasAuthority
    (:Authority
      (Utilities|IsValid _actortechnique
        (:Is%20Valid
          (bind _asitechnique (Utilities|Casting|CastToITechnique _actortechnique))
          (Default|RTrackpadUpdate _asitechnique (Math|Vector2D|MakeVector2D (Variables|Default|GetRThumbX) (Variables|Default|GetRThumbY))))))
    (:Remote
      (CallFunction|ServerRTrackpadUpdate (Math|Vector2D|MakeVector2D (Variables|Default|GetRThumbX) (Variables|Default|GetRThumbY))))))

(event Input|KeyboardEvents|MotionControllerRightTrigger
  (params (Key :type Key%20Structure :default "AnyKey"))
  (bind _actortechnique (Variables|Default|GetActorTechnique))
  (bind _asitechnique (Utilities|Casting|CastToITechnique _actortechnique))
  ;[1 1 1] Trigger
  (:Pressed
    (Networking|SwitchHasAuthority
      (:Authority
        (Default|RTriggerPressed _asitechnique))
      (:Remote
        (CallFunction|ServerRTriggerPress))))
  (:Released
    (Networking|SwitchHasAuthority
      (:Authority
        (Default|RTriggerReleased _asitechnique))
      (:Remote
        (CallFunction|ServerRTriggerReleased)))))

(event Input|KeyboardEvents|MotionControllerRightGrip1
  (params (Key :type Key%20Structure :default "AnyKey"))
  (bind _actortechnique (Variables|Default|GetActorTechnique))
  (:Released
    (Networking|SwitchHasAuthority
      (:Authority
        (Utilities|IsValid _actortechnique
          (:Is%20Valid
            (bind _asitechnique (Utilities|Casting|CastToITechnique _actortechnique))
            (Default|RGripReleased _asitechnique))))
      (:Remote
        (CallFunction|ServerRGripReleased)))))

(event Input|KeyboardEvents|MotionControllerRightGrip2
  (params (Key :type Key%20Structure :default "AnyKey"))
  (bind _actortechnique (Variables|Default|GetActorTechnique))
  (:Released
    (Networking|SwitchHasAuthority
      (:Authority
        (Utilities|IsValid _actortechnique
          (:Is%20Valid
            (bind _asitechnique (Utilities|Casting|CastToITechnique _actortechnique))
            (Default|RGripReleased _asitechnique))))
      (:Remote
        (CallFunction|ServerRGripReleased)))))

(event Input|KeyboardEvents|MotionControllerRightThumbstick
  (params (Key :type Key%20Structure :default "AnyKey"))
  (bind _actortechnique (Variables|Default|GetActorTechnique))
  ;[1 1 1] RTrackpad
  (:Released
    (Networking|SwitchHasAuthority
      (:Authority
        (Utilities|IsValid _actortechnique
          (:Is%20Valid
            (bind _asitechnique (Utilities|Casting|CastToITechnique _actortechnique))
            (Default|RTrackpadReleased _asitechnique))))
      (:Remote
        (CallFunction|ServerRTrackpad)))))

(fn ConstructionScript)

(fn SwitchTechnique
  (params (Command :type String) (Pawn :type I%20Pawn%20Interface))
  (switch string Command
    (:Default
      (Variables|Default|SetClassType "/Game/Blueprints/Techniques/Controller.Controller_C"))
    (:Ray
      (Variables|Default|SetClassType "/Game/Blueprints/Techniques/RayPointer.RayPointer_C"))
    (:Cone
      (Variables|Default|SetClassType "/Game/Blueprints/Techniques/ConePointer.ConePointer_C"))
    (:Hand
      (Variables|Default|SetClassType "/Game/Blueprints/Techniques/HandController.HandController_C"))
    (:RayManipulator
      (Variables|Default|SetClassType "/Game/Blueprints/Techniques/RayManipulator.RayManipulator_C"))
    (:GoGo
      (Variables|Default|SetClassType "/Game/Blueprints/Techniques/GoGoController.GoGoController_C"))
    (:Shape
      (Variables|Default|SetClassType "/Game/Blueprints/Techniques/ShapeRadialMenu.ShapeRadialMenu_C"))
    (:Teleporter
      (Variables|Default|SetClassType "/Game/Blueprints/Techniques/Teleporter.Teleporter_C"))
    (:Wim
      (Variables|Default|SetClassType "/Game/Blueprints/Techniques/WorldInMiniature.WorldInMiniature_C"))
    (:UI
      (Variables|Default|SetClassType "/Game/Blueprints/Techniques/UIController.UIController_C"))
    (:dummyWim
      (Variables|Default|SetClassType "/Game/Blueprints/Actors/DummyWIM.DummyWIM_C")))
  (bind _returnvalue (Game|SpawnActorfromClass (Variables|Default|GetClassType) (Math|Transform|MakeTransform "0, 0, 0") "AlwaysSpawn" (.AsActor (Utilities|Casting|CastToActor Pawn)) 0))
  (CallFunction|AttachActortoController _returnvalue "NewEnumerator1" Pawn)
  (Variables|Default|SetActorTechnique _returnvalue))

(fn AttachActortoController
  (params (Actor :type Actor%20Object%20Reference) (Hand :type ViveControllerEnum%20Enum) (Pawn :type I%20Pawn%20Interface))
  (LocalVariables|SetNew%20Actor Actor)
  (bind _motioncontroller (Default|GetMotionController Pawn Hand))
  (Utilities|FlowControl|Sequence
    (:then_0
      (bind _output_get (LocalVariables|SetParent%20Component _motioncontroller)))
    (:then_1
      (bind _array_element (Utilities|Array|ForEachLoopwithBreak (Components|GetChildrenComponents _motioncontroller true) :!label _label)
        (:LoopBody
          (if (Utilities|DoesObjectImplementInterface (Components|GetOwner _array_element) "/Game/Blueprints/Techniques/ITechnique.ITechnique_C")
            (Actor|DestroyActor (Components|GetOwner _array_element))
            (goto _label Break)))))
    (:then_2
      (Transformation|AttachComponentToComponent (LocalVariables|GetNew%20Actor) _output_get "None" "KeepRelative" "KeepRelative" "KeepRelative" true))))