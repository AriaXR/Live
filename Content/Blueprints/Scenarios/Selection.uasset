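; Scenario logic for a step-by-step lesson teaching 3D selection by ray-casting and bounding boxes, with local and multi variants.
; Functions switch on a step index to set narrated info text, create Level Sequence players and return advance checks with wait delays.
; Step functions toggle target selectability and switch users to the Ray technique by role.
; The final hands-on check looks for a target whose bounding box has been displayed.
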(fn SelectionStepLocal
  (params (Step :type Integer))
  (switch int Step
    (:0
      (Utilities|FlowControl|Sequence
        (:then_0
          ;[1 1 1] Disable Arrow
          (bind _outactors (Actor|GetAllActorswithInterface 0 "/Game/Blueprints/Pawns/IPawn.IPawn_C"))
          (for _array_element _outactors
            (bind _arrow (Class|IPawn|GetArrow(Message) _array_element))
            (Rendering|SetActorHiddenInGame _arrow true)))
        (:then_1
          ;[1 1 1] Show Targets
          (bind _outactors_2 (Actor|GetAllActorsOfClass 0 "/Game/Blueprints/Actors/TestActor.TestActor_C"))
          (for _array_element_2 _outactors_2
            (Variables|/Game/Blueprints/Actors/TestActor.TestActor_C|SetIsSelectionEnabled _array_element_2 true)))))
    (:1
      ;[1 1 1] Make targets selectable
      (bind _outactors_3 (Actor|GetAllActorsOfClass 0 "/Game/Blueprints/Actors/TestActor.TestActor_C"))
      (for _array_element_3 _outactors_3
        (Variables|/Game/Blueprints/Actors/TestActor.TestActor_C|SetIsSelectionEnabled _array_element_3 false)))
    (:2
      (Utilities|FlowControl|Sequence
        (:then_0
          ;[1 1 1] Enable target selection and make them visible
          (bind _outactors_4 (Actor|GetAllActorswithTag 0 "ExampleTarget"))
          (for _array_element_4 _outactors_4
            (bind _astest_actor (Utilities|Casting|CastToTestActor _array_element_4))
            (Variables|/Game/Blueprints/Actors/TestActor.TestActor_C|SetIsSelectionEnabled _astest_actor true))
          ;[1 1 1] Disable ray
          (bind _outactors_5 (Actor|GetAllActorsOfClass 0 "/Game/Blueprints/Actors/DummyRayPointer.DummyRayPointer_C"))
          (Default|ToggleRayVisibility (Utilities|Array|Get(acopy) _outactors_5)))
        (:then_1
          ;[1 1 1] Switch off controller light
          (bind _actor (CallFunction|GetActorOfType "/Game/Blueprints/Actors/DummyRayPointer.DummyRayPointer_C"))
          (bind _asdummy_ray_pointer (Utilities|Casting|CastToDummyRayPointer _actor))
          (Default|ToggleLight _asdummy_ray_pointer))))
    (:6
      (Utilities|FlowControl|Sequence
        (:then_0
          (CallFunction|SwitchTechniqueifRole "Ray" "NewEnumerator1"))
        (:then_1
          (bind _outactors_6 (Actor|GetAllActorsOfClass 0 "/Game/Blueprints/Actors/TestActor.TestActor_C"))
          (for _array_element_5 _outactors_6
            (Variables|/Game/Blueprints/Actors/TestActor.TestActor_C|SetIsSelectionEnabled _array_element_5 true)))))))

(fn CreateSelectionAnimationStep
  (params (Step :type Integer))
  (switch int Step
    (:0
      (bind _returnvalue (Sequencer|Player|CreateLevelSequencePlayer 0 "/Game/Assets/Animations/SelectionStep1.SelectionStep1"))
      (return _returnvalue))
    (:1
      (bind _returnvalue_2 (Sequencer|Player|CreateLevelSequencePlayer 0 "/Game/Assets/Animations/SelectionStep2.SelectionStep2"))
      (return _returnvalue_2))
    (:2
      _)
    (:3
      (bind _returnvalue_3 (Sequencer|Player|CreateLevelSequencePlayer 0 "/Game/Assets/Animations/SelectionStep3.SelectionStep3"))
      (return _returnvalue_3))
    (:4
      (bind _returnvalue_4 (Sequencer|Player|CreateLevelSequencePlayer 0 "/Game/Assets/Animations/SelectionStep4.SelectionStep4"))
      (return _returnvalue_4))
    (:5
      (bind _returnvalue_5 (Sequencer|Player|CreateLevelSequencePlayer 0 "/Game/Assets/Animations/SelectionStep5.SelectionStep5"))
      (return _returnvalue_5))
    (:6
      (bind _returnvalue_6 (Sequencer|Player|CreateLevelSequencePlayer 0 "/Game/Assets/Animations/SelectionStep6.SelectionStep6"))
      (return _returnvalue_6))
    (:7
      _))
  (return 0))

(fn SelectionCheck
  (params (Step :type Integer) (Pawn :type I%20Pawn%20Interface))
  (switch int Step
    (:0
      (bind _canprogress (Default|CheckArrow Pawn))
      (return _canprogress 0.0))
    (:1
      (return true 1e+01))
    (:2
      (return true 9.0))
    (:3
      (return true 9.0))
    (:4
      (return true 1e+01))
    (:5
      (return true 8.0))
    (:6
      (return true 8.0))
    (:7
      (bind _outactors (Actor|GetAllActorsOfClass 0 "/Game/Blueprints/Actors/TestActor.TestActor_C"))
      (for _array_element _outactors
        (if (>= (Variables|/Game/Blueprints/Actors/TestActor.TestActor_C|GetBBTimesDisplayed _array_element) 1)
          (return true 1.0))))
    (:8
      (return _canprogress 0.0))))

(fn SetSelectionInfoStep
  (params (Widget :type Widget%20Object%20Reference) (Step :type Integer) (Pawn :type I%20Pawn%20Interface))
  (bind _output_get (LocalVariables|SetTargetPawn Pawn))
  (Default|HideAdvance _output_get)
  (LocalVariables|SetInfoBox (.AsInfo%20Box (Utilities|Casting|CastToInfoBox Widget)))
  (switch int Step
    (:0
      (Rendering|Components|TextRender|SetText (Variables|/Game/Blueprints/UserInterface/InfoBox.InfoBox_C|GetDescription (LocalVariables|GetInfoBox)) "Selection is one of the fundamental tasks of 3D Interaction. It allows users to indicate objects with which they wish to interact.")
      (LocalVariables|SetSoundClip "/Game/Assets/Sound/Sel01.Sel01")
      (Default|ShowInfowithDelay (LocalVariables|GetTargetPawn) 3.0 (LocalVariables|GetSoundClip) :!label _label))
    (:1
      (Default|HideInfo (LocalVariables|GetTargetPawn))
      (Rendering|Components|TextRender|SetText (Variables|/Game/Blueprints/UserInterface/InfoBox.InfoBox_C|GetDescription (LocalVariables|GetInfoBox)) "To select an object in 3D we need a pointing device, such as a controller.")
      (LocalVariables|SetSoundClip "/Game/Assets/Sound/Sel02.Sel02")
      (Default|ShowInfowithDelay (LocalVariables|GetTargetPawn) 5.0 (LocalVariables|GetSoundClip)))
    (:2
      (Default|HideInfo (LocalVariables|GetTargetPawn))
      (Rendering|Components|TextRender|SetText (Variables|/Game/Blueprints/UserInterface/InfoBox.InfoBox_C|GetDescription (LocalVariables|GetInfoBox)) "Ray-casting refers to using the orientation of the controller to determine a ray. If the ray intersects the 3D object, it becomes selected.")
      (LocalVariables|SetSoundClip "/Game/Assets/Sound/Sel03.Sel03")
      (goto _label))
    (:3
      (Default|HideInfo (LocalVariables|GetTargetPawn))
      (Rendering|Components|TextRender|SetText (Variables|/Game/Blueprints/UserInterface/InfoBox.InfoBox_C|GetDescription (LocalVariables|GetInfoBox)) "What happens if the orientation changes? 
 
In this case, even though the ray does not intersect the Pyramid, it is still considered to be selected.")
      (LocalVariables|SetSoundClip "/Game/Assets/Sound/Sel04.Sel04")
      (Default|ChangeDescriptionFontSize (LocalVariables|GetInfoBox) 38)
      (goto _label))
    (:4
      (Default|HideInfo (LocalVariables|GetTargetPawn))
      (Rendering|Components|TextRender|SetText (Variables|/Game/Blueprints/UserInterface/InfoBox.InfoBox_C|GetDescription (LocalVariables|GetInfoBox)) "In order to simplify calculations, in this case the check happens between the ray and a Bounding Box.")
      (LocalVariables|SetSoundClip "/Game/Assets/Sound/Sel05.Sel05")
      (Default|ChangeDescriptionFontSize (LocalVariables|GetInfoBox) 40)
      (goto _label))
    (:5
      (Default|HideInfo (LocalVariables|GetTargetPawn))
      (Rendering|Components|TextRender|SetText (Variables|/Game/Blueprints/UserInterface/InfoBox.InfoBox_C|GetDescription (LocalVariables|GetInfoBox)) "In general, various bounding objects are used such as spheres, capsules, or hierarchies of objects.")
      (LocalVariables|SetSoundClip "/Game/Assets/Sound/Sel06.Sel06")
      (goto _label))
    (:6
      (Default|HideInfo (LocalVariables|GetTargetPawn))
      (Rendering|Components|TextRender|SetText (Variables|/Game/Blueprints/UserInterface/InfoBox.InfoBox_C|GetDescription (LocalVariables|GetInfoBox)) "Try experimenting now! Targets will be highlighted when selected. The trigger displays the bounding box. Once you have selected an object, press \"Next\".")
      (LocalVariables|SetSoundClip "/Game/Assets/Sound/Sel07.Sel07")
      (goto _label))
    (:7
      (Default|HideInfo (LocalVariables|GetTargetPawn))
      (Rendering|Components|TextRender|SetText (Variables|/Game/Blueprints/UserInterface/InfoBox.InfoBox_C|GetDescription (LocalVariables|GetInfoBox)) "This concludes this lesson!")
      (LocalVariables|SetSoundClip "/Game/Assets/Sound/LectureOver.LectureOver")
      (Default|ShowInfowithDelay (LocalVariables|GetTargetPawn) 3.0 (LocalVariables|GetSoundClip))))
  (return true))

(fn SelectionStepMulti
  (params (Step :type Integer))
  (switch int Step
    (:0
      (Utilities|FlowControl|Sequence
        (:then_0
          ;[1 1 1] Disable Arrow
          (bind _outactors (Actor|GetAllActorswithInterface 0 "/Game/Blueprints/Pawns/IPawn.IPawn_C"))
          (for _array_element _outactors
            (bind _arrow (Class|IPawn|GetArrow(Message) _array_element))
            (Rendering|SetActorHiddenInGame _arrow true)))
        (:then_1
          ;[1 1 1] Show Targets
          (bind _outactors_2 (Actor|GetAllActorsOfClass 0 "/Game/Blueprints/Actors/TestActor.TestActor_C"))
          (for _array_element_2 _outactors_2
            (Variables|/Game/Blueprints/Actors/TestActor.TestActor_C|SetIsSelectionEnabled _array_element_2 true)))))
    (:1
      (Utilities|FlowControl|Sequence
        (:then_0
          ;[1 1 1] Make targets selectable
          (bind _outactors_3 (Actor|GetAllActorsOfClass 0 "/Game/Blueprints/Actors/TestActor.TestActor_C"))
          (for _array_element_3 _outactors_3
            (Variables|/Game/Blueprints/Actors/TestActor.TestActor_C|SetIsSelectionEnabled _array_element_3 false)))
        (:then_1
          (CallFunction|SwitchTechniqueifRole "Ray" "NewEnumerator2"))))
    (:2
      (Utilities|FlowControl|Sequence
        (:then_0
          ;[1 1 1] Enable target selection and make them visible
          (bind _outactors_4 (Actor|GetAllActorswithTag 0 "ExampleTarget"))
          (for _array_element_4 _outactors_4
            (bind _astest_actor (Utilities|Casting|CastToTestActor _array_element_4))
            (Variables|/Game/Blueprints/Actors/TestActor.TestActor_C|SetIsSelectionEnabled _astest_actor true)))))
    (:6
      (Utilities|FlowControl|Sequence
        (:then_0
          (CallFunction|SwitchTechniqueifRole "Ray" "NewEnumerator1"))
        (:then_1
          (bind _outactors_5 (Actor|GetAllActorsOfClass 0 "/Game/Blueprints/Actors/TestActor.TestActor_C"))
          (for _array_element_5 _outactors_5
            (Variables|/Game/Blueprints/Actors/TestActor.TestActor_C|SetIsSelectionEnabled _array_element_5 true)))))))

(fn CreateSelectionAnimationMulti
  (params (Step :type Integer))
  (switch int Step
    (:0
      (bind _returnvalue (Sequencer|Player|CreateLevelSequencePlayer 0 "/Game/Assets/Animations/SelectionStep1.SelectionStep1"))
      (return _returnvalue))
    (:2
      _)
    (:4
      (bind _returnvalue_2 (Sequencer|Player|CreateLevelSequencePlayer 0 "/Game/Assets/Animations/SelectionStep4.SelectionStep4"))
      (return _returnvalue_2))
    (:5
      (bind _returnvalue_3 (Sequencer|Player|CreateLevelSequencePlayer 0 "/Game/Assets/Animations/SelectionStep5.SelectionStep5"))
      (return _returnvalue_3))
    (:6
      (bind _returnvalue_4 (Sequencer|Player|CreateLevelSequencePlayer 0 "/Game/Assets/Animations/SelectionStep6.SelectionStep6"))
      (return _returnvalue_4))
    (:7
      _))
  (return 0))