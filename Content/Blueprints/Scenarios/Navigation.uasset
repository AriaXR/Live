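; Step-driven scenario logic for a VR lesson teaching three navigation techniques: on-rails UFO ride, teleport through a coin-marked maze, and World in Miniature.
; Parallel functions switch on step index to set up actors and techniques, create sequence players, gate progress with checks and delays, and show narrated InfoBox text.
; Local and Multi variants differ in demo sequence and user-role targeting, with Multi also switching a second role's technique.
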(fn NavigationLocal
  (params (Step :type Integer))
  (switch int Step
    (:0
      (Utilities|FlowControl|Sequence
        (:then_0
          ;[1 1 1] Disable Arrow
          (bind _outactors (Actor|GetAllActorswithInterface 0 "/Game/Blueprints/Pawns/IPawn.IPawn_C"))
          (for _array_element _outactors
            (bind _arrow (Class|IPawn|GetArrow(Message) _array_element))
            (Rendering|SetActorHiddenInGame _arrow true)))))
    (:2
      ;[1 1 1] Spawn "on rails" UFO technique
      (bind _player_controller (CallFunction|GetPlayerController "NewEnumerator1"))
      (Default|ServerSpawnActor _player_controller "/Game/Blueprints/Actors/UFONavigator.UFONavigator_C" (Math|Transform|MakeTransform "0,0.000000,0.000000" "0.000000, 0, 0") 0 false false))
    (:3
      (Utilities|FlowControl|Sequence
        (:then_0
          ;[1 0.6269 0.3385] Activate Labyrinth Waypoints
          (CallFunction|SetAllActorsVisibility true "Labyrinth")
          (bind _outactors_2 (Actor|GetAllActorsOfClass 0 "/Game/Blueprints/Actors/LabyrinthWaypoint.LabyrinthWaypoint_C"))
          (for _array_element_2 _outactors_2
            (Rendering|SetActorHiddenInGame _array_element_2 false)
            (Variables|/Game/Blueprints/Actors/LabyrinthWaypoint.LabyrinthWaypoint_C|SetbActive _array_element_2 true)))
        (:then_1
          ;[1 0.6269 0.3385] Re-enable arrow and point it towards first waypoint
          (bind _found_pawns (CallFunction|GetAllPawnsbyUserClass "NewEnumerator1"))
          (bind _arrow_2 (Default|GetArrow (Utilities|Array|Get(acopy) _found_pawns)))
          (Rendering|SetActorHiddenInGame _arrow_2 false))
        (:then_2
          (bind _outactors_3 (Actor|GetAllActorswithTag 0 "LabStart"))
          (Default|PointTowards _arrow_2 (Utilities|Array|Get(acopy) _outactors_3)))
        (:then_3
          ;[1 0.6269 0.3385] Switch to Teleporter technique
          (CallFunction|SwitchTechniqueifRole "Teleporter" "NewEnumerator1")
          (bind _outactors_4 (Actor|GetAllActorswithTag 0 "TeleportLocation")))
        (:then_4
          ;[1 0.6269 0.3385] Remove UFOs
          (bind _outactors_5 (Actor|GetAllActorswithTag 0 "UFO"))
          (bind _player_controller_2 (CallFunction|GetPlayerController "NewEnumerator1"))
          (for _array_element_3 _outactors_5
            (Default|ServerDestroyActor _player_controller_2 _array_element_3)))))
    (:4
      (Utilities|FlowControl|Sequence
        (:then_0
          ;[1 1 1] Switch to World-in-Miniature
          (CallFunction|SwitchTechniqueifRole "dummyWim" "NewEnumerator1"))
        (:then_1
          (bind _outactors_6 (Actor|GetAllActorsOfClass 0 "/Game/Blueprints/Actors/LabyrinthWaypoint.LabyrinthWaypoint_C"))
          (for _array_element_4 _outactors_6
            (Default|Reset _array_element_4)))))
    (:5
      (CallFunction|SwitchTechniqueifRole "wim" "NewEnumerator1"))))

(fn CreateNavigationAnimationStep
  (params (Step :type Integer))
  (switch int Step
    (:1
      (bind _returnvalue (Sequencer|Player|CreateLevelSequencePlayer 0 "/Game/Assets/Animations/NavigationStep1a.NavigationStep1a"))
      (return _returnvalue))
    (:3
      (bind _returnvalue_2 (Sequencer|Player|CreateLevelSequencePlayer 0 "/Game/Assets/Animations/NavigationStep2.NavigationStep2"))
      (return _returnvalue_2))))

(fn NavigationCheck
  (params (Step :type Integer) (Pawn :type I%20Pawn%20Interface))
  (switch int Step
    (:0
      (bind _canprogress (Default|CheckArrow Pawn))
      (return _canprogress 0.0))
    (:1
      (return true 7.0))
    (:2
      (return true 11.0))
    (:3
      (return true 23.0))
    (:4
      _)
    (:5
      (bind _outactors (Actor|GetAllActorsOfClass 0 "/Game/Blueprints/Actors/DummyWIM.DummyWIM_C"))
      (return (Variables|/Game/Blueprints/Actors/DummyWIM.DummyWIM_C|GetbPlayed (Utilities|Array|Get(acopy) _outactors)) 1e+01))
    (:6
      _))
  (bind _outactors_2 (Actor|GetAllActorsOfClass 0 "/Game/Blueprints/Actors/LabyrinthWaypoint.LabyrinthWaypoint_C"))
  (LocalVariables|SetwpCount 0)
  (for _array_element _outactors_2
    (if (Variables|/Game/Blueprints/Actors/LabyrinthWaypoint.LabyrinthWaypoint_C|GetbIsReached _array_element)
      (Math|Integer|IncrementInt (LocalVariables|GetwpCount))))
  (return (> (LocalVariables|GetwpCount) 0) 0.0))

(fn SetNavigationInfoStep
  (params (Widget :type Widget%20Object%20Reference) (Step :type Integer) (Pawn :type I%20Pawn%20Interface))
  (bind _output_get (LocalVariables|SetTargetPawn Pawn))
  (Default|HideAdvance _output_get)
  (bind _asinfo_box (Utilities|Casting|CastToInfoBox Widget))
  (LocalVariables|SetInfoBox _asinfo_box)
  (switch int Step
    (:0
      (Rendering|Components|TextRender|SetText (Variables|/Game/Blueprints/UserInterface/InfoBox.InfoBox_C|GetDescription (LocalVariables|GetInfoBox)) "Navigation techniques allow users to move in 3D Virtual Environments. We will demonstrate three different approaches.")
      (LocalVariables|SetSoundClip "/Game/Assets/Sound/Nav01.Nav01")
      (Default|ShowInfowithDelay (LocalVariables|GetTargetPawn) 0.0 (LocalVariables|GetSoundClip)))
    (:1
      (Default|HideInfo (LocalVariables|GetTargetPawn))
      (Rendering|Components|TextRender|SetText (Variables|/Game/Blueprints/UserInterface/InfoBox.InfoBox_C|GetDescription (LocalVariables|GetInfoBox)) "The first, is commonly referred to as \"on rails\" navigation, where the user is moved through a pre-defined path.  
 
Press \"Next\" to start the ride!")
      (LocalVariables|SetSoundClip "/Game/Assets/Sound/Nav02.Nav02")
      (Default|ChangeDescriptionFontSize (LocalVariables|GetInfoBox) 38)
      (Default|ShowInfowithDelay (LocalVariables|GetTargetPawn) 3.0 (LocalVariables|GetSoundClip)))
    (:2
      (Default|HideInfo (LocalVariables|GetTargetPawn))
      (Rendering|Components|TextRender|SetText (Variables|/Game/Blueprints/UserInterface/InfoBox.InfoBox_C|GetDescription (LocalVariables|GetInfoBox)) "The second technique allows you to \"jump\" to a new location using your right controller. Press \"next\" to see a demonstration.")
      (LocalVariables|SetSoundClip "/Game/Assets/Sound/Nav03.Nav03")
      (Default|ChangeDescriptionFontSize (LocalVariables|GetInfoBox) 40)
      (Default|ShowInfowithDelay (LocalVariables|GetTargetPawn) 17.0 (LocalVariables|GetSoundClip)))
    (:3
      (Default|HideInfo (LocalVariables|GetTargetPawn))
      (Rendering|Components|TextRender|SetText (Variables|/Game/Blueprints/UserInterface/InfoBox.InfoBox_C|GetDescription (LocalVariables|GetInfoBox)) "Pressing the trigger will show your teleport destination. You can use your wrist to change your orientation. You can only teleport within the range showed by the controller. 
 
See if you can exit this maze! The arrow will give you hints on the right direction. Reach the yellow coins to get more hints.")
      (LocalVariables|SetSoundClip "/Game/Assets/Sound/Nav04.Nav04")
      (Default|ChangeDescriptionFontSize (LocalVariables|GetInfoBox) 30)
      (Default|ShowInfowithDelay (LocalVariables|GetTargetPawn) 4.0 (LocalVariables|GetSoundClip)))
    (:4
      (Default|HideInfo (LocalVariables|GetTargetPawn))
      (Rendering|Components|TextRender|SetText (Variables|/Game/Blueprints/UserInterface/InfoBox.InfoBox_C|GetDescription (LocalVariables|GetInfoBox)) "The final technique is called the \"World in Miniature\". Press the RIGHT trigger to play an animation showing how it works.  
 
Your controller displays a miniature version of the world where the blue indicator shows your current location and the yellow indicator shows your teleport target. When you are ready, press \"next\".")
      (LocalVariables|SetSoundClip "/Game/Assets/Sound/Nav05.Nav05")
      (Default|ChangeDescriptionFontSize (LocalVariables|GetInfoBox) 30)
      (Default|ShowInfowithDelay (LocalVariables|GetTargetPawn) 1.0 (LocalVariables|GetSoundClip) :!label _label))
    (:5
      (Default|HideInfo (LocalVariables|GetTargetPawn))
      (Rendering|Components|TextRender|SetText (Variables|/Game/Blueprints/UserInterface/InfoBox.InfoBox_C|GetDescription (LocalVariables|GetInfoBox)) "Use the RIGHT trackpad to choose your teleport target and then press the trigger to teleport. Use your head to change the destination orientation. 
 
See if you can find the coins again!")
      (LocalVariables|SetSoundClip "/Game/Assets/Sound/Nav06.Nav06")
      (Default|ChangeDescriptionFontSize (LocalVariables|GetInfoBox) 40)
      (goto _label))
    (:6
      (Default|HideInfo (LocalVariables|GetTargetPawn))
      (Rendering|Components|TextRender|SetText (Variables|/Game/Blueprints/UserInterface/InfoBox.InfoBox_C|GetDescription (LocalVariables|GetInfoBox)) "This concludes this lesson.")
      (LocalVariables|SetSoundClip "/Game/Assets/Sound/LectureOver.LectureOver")
      (goto _label)))
  (return true))

(fn NavigationMulti
  (params (Step :type Integer))
  (switch int Step
    (:0
      (Utilities|FlowControl|Sequence
        (:then_0
          ;[1 1 1] Disable Arrow
          (bind _outactors (Actor|GetAllActorswithInterface 0 "/Game/Blueprints/Pawns/IPawn.IPawn_C"))
          (for _array_element _outactors
            (bind _arrow (Class|IPawn|GetArrow(Message) _array_element))
            (Rendering|SetActorHiddenInGame _arrow true)))))
    (:2
      (Utilities|FlowControl|Sequence
        (:then_0
          ;[1 1 1] Spawn "on rails" UFO technique
          (bind _player_controller (CallFunction|GetPlayerController "NewEnumerator1"))
          (Default|ServerSpawnActor _player_controller "/Game/Blueprints/Actors/UFONavigator.UFONavigator_C" (Math|Transform|MakeTransform "0,0.000000,0.000000" "0.000000, 0, 0") 0 false false))
        (:then_1
          (CallFunction|SwitchTechniqueifRole "Teleporter" "NewEnumerator2"))))
    (:3
      (Utilities|FlowControl|Sequence
        (:then_0
          ;[1 0.6269 0.3385] Activate Labyrinth Waypoints
          (CallFunction|SetAllActorsVisibility true "Labyrinth")
          (bind _outactors_2 (Actor|GetAllActorsOfClass 0 "/Game/Blueprints/Actors/LabyrinthWaypoint.LabyrinthWaypoint_C"))
          (for _array_element_2 _outactors_2
            (Rendering|SetActorHiddenInGame _array_element_2 false)
            (Variables|/Game/Blueprints/Actors/LabyrinthWaypoint.LabyrinthWaypoint_C|SetbActive _array_element_2 true)))
        (:then_1
          ;[1 0.6269 0.3385] Re-enable arrow and point it towards first waypoint
          (bind _found_pawns (CallFunction|GetAllPawnsbyUserClass "NewEnumerator1"))
          (bind _arrow_2 (Default|GetArrow (Utilities|Array|Get(acopy) _found_pawns)))
          (Rendering|SetActorHiddenInGame _arrow_2 false))
        (:then_2
          (bind _outactors_3 (Actor|GetAllActorswithTag 0 "LabStart"))
          (Default|PointTowards _arrow_2 (Utilities|Array|Get(acopy) _outactors_3)))
        (:then_3
          ;[1 0.6269 0.3385] Switch to Teleporter technique
          (CallFunction|SwitchTechniqueifRole "Teleporter" "NewEnumerator1"))
        (:then_4
          ;[1 0.6269 0.3385] Remove UFOs
          (bind _outactors_4 (Actor|GetAllActorswithTag 0 "UFO"))
          (bind _player_controller_2 (CallFunction|GetPlayerController "NewEnumerator0"))
          (for _array_element_3 _outactors_4
            (Default|ServerDestroyActor _player_controller_2 _array_element_3)))))
    (:4
      (Utilities|FlowControl|Sequence
        (:then_0
          ;[1 1 1] Switch to World-in-Miniature
          (CallFunction|SwitchTechniqueifRole "wim" "NewEnumerator2"))
        (:then_1
          (bind _outactors_5 (Actor|GetAllActorsOfClass 0 "/Game/Blueprints/Actors/LabyrinthWaypoint.LabyrinthWaypoint_C"))
          (for _array_element_4 _outactors_5
            (Default|Reset _array_element_4)))))
    (:5
      (CallFunction|SwitchTechniqueifRole "wim" "NewEnumerator1"))))

(fn CreateNavigationAnimationMulti
  (params (Step :type Integer))
  (switch int Step
    (:1
      (bind _returnvalue (Sequencer|Player|CreateLevelSequencePlayer 0 "/Game/Assets/Animations/NavigationStep1a.NavigationStep1a"))
      (return _returnvalue))
    (:3
      (bind _returnvalue_2 (Sequencer|Player|CreateLevelSequencePlayer 0 "/Game/Assets/Animations/NavigationStep2multi.NavigationStep2multi"))
      (return _returnvalue_2))))