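; Scenario logic for a VR lesson on System-Control techniques, teaching radial, object-based contextual and world-based 3D menus.
; Step-indexed functions set narrated info text, create Level Sequence players, and switch techniques by user role while toggling or resetting the menus.
; SystemCheck returns whether each step is complete, with a wait delay, testing actual menu use on practice steps.
; Separate Local and Multi variants handle step changes and animations.
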(fn SetSystemInfoStep
  (params (Widget :type Widget%20Object%20Reference) (Step :type Integer) (Pawn :type I%20Pawn%20Interface))
  (bind _output_get (LocalVariables|SetTargetPawn Pawn))
  (Default|HideAdvance _output_get)
  (bind _asinfo_box (Utilities|Casting|CastToInfoBox Widget))
  (LocalVariables|SetInfoBox _asinfo_box)
  (switch int Step
    (:0
      (Rendering|Components|TextRender|SetText (Variables|/Game/Blueprints/UserInterface/InfoBox.InfoBox_C|GetDescription (LocalVariables|GetInfoBox)) "System-Control techniques let users affect the state of a system. For example, changing the shape of an object or its colour. 
 
We will look at different types of 3D menus and widgets.")
      (LocalVariables|SetSoundClip "/Game/Assets/Sound/SC01.SC01")
      (Default|ChangeDescriptionFontSize (LocalVariables|GetInfoBox) 34 :!label _label)
      (Default|ShowInfowithDelay (LocalVariables|GetTargetPawn) 1.0 (LocalVariables|GetSoundClip) :!label _label_2))
    (:1
      (Default|HideInfo (LocalVariables|GetTargetPawn))
      (Rendering|Components|TextRender|SetText (Variables|/Game/Blueprints/UserInterface/InfoBox.InfoBox_C|GetDescription (LocalVariables|GetInfoBox)) "One way to classify these techniques is according to which object the 3DUI, 3D User Interface, is associated to. Device-referenced 3DUIs are those related to a particular device, such as the Controller.")
      (LocalVariables|SetSoundClip "/Game/Assets/Sound/SC02.SC02")
      (Default|ChangeDescriptionFontSize (LocalVariables|GetInfoBox) 40 :!label _label_3)
      (goto _label_2))
    (:2
      (Default|HideInfo (LocalVariables|GetTargetPawn))
      (Rendering|Components|TextRender|SetText (Variables|/Game/Blueprints/UserInterface/InfoBox.InfoBox_C|GetDescription (LocalVariables|GetInfoBox)) "A typical layout consists in arranging options around the controller in a radial menu. If the user moves the controller, the radial menu moves with it.  
Each shape represents an option you can select to change the appearance of the object in front of you.")
      (LocalVariables|SetSoundClip "/Game/Assets/Sound/SC03.SC03")
      (goto _label))
    (:3
      (Default|HideInfo (LocalVariables|GetTargetPawn))
      (Rendering|Components|TextRender|SetText (Variables|/Game/Blueprints/UserInterface/InfoBox.InfoBox_C|GetDescription (LocalVariables|GetInfoBox)) "Each sector of the trackpad corresponds to a different option. 
 
Press the trackpad to apply it to the object in front of you.")
      (LocalVariables|SetSoundClip "/Game/Assets/Sound/SC04.SC04")
      (Default|ChangeDescriptionFontSize (LocalVariables|GetInfoBox) 40)
      (goto _label_2))
    (:4
      (Default|HideInfo (LocalVariables|GetTargetPawn))
      (Rendering|Components|TextRender|SetText (Variables|/Game/Blueprints/UserInterface/InfoBox.InfoBox_C|GetDescription (LocalVariables|GetInfoBox)) "An object-based menu is one that associates possible actions to a specific object. Like the menu you see displayed in proximity of the object in front of you. 
 
Press next to try using this technique.")
      (LocalVariables|SetSoundClip "/Game/Assets/Sound/SC05.SC05")
      (goto _label_2))
    (:5
      (Default|HideInfo (LocalVariables|GetTargetPawn))
      (Rendering|Components|TextRender|SetText (Variables|/Game/Blueprints/UserInterface/InfoBox.InfoBox_C|GetDescription (LocalVariables|GetInfoBox)) "Point at the object with your controller and the menu will reappear. Then point at an option and press the trigger to apply it.")
      (LocalVariables|SetSoundClip "/Game/Assets/Sound/SC06.SC06")
      (goto _label_2))
    (:6
      (Default|HideInfo (LocalVariables|GetTargetPawn))
      (Rendering|Components|TextRender|SetText (Variables|/Game/Blueprints/UserInterface/InfoBox.InfoBox_C|GetDescription (LocalVariables|GetInfoBox)) "The final technique consists in a \"World-based\" menu. That is, an interface that uses 2D widgets, but exists as a 3D object in the Virtual Environment, that you could walk close to or away from, if needed. 
 
Press next to interact with it.")
      (LocalVariables|SetSoundClip "/Game/Assets/Sound/SC07.SC07")
      (Default|ShowInfowithDelay (LocalVariables|GetTargetPawn) 3.0 (LocalVariables|GetSoundClip)))
    (:7
      (Default|HideInfo (LocalVariables|GetTargetPawn))
      (Rendering|Components|TextRender|SetText (Variables|/Game/Blueprints/UserInterface/InfoBox.InfoBox_C|GetDescription (LocalVariables|GetInfoBox)) "You can interact with the menu by pointing at its widgets and pressing the trigger to perform the associated action.")
      (LocalVariables|SetSoundClip "/Game/Assets/Sound/SC08.SC08")
      (goto _label_2))
    (:8
      (Default|HideInfo (LocalVariables|GetTargetPawn))
      (Rendering|Components|TextRender|SetText (Variables|/Game/Blueprints/UserInterface/InfoBox.InfoBox_C|GetDescription (LocalVariables|GetInfoBox)) "This concludes this lesson! Thank you for participating.")
      (LocalVariables|SetSoundClip "/Game/Assets/Sound/LectureOver.LectureOver")
      (goto _label_3)))
  (return true))

(fn SystemStepLocal
  (params (Step :type Integer))
  (switch int Step
    (:0
      ;[1 1 1] Disable Arrow
      (bind _outactors (Actor|GetAllActorswithInterface 0 "/Game/Blueprints/Pawns/IPawn.IPawn_C"))
      (for _array_element _outactors
        (bind _arrow (Class|IPawn|GetArrow(Message) _array_element))
        (Rendering|SetActorHiddenInGame _arrow true)))
    (:3
      (Utilities|FlowControl|Sequence
        (:then_0
          ;[1 1 1] Stop animation
          (CallFunction|GetPlayerController "NewEnumerator0")
          (bind _actor (CallFunction|GetActorOfType "/Game/Blueprints/Actors/FakeShapeRadialMenu.FakeShapeRadialMenu_C"))
          (Variables|/Game/Blueprints/Actors/FakeShapeRadialMenu.FakeShapeRadialMenu_C|SetbAnimate (.AsFake%20Shape%20Radial%20Menu (Utilities|Casting|CastToFakeShapeRadialMenu _actor)) false))
        (:then_1
          ;[1 0.6269 0.3385] Switch techniques
          (CallFunction|SwitchTechniqueifRole "Shape" "NewEnumerator1"))))
    (:4
      (Utilities|FlowControl|Sequence
        (:then_0
          ;[1 1 1] Enable ContextualMenu
          (bind _actor_2 (CallFunction|GetActorOfType "/Game/Blueprints/Actors/ContextualMenuActor.ContextualMenuActor_C" :!label _label))
          (bind _ascontextual_menu_actor (Utilities|Casting|CastToContextualMenuActor _actor_2)))
        (:then_1
          (Default|SetMenuVisibility _ascontextual_menu_actor false))
        (:then_2
          (CallFunction|SwitchTechniqueifRole "Controller" "NewEnumerator1" :!label _label_2))))
    (:5
      (Utilities|FlowControl|Sequence
        (:then_0
          (goto _label))
        (:then_1
          ;[1 1 1] Disable ContextualMenu
          (Default|SetMenuVisibility _ascontextual_menu_actor true :!label _label_3))
        (:then_2
          (CallFunction|SwitchTechniqueifRole "UI" "NewEnumerator1" :!label _label_4))
        (:then_3
          (bind _actor_3 (CallFunction|GetActorOfType "/Game/Blueprints/Actors/WorldBasedMenu.WorldBasedMenu_C" :!label _label_5))
          (bind _asworld_based_menu (Utilities|Casting|CastToWorldBasedMenu _actor_3))
          (Default|UpdateSelection (.AsUI%20World%20Based%20Menu (Utilities|Casting|CastToUI_WorldBasedMenu (UserInterface|GetUserWidgetObject (Variables|/Game/Blueprints/Actors/WorldBasedMenu.WorldBasedMenu_C|GetWidget _asworld_based_menu)))) "Cube" "Black")
          (Variables|/Game/Blueprints/UserInterface/UI_WorldBasedMenu.UI_WorldBasedMenu_C|SetbHasBeenUsed (.AsUI%20World%20Based%20Menu (Utilities|Casting|CastToUI_WorldBasedMenu (UserInterface|GetUserWidgetObject (Variables|/Game/Blueprints/Actors/WorldBasedMenu.WorldBasedMenu_C|GetWidget _asworld_based_menu)))) false))))
    (:6
      (Utilities|FlowControl|Sequence
        (:then_0
          (goto _label_3))
        (:then_1
          (goto _label_2))
        (:then_2
          (bind _actor_4 (CallFunction|GetActorOfType "/Game/Blueprints/Actors/ContextualMenuActor.ContextualMenuActor_C"))
          (bind _ascontextual_menu_actor_2 (Utilities|Casting|CastToContextualMenuActor _actor_4))
          (Variables|/Game/Blueprints/Actors/ContextualMenuActor.ContextualMenuActor_C|SetbMenuActive _ascontextual_menu_actor_2 false))
        (:then_3
          (goto _label_5))))
    (:7
      (Utilities|FlowControl|Sequence
        (:then_0
          (goto _label_5))
        (:then_1
          (goto _label_4))))))

(fn CreateSystemAnimationStep
  (params (Step :type Integer))
  (switch int Step
    (:1
      (bind _returnvalue (Sequencer|Player|CreateLevelSequencePlayer 0 "/Game/Assets/Animations/SystemStep1.SystemStep1"))
      (return _returnvalue))
    (:2
      (bind _returnvalue_2 (Sequencer|Player|CreateLevelSequencePlayer 0 "/Game/Assets/Animations/SystemStep2.SystemStep2"))
      (return _returnvalue_2))
    (:3
      (bind _returnvalue_3 (Sequencer|Player|CreateLevelSequencePlayer 0 "/Game/Assets/Animations/SystemStep3.SystemStep3"))
      (return _returnvalue_3))
    (:4
      (bind _returnvalue_4 (Sequencer|Player|CreateLevelSequencePlayer 0 "/Game/Assets/Animations/SystemStep4.SystemStep4"))
      (return _returnvalue_4))
    (:5
      (bind _returnvalue_5 (Sequencer|Player|CreateLevelSequencePlayer 0 "/Game/Assets/Animations/SystemStep5.SystemStep5"))
      (return _returnvalue_5))
    (:6
      (bind _returnvalue_6 (Sequencer|Player|CreateLevelSequencePlayer 0 "/Game/Assets/Animations/SystemStep6.SystemStep6"))
      (return _returnvalue_6))
    (:7
      (bind _returnvalue_7 (Sequencer|Player|CreateLevelSequencePlayer 0 "/Game/Assets/Animations/SystemStep7.SystemStep7"))
      (return _returnvalue_7))))

(fn SystemCheck
  (params (Step :type Integer) (Pawn :type I%20Pawn%20Interface))
  (switch int Step
    (:0
      (bind _canprogress (Default|CheckArrow Pawn))
      (return _canprogress 0.0))
    (:1
      (return true 11.0))
    (:2
      (return true 12.0))
    (:3
      (return true 15.0))
    (:4
      ;[1 1 1] Check if Radial Menu used
      (bind _actor (CallFunction|GetActorOfType "/Game/Blueprints/Techniques/ShapeRadialMenu.ShapeRadialMenu_C"))
      (bind _asshape_radial_menu (Utilities|Casting|CastToShapeRadialMenu _actor)
        (:then
          (return (> (Variables|/Game/Blueprints/Techniques/ShapeRadialMenu.ShapeRadialMenu_C|GetTimesChanged _asshape_radial_menu) 0) 0.0))
        (:CastFailed
          (return false 0.0))))
    (:5
      (return true 11.0))
    (:6
      ;[1 1 1] Check if Contextual Menu used
      (bind _actor_2 (CallFunction|GetActorOfType "/Game/Blueprints/Actors/ContextualMenuActor.ContextualMenuActor_C"))
      (bind _ascontextual_menu_actor (Utilities|Casting|CastToContextualMenuActor _actor_2)
        (:then
          (return (Variables|/Game/Blueprints/Actors/ContextualMenuActor.ContextualMenuActor_C|GetbHasBeenUsed _ascontextual_menu_actor) 0.0))
        (:CastFailed
          (return false 0.0))))
    (:7
      (return true 16.0))
    (:8
      ;[1 1 1] Check if WoldBased Menu used
      (bind _actor_3 (CallFunction|GetActorOfType "/Game/Blueprints/Actors/WorldBasedMenu.WorldBasedMenu_C"))
      (bind _asworld_based_menu (Utilities|Casting|CastToWorldBasedMenu _actor_3)
        (:then
          (return (Variables|/Game/Blueprints/UserInterface/UI_WorldBasedMenu.UI_WorldBasedMenu_C|GetbHasBeenUsed (.AsUI%20World%20Based%20Menu (Utilities|Casting|CastToUI_WorldBasedMenu (UserInterface|GetUserWidgetObject (Variables|/Game/Blueprints/Actors/WorldBasedMenu.WorldBasedMenu_C|GetWidget _asworld_based_menu))))) 0.0))
        (:CastFailed
          (return false 0.0))))
    (:9
      (return false 4.0))))

(fn SystemStepMulti
  (params (Step :type Integer))
  (switch int Step
    (:0
      ;[1 1 1] Disable Arrow
      (bind _outactors (Actor|GetAllActorswithInterface 0 "/Game/Blueprints/Pawns/IPawn.IPawn_C"))
      (for _array_element _outactors
        (bind _arrow (Class|IPawn|GetArrow(Message) _array_element))
        (Rendering|SetActorHiddenInGame _arrow true)))
    (:2
      (CallFunction|SwitchTechniqueifRole "Shape" "NewEnumerator2"))
    (:3
      (CallFunction|SwitchTechniqueifRole "Shape" "NewEnumerator1"))
    (:4
      (Utilities|FlowControl|Sequence
        (:then_0
          ;[1 1 1] Enable ContextualMenu
          (bind _actor (CallFunction|GetActorOfType "/Game/Blueprints/Actors/ContextualMenuActor.ContextualMenuActor_C" :!label _label))
          (bind _ascontextual_menu_actor (Utilities|Casting|CastToContextualMenuActor _actor)))
        (:then_1
          (Default|SetMenuVisibility _ascontextual_menu_actor false))
        (:then_2
          (CallFunction|SwitchTechniqueifRole "UI" "NewEnumerator2")
          (CallFunction|SwitchTechniqueifRole "Controller" "NewEnumerator1"))))
    (:5
      (Utilities|FlowControl|Sequence
        (:then_0
          (goto _label))
        (:then_1
          ;[1 1 1] Disable ContextualMenu
          (Default|SetMenuVisibility _ascontextual_menu_actor true :!label _label_2))
        (:then_2
          (CallFunction|SwitchTechniqueifRole "UI" "NewEnumerator1"))
        (:then_3
          (bind _actor_2 (CallFunction|GetActorOfType "/Game/Blueprints/Actors/WorldBasedMenu.WorldBasedMenu_C" :!label _label_3))
          (bind _asworld_based_menu (Utilities|Casting|CastToWorldBasedMenu _actor_2))
          (Default|UpdateSelection (.AsUI%20World%20Based%20Menu (Utilities|Casting|CastToUI_WorldBasedMenu (UserInterface|GetUserWidgetObject (Variables|/Game/Blueprints/Actors/WorldBasedMenu.WorldBasedMenu_C|GetWidget _asworld_based_menu)))) "Cube" "Black"))))
    (:6
      (Utilities|FlowControl|Sequence
        (:then_0
          (goto _label_2))
        (:then_1
          (CallFunction|SwitchTechniqueifRole "Controller" "NewEnumerator1"))
        (:then_2
          (bind _actor_3 (CallFunction|GetActorOfType "/Game/Blueprints/Actors/ContextualMenuActor.ContextualMenuActor_C"))
          (bind _ascontextual_menu_actor_2 (Utilities|Casting|CastToContextualMenuActor _actor_3))
          (Variables|/Game/Blueprints/Actors/ContextualMenuActor.ContextualMenuActor_C|SetbMenuActive _ascontextual_menu_actor_2 false))))
    (:7
      (Utilities|FlowControl|Sequence
        (:then_0
          (goto _label_3))
        (:then_1
          (CallFunction|SwitchTechniqueifRole "UI" "NewEnumerator1"))))))

(fn CreateSystemAnimationStepMulti
  (params (Step :type Integer))
  (switch int Step
    (:1
      (bind _returnvalue (Sequencer|Player|CreateLevelSequencePlayer 0 "/Game/Assets/Animations/SystemStep1.SystemStep1"))
      (return _returnvalue))
    (:6
      (bind _returnvalue_2 (Sequencer|Player|CreateLevelSequencePlayer 0 "/Game/Assets/Animations/SystemStep6m.SystemStep6m"))
      (return _returnvalue_2))))