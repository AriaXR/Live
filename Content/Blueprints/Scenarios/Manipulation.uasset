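; Scenario Blueprint for a narrated VR lesson on object manipulation, teaching the hand grab and GoGo extended-arm techniques.
; Step-indexed functions set info-box text and voice clips, create Level Sequence animations, and check completion through InteractedWith flags or fixed delays.
; Local and multi variants drive each step's world changes: showing, resetting and dropping throwables, spawning Lego bricks, and switching technique by user role.
; The multi variant adds a server-only spawn guard and staggers GoGo between roles.
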(fn ManipulationLocal
  (params (Step :type Integer))
  (switch int Step
    (:0
      (Utilities|FlowControl|Sequence
        (:then_0
          ;[1 1 1] Disable Arrow
          (bind _outactors (Actor|GetAllActorswithInterface 0 "/Game/Blueprints/Pawns/IPawn.IPawn_C"))
          (for _array_element _outactors
            (bind _arrow (Class|IPawn|GetArrow(Message) _array_element))
            (Rendering|SetActorHiddenInGame _arrow true)))
        (:then_1
          ;[1 1 1] Show throwables
          (bind _outactors_2 (Actor|GetAllActorsOfClass 0 "/Game/Blueprints/Actors/ThrowableActor.ThrowableActor_C"))
          (for _array_element_2 _outactors_2
            (Rendering|SetActorHiddenInGame _array_element_2 false)
            (Default|RandomState _array_element_2)))))
    (:2
      (Utilities|FlowControl|Sequence
        (:then_0
          ;[1 1 1] Return throwables to original location
          (bind _outactors_3 (Actor|GetAllActorswithTag 0 "Throwables"))
          (for _array_element_3 _outactors_3
            (Default|ReturnState (.AsThrowable%20Actor (Utilities|Casting|CastToThrowableActor _array_element_3)))))
        (:then_1
          (CallFunction|SwitchTechniqueifRole "Hand" "NewEnumerator1"))))
    (:3
      (Utilities|FlowControl|Sequence
        (:then_0
          ;[1 1 1] Return all throwables to original location
          (bind _outactors_4 (Actor|GetAllActorsOfClass 0 "/Game/Blueprints/Actors/ThrowableActor.ThrowableActor_C"))
          (for _array_element_4 _outactors_4
            (Default|ReturnState _array_element_4)))
        (:then_1
          ;[1 1 1] Reset "InteractedWith"
          (bind _outactors_5 (Actor|GetAllActorswithTag 0 "Throwables"))
          (for _array_element_5 _outactors_5
            (Variables|/Game/Blueprints/Actors/ThrowableActor.ThrowableActor_C|SetbInteractedWith (.AsThrowable%20Actor (Utilities|Casting|CastToThrowableActor _array_element_5)) false)))))
    (:4
      (Utilities|FlowControl|Sequence
        (:then_0
          ;[1 1 1] Make throwables fall down the floor
          (bind _outactors_6 (Actor|GetAllActorsOfClass 0 "/Game/Blueprints/Actors/ThrowableActor.ThrowableActor_C"))
          (for _array_element_6 _outactors_6
            (Collision|SetCollisionProfileName (Variables|/Game/Blueprints/Actors/ThrowableActor.ThrowableActor_C|GetTargetMesh _array_element_6) "OverlapAll" :!class /Script/Engine.PrimitiveComponent)
            (Default|MovetoState _array_element_6 (Math|Transform|MakeTransform (+ (.Location (Math|Transform|BreakTransform (Transformation|GetActorTransform _array_element_6))) "0, 0,-200.000000") (.Rotation (Math|Transform|BreakTransform (Transformation|GetActorTransform _array_element_6))) (.Scale (Math|Transform|BreakTransform (Transformation|GetActorTransform _array_element_6)))) 1.0)))
        (:then_1
          ;[1 1 1] Spawn Lego bricks
          (bind _outactors_7 (Actor|GetAllActorswithTag 0 "LegoPillars"))
          (bind _player_controller (CallFunction|GetPlayerController "NewEnumerator1"))
          (for _array_element_7 _outactors_7
            (Default|ServerSpawnActor _player_controller "/Game/Blueprints/CreateRandomTargets.CreateRandomTargets_C" (Math|Transform|MakeTransform (+ (Transformation|GetActorLocation _array_element_7) "0, 0,200.000000")) _player_controller false false)))
        (:then_2
          (CallFunction|SwitchTechniqueifRole "GoGo" "NewEnumerator1"))))))

(fn CreateManipulationAnimationStep
  (params (Step :type Integer))
  (switch int Step
    (:2
      (bind _returnvalue (Sequencer|Player|CreateLevelSequencePlayer 0 "/Game/Assets/Animations/ManipulationStep1.ManipulationStep1"))
      (return _returnvalue))
    (:3
      (bind _returnvalue_2 (Sequencer|Player|CreateLevelSequencePlayer 0 "/Game/Assets/Animations/ManipulationStep2.ManipulationStep2"))
      (return _returnvalue_2))
    (:4
      (bind _returnvalue_3 (Sequencer|Player|CreateLevelSequencePlayer 0 "/Game/Assets/Animations/ManipulationStep3.ManipulationStep3"))
      (return _returnvalue_3))
    (:5
      (bind _returnvalue_4 (Sequencer|Player|CreateLevelSequencePlayer 0 "/Game/Assets/Animations/ManipulationStep4.ManipulationStep4"))
      (return _returnvalue_4))))

(fn ManipulationCheck
  (params (Step :type Integer) (Pawn :type I%20Pawn%20Interface))
  (switch int Step
    (:0
      (bind _canprogress (Default|CheckArrow Pawn))
      (return _canprogress 0.0))
    (:1
      (return true 9.0))
    (:2
      (return true 6.0))
    (:3
      (bind _outactors (Actor|GetAllActorswithTag 0 "Throwables" :!label _label))
      (for _array_element _outactors
        (if (Variables|/Game/Blueprints/Actors/ThrowableActor.ThrowableActor_C|GetbInteractedWith (.AsThrowable%20Actor (Utilities|Casting|CastToThrowableActor _array_element)))
          (return (Variables|/Game/Blueprints/Actors/ThrowableActor.ThrowableActor_C|GetbInteractedWith (.AsThrowable%20Actor (Utilities|Casting|CastToThrowableActor _array_element))) 1.0))))
    (:4
      (goto _label))
    (:5
      (return true 19.0))
    (:6
      (bind _outactors_2 (Actor|GetAllActorsOfClass 0 "/Game/Blueprints/Actors/BrickActor.BrickActor_C"))
      (for _array_element_2 _outactors_2
        (if (Variables|/Game/Blueprints/Actors/BrickActor.BrickActor_C|GetbInteractedWith _array_element_2)
          (return (Variables|/Game/Blueprints/Actors/BrickActor.BrickActor_C|GetbInteractedWith _array_element_2) 1.0))))))

(fn SetManipulationInfoStep
  (params (Widget :type Widget%20Object%20Reference) (Step :type Integer) (Pawn :type I%20Pawn%20Interface))
  (bind _output_get (LocalVariables|SetTargetPawn Pawn))
  (Default|HideAdvance _output_get)
  (bind _asinfo_box (Utilities|Casting|CastToInfoBox Widget))
  (LocalVariables|SetInfoBox _asinfo_box)
  (switch int Step
    (:Default
      (return false))
    (:0
      (Rendering|Components|TextRender|SetText (Variables|/Game/Blueprints/UserInterface/InfoBox.InfoBox_C|GetDescription (LocalVariables|GetInfoBox)) "Manipulation is the act of altering an object's position and orientation.")
      (LocalVariables|SetSoundClip "/Game/Assets/Sound/Man01.Man01")
      (Default|ShowInfowithDelay (LocalVariables|GetTargetPawn) 5.0 (LocalVariables|GetSoundClip)))
    (:1
      (Default|HideInfo (LocalVariables|GetTargetPawn))
      (Rendering|Components|TextRender|SetText (Variables|/Game/Blueprints/UserInterface/InfoBox.InfoBox_C|GetDescription (LocalVariables|GetInfoBox)) "There are various techniques to manipulate an object. The most natural of which, is the hand metaphor.")
      (LocalVariables|SetSoundClip "/Game/Assets/Sound/Man02.Man02")
      (Default|ShowInfowithDelay (LocalVariables|GetTargetPawn) 1.0 (LocalVariables|GetSoundClip) :!label _label))
    (:2
      (Default|HideInfo (LocalVariables|GetTargetPawn))
      (Rendering|Components|TextRender|SetText (Variables|/Game/Blueprints/UserInterface/InfoBox.InfoBox_C|GetDescription (LocalVariables|GetInfoBox)) "On your right there are a few objects with which you can interact. Pressing the trigger \"grabs\" the object. Try it!")
      (LocalVariables|SetSoundClip "/Game/Assets/Sound/Man03.Man03")
      (Default|ShowInfowithDelay (LocalVariables|GetTargetPawn) 3.0 (LocalVariables|GetSoundClip) :!label _label_2))
    (:3
      (Default|HideInfo (LocalVariables|GetTargetPawn))
      (Rendering|Components|TextRender|SetText (Variables|/Game/Blueprints/UserInterface/InfoBox.InfoBox_C|GetDescription (LocalVariables|GetInfoBox)) "Try to throw them at the targets in front of you! Then, to progress press \"Next\". ")
      (LocalVariables|SetSoundClip "/Game/Assets/Sound/Man04.Man04")
      (goto _label_2))
    (:4
      (Default|HideInfo (LocalVariables|GetTargetPawn))
      (Rendering|Components|TextRender|SetText (Variables|/Game/Blueprints/UserInterface/InfoBox.InfoBox_C|GetDescription (LocalVariables|GetInfoBox)) "If objects are distant, you can use the \"GoGo\" technique, which uses an \"extensible arm\". When your controller is close to your body, it works like the previous hand technique. However, when you extend your arm, your hand will be able to reach longer distances. 
 
Press \"Next\" to see a demonstration.")
      (LocalVariables|SetSoundClip "/Game/Assets/Sound/Man05.Man05")
      (Default|ChangeDescriptionFontSize (LocalVariables|GetInfoBox) 36)
      (goto _label_2))
    (:5
      (Default|HideInfo (LocalVariables|GetTargetPawn))
      (Rendering|Components|TextRender|SetText (Variables|/Game/Blueprints/UserInterface/InfoBox.InfoBox_C|GetDescription (LocalVariables|GetInfoBox)) "Now try to use the GoGo technique to sort the bricks from the plates in the two containers in front of you.")
      (LocalVariables|SetSoundClip "/Game/Assets/Sound/Man06.Man06")
      (Default|ChangeDescriptionFontSize (LocalVariables|GetInfoBox) 48)
      (goto _label_2))
    (:6
      (Default|HideInfo (LocalVariables|GetTargetPawn))
      (Rendering|Components|TextRender|SetText (Variables|/Game/Blueprints/UserInterface/InfoBox.InfoBox_C|GetDescription (LocalVariables|GetInfoBox)) "This concludes this lesson! Thank you for participating.")
      (LocalVariables|SetSoundClip "/Game/Assets/Sound/LectureOver.LectureOver")
      (goto _label)))
  (return true))

(fn CreateManipulationAnimationMulti
  (params (Step :type Integer))
  (switch int Step
    (:2
      (bind _returnvalue (Sequencer|Player|CreateLevelSequencePlayer 0 "/Game/Assets/Animations/ManipulationStep1multi.ManipulationStep1multi"))
      (return _returnvalue))
    (:3
      (bind _returnvalue_2 (Sequencer|Player|CreateLevelSequencePlayer 0 "/Game/Assets/Animations/ManipulationStep2multi.ManipulationStep2multi"))
      (return _returnvalue_2))
    (:4
      (bind _returnvalue_3 (Sequencer|Player|CreateLevelSequencePlayer 0 "/Game/Assets/Animations/ManipulationStep3.ManipulationStep3"))
      (return _returnvalue_3))
    (:5
      (bind _returnvalue_4 (Sequencer|Player|CreateLevelSequencePlayer 0 "/Game/Assets/Animations/ManipulationStep5multi.ManipulationStep5multi"))
      (return _returnvalue_4))))

(fn ManipulationMulti
  (params (Step :type Integer))
  (switch int Step
    (:0
      (Utilities|FlowControl|Sequence
        (:then_0
          ;[1 1 1] Disable Arrow
          (bind _outactors (Actor|GetAllActorswithInterface 0 "/Game/Blueprints/Pawns/IPawn.IPawn_C"))
          (for _array_element _outactors
            (bind _arrow (Class|IPawn|GetArrow(Message) _array_element))
            (Rendering|SetActorHiddenInGame _arrow true)))
        (:then_1
          ;[1 1 1] Show throwables
          (bind _outactors_2 (Actor|GetAllActorsOfClass 0 "/Game/Blueprints/Actors/ThrowableActor.ThrowableActor_C"))
          (for _array_element_2 _outactors_2
            (Rendering|SetActorHiddenInGame _array_element_2 false)
            (Default|RandomState _array_element_2)))))
    (:2
      (Utilities|FlowControl|Sequence
        (:then_0
          ;[1 1 1] Return throwables to original location
          (bind _outactors_3 (Actor|GetAllActorswithTag 0 "Throwables"))
          (for _array_element_3 _outactors_3
            (Default|ReturnState (.AsThrowable%20Actor (Utilities|Casting|CastToThrowableActor _array_element_3)))))
        (:then_1
          (CallFunction|SwitchTechniqueifRole "Hand" "NewEnumerator1")
          (CallFunction|SwitchTechniqueifRole "Hand" "NewEnumerator2"))))
    (:3
      (Utilities|FlowControl|Sequence
        (:then_0
          ;[1 1 1] Return all throwables to original location
          (bind _outactors_4 (Actor|GetAllActorsOfClass 0 "/Game/Blueprints/Actors/ThrowableActor.ThrowableActor_C"))
          (for _array_element_4 _outactors_4
            (Default|ReturnState _array_element_4)))
        (:then_1
          ;[1 1 1] Reset "InteractedWith"
          (bind _outactors_5 (Actor|GetAllActorswithTag 0 "Throwables"))
          (for _array_element_5 _outactors_5
            (Variables|/Game/Blueprints/Actors/ThrowableActor.ThrowableActor_C|SetbInteractedWith (.AsThrowable%20Actor (Utilities|Casting|CastToThrowableActor _array_element_5)) false)))))
    (:4
      (Utilities|FlowControl|Sequence
        (:then_0
          ;[1 1 1] Make throwables fall down the floor
          (bind _outactors_6 (Actor|GetAllActorsOfClass 0 "/Game/Blueprints/Actors/ThrowableActor.ThrowableActor_C"))
          (for _array_element_6 _outactors_6
            (Collision|SetCollisionProfileName (Variables|/Game/Blueprints/Actors/ThrowableActor.ThrowableActor_C|GetTargetMesh _array_element_6) "OverlapAll" :!class /Script/Engine.PrimitiveComponent)
            (Default|MovetoState _array_element_6 (Math|Transform|MakeTransform (+ (.Location (Math|Transform|BreakTransform (Transformation|GetActorTransform _array_element_6))) "0, 0,-200.000000") (.Rotation (Math|Transform|BreakTransform (Transformation|GetActorTransform _array_element_6))) (.Scale (Math|Transform|BreakTransform (Transformation|GetActorTransform _array_element_6)))) 1.0)))
        (:then_1
          ;[1 1 1] Spawn Lego bricks
          (if (Networking|IsServer)
            (bind _outactors_7 (Actor|GetAllActorswithTag 0 "LegoPillars"))
            (bind _player_controller (CallFunction|GetPlayerController "NewEnumerator1"))
            (for _array_element_7 _outactors_7
              (Default|ServerSpawnActor _player_controller "/Game/Blueprints/CreateRandomTargets.CreateRandomTargets_C" (Math|Transform|MakeTransform (+ (Transformation|GetActorLocation _array_element_7) "0, 0,200.000000")) 0 false false))))
        (:then_2
          (CallFunction|SwitchTechniqueifRole "GoGo" "NewEnumerator2"))))
    (:5
      (CallFunction|SwitchTechniqueifRole "GoGo" "NewEnumerator1"))))