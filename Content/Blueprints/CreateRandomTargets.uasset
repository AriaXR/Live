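; Target spawner actor that scatters colored brick and plate BrickActors in a small box around its location.
; On BeginPlay or the Start event, the authority waits briefly, then runs a sequence of six mesh and material pairs, each spawning a sixth of TargetNumber.
; ServerSpawn creates each actor at a random point, passing the current mesh and material as spawn parameters.
; An unconnected chain for setting mesh, material and physics after spawning never runs.
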(event Custom|Start
  (Networking|SwitchHasAuthority
    (:Authority
      (Utilities|FlowControl|Delay 5.0)
      (Utilities|FlowControl|Sequence
        (:then_0
          (Variables|Default|SetMeshType "/Game/Assets/Bricks/Brick1x1.Brick1x1")
          (Variables|Default|SetMaterial "/Game/Assets/Abstract/Materials/MI_BrickGreen.MI_BrickGreen"))
        (:then_1
          (Variables|Default|SetMeshType "/Game/Assets/Bricks/Brick2x2.Brick2x2")
          (Variables|Default|SetMaterial "/Game/Assets/Abstract/Materials/MI_BrickRed.MI_BrickRed"))
        (:then_2
          (Variables|Default|SetMeshType "/Game/Assets/Bricks/Brick1x4.Brick1x4")
          (Variables|Default|SetMaterial "/Game/Assets/Abstract/Materials/MI_BrickLBG.MI_BrickLBG"))
        (:then_3
          (Variables|Default|SetMeshType "/Game/Assets/Bricks/Plate1x4.Plate1x4")
          (Variables|Default|SetMaterial "/Game/Assets/Abstract/Materials/MI_BrickBlue.MI_BrickBlue"))
        (:then_4
          (Variables|Default|SetMeshType "/Game/Assets/Bricks/Plate2x4.Plate2x4")
          (Variables|Default|SetMaterial "/Game/Assets/Abstract/Materials/MI_BrickMagenta.MI_BrickMagenta"))
        (:then_5
          (Variables|Default|SetMeshType "/Game/Assets/Bricks/Plate2x2.Plate2x2")
          (Variables|Default|SetMaterial "/Game/Assets/Abstract/Materials/MI_ReddishBrown.MI_ReddishBrown")))
      (for _index (range 1 (/ (Variables|Default|GetTargetNumber) 6))
        (CallFunction|ServerSpawn)))))

(event Custom|ServerSpawn
  (bind _returnvalue (Game|SpawnActorfromClass "/Game/Blueprints/Actors/BrickActor.BrickActor_C" (Math|Transform|MakeTransform (Math|Random|RandomPointinBoundingBox (Transformation|GetWorldLocation (Variables|Default|GetDefaultSceneRoot)) (Math|Vector|MakeVector 5e+01 5e+01 2e+01))) "Undefined" 0 (Variables|Default|GetMeshType) (Variables|Default|GetMaterial))))

(event Collision|EventActorBeginOverlap
  (params (OtherActor :type Actor%20Object%20Reference)))

(event EventBeginPlay
  (Networking|SwitchHasAuthority
    (:Authority
      (Utilities|FlowControl|Delay 5.0)
      (Utilities|FlowControl|Sequence
        (:then_0
          (Variables|Default|SetMeshType "/Game/Assets/Bricks/Brick1x1.Brick1x1")
          (Variables|Default|SetMaterial "/Game/Assets/Abstract/Materials/MI_BrickGreen.MI_BrickGreen"))
        (:then_1
          (Variables|Default|SetMeshType "/Game/Assets/Bricks/Brick2x2.Brick2x2")
          (Variables|Default|SetMaterial "/Game/Assets/Abstract/Materials/MI_BrickRed.MI_BrickRed"))
        (:then_2
          (Variables|Default|SetMeshType "/Game/Assets/Bricks/Brick1x4.Brick1x4")
          (Variables|Default|SetMaterial "/Game/Assets/Abstract/Materials/MI_BrickLBG.MI_BrickLBG"))
        (:then_3
          (Variables|Default|SetMeshType "/Game/Assets/Bricks/Plate1x4.Plate1x4")
          (Variables|Default|SetMaterial "/Game/Assets/Abstract/Materials/MI_BrickBlue.MI_BrickBlue"))
        (:then_4
          (Variables|Default|SetMeshType "/Game/Assets/Bricks/Plate2x4.Plate2x4")
          (Variables|Default|SetMaterial "/Game/Assets/Abstract/Materials/MI_BrickMagenta.MI_BrickMagenta"))
        (:then_5
          (Variables|Default|SetMeshType "/Game/Assets/Bricks/Plate2x2.Plate2x2")
          (Variables|Default|SetMaterial "/Game/Assets/Abstract/Materials/MI_ReddishBrown.MI_ReddishBrown")))
      (for _index (range 1 (/ (Variables|Default|GetTargetNumber) 6))
        (CallFunction|ServerSpawn)))))

(event EventTick
  (params (DeltaSeconds :type Float%20%28single-precision%29)))

(fn ConstructionScript)