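; PhysicsCube is a cube actor in the VR physics world that offers itself for pickup to whatever hits it.
; On BeginPlay it sets a random material from the first five entries of its RandomCubeColors array.
; On each mesh hit it sends PickupObjectMessage to the other actor, passing itself and left or right hand flags read from the hit component's tags.
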(event OnComponentHit(StaticMeshComponent)
  (params (HitComponent :type Primitive%20Component%20Object%20Reference) (OtherActor :type Actor%20Object%20Reference) (OtherComp :type Primitive%20Component%20Object%20Reference) (NormalImpulse :type Vector :default "0, 0, 0") (Hit :type Hit%20Result%20Structure%20%28by%20ref%29))
  (if (Utilities|DoesObjectImplementInterface OtherActor "/Game/Blueprints/Techniques/PickUpObjectInterface.PickUpObjectInterface_C")
    _
    (else
      _))
  (Class|PickUpObjectInterface|PickupObject(Message) OtherActor self (Components|ComponentHasTag OtherComp "righthand") (Components|ComponentHasTag OtherComp "lefthand")))

(event EventBeginPlay
  ;[1 1 1] Set Random Color
  (Rendering|Material|SetMaterial (Variables|Debug|GetStaticMeshComponent) 0 (Utilities|Array|Get(acopy) (Utilities|Struct|BreakPrototypeMaterials (Variables|Default|GetRandomCubeColors)) (Math|Random|RandomIntegerinRange 0 4))))

(fn ConstructionScript)