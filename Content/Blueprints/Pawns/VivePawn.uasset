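; HTC Vive pawn for multi-user VR lecture scenarios, carrying an InfoBox, radial command menu, pointer arrow and tracked controllers.
; Scenario initialisation sets title, commands and role-based UI visibility, polling progression when solo.
; Menu clicks advance lecture steps through authority-checked events that update info text, run VR commands and set animation sequences.
; The locally controlled pawn sends camera and controller transforms every tick for replication, untested beyond two users.
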(event Custom|ClientCreateCommands
  ;[1 0.4824 0.04706] Create Commands
  (bind _commands (CallFunction|CreateCommands (Variables|Default|GetScenario) (.UserClass (Utilities|Struct|BreakUser (Variables|Default|GetUser)))))
  (Variables|/Game/Blueprints/UserInterface/RadialMenu.RadialMenu_C|SetCommands (Utilities|GetRadialMenuWidget) _commands))

(event Custom|MultiStepFeedback
  (params (LectureStep :type Integer))
  (CallFunction|SelectionStepNetwork LectureStep))

(event Custom|RaisePossess
  (Pawn|Possess (Game|GetPlayerController 0) self))

(event Custom|ClientInitialisation
  (params (Scenario :type ScenarioEnum%20Enum))
  ;[1 0.4824 0.04706] Client Initialisation
  (bind _output_get (Variables|Default|SetScenario Scenario))
  (Utilities|FlowControl|Sequence
    (:then_0
      (bind _title (CallFunction|TitlefromScenarioEnum _output_get))
      (Rendering|Components|TextRender|SetText (Variables|/Game/Blueprints/UserInterface/InfoBox.InfoBox_C|GetTitle (|GetInfoBoxWidget)) (Utilities|Text|ToText(String) _title)))
    (:then_1
      (bind _outactors (Actor|GetAllActorswithTag "Indicator"))
      (Default|PointTowards (.AsArrow%20Actor (Utilities|Casting|CastToArrowActor (Variables|/Script/Engine.ChildActorComponent|GetChildActor (Variables|Default|GetArrowActor)))) (Utilities|Array|Get(acopy) _outactors)))
    (:then_2
      (Default|SetAdvanceVisibility (Utilities|GetRadialMenuWidget) false)
      (if (== (Default|UserCount (Utilities|LiveInstance)) 1)
        (Utilities|Time|SetTimerbyEvent (delegate Custom|CheckProgression) 1.0 true)
        (else
          ;[1 1 1] If there are two users, disable the InfoBox for the "User" role
          (if (Utilities|Enum|Equal(Enum) (.UserClass (Utilities|Struct|BreakUser (Variables|Default|GetUser))) "NewEnumerator1")
            (Development|SetHiddeninGame (Variables|Default|GetRadialMenu) true false)
            (Development|SetHiddeninGame (Variables|Default|GetInfoBox) true false)))))))

(event Custom|ServerAdvance
  (params (Command :type String))
  (bind _liveinstance (Utilities|LiveInstance))
  (bind _infobox (Variables|Default|GetInfoBox))
  (bind _lecturestep (Variables|Default|GetLectureStep))
  (bind (_returnvalue _font) (|GetInfoBoxtext _infobox))
  ;[1 1 1] ServerAdvanceStep
  (Networking|SwitchHasAuthority
    (:Authority
      (bind _output_get (Variables|Default|SetCurrentCommand Command))
      (switch string _output_get
        (:Next
          (CallFunction|ClientFB (Variables|/Game/Blueprints/LiveInstance.LiveInstance_C|GetCurrentScenario _liveinstance) _output_get _lecturestep (Default|UserCount _liveinstance))
          (CallFunction|ClientSetDescription _returnvalue (.Size (Utilities|Struct|BreakSlateFontInfo _font)))
          (Math|Integer|IncrementInt _lecturestep))))))

(event Custom|ServerNotifyUpdate
  (params (Id :type Integer) (Actor :type Transform) (RightController :type Transform) (LeftController :type Transform))
  ;[0 0.595 0.05287] Sync Transforms
  (if (not (Pawn|IsLocallyControlled))
    (CallFunction|ClientUpdate Actor RightController LeftController)))

(event Custom|ClientSetDescription
  (params (Text :type Text) (FontSize :type Integer))
  ;[1 1 1] Hack to overcome Network black magic ¯\_(ツ)_/¯
  (bind _found_pawns (CallFunction|GetAllPawnsbyUserClass "NewEnumerator1"))
  (bind _infobox (Default|GetInfoBox (Utilities|Array|Get(acopy) _found_pawns)))
  (Rendering|Components|TextRender|SetText (Variables|/Game/Blueprints/UserInterface/InfoBox.InfoBox_C|GetDescription (.AsInfo%20Box (Utilities|Casting|CastToInfoBox (UserInterface|GetUserWidgetObject _infobox)))) Text)
  (Default|ChangeDescriptionFontSize (.AsInfo%20Box (Utilities|Casting|CastToInfoBox (UserInterface|GetUserWidgetObject _infobox))) FontSize)
  (Default|HideAdvance (Utilities|Array|Get(acopy) _found_pawns)))

(event Custom|ClientUpdate
  (params (Actor :type Transform) (RightController :type Transform) (LeftController :type Transform))
  ;[0 0.595 0.05287] Sync Transforms
  (Transformation|SetWorldTransform (Variables|Default|GetL_MotionController) LeftController false false)
  (Transformation|SetWorldTransform (Variables|Default|GetR_MotionController) RightController false false)
  (Transformation|SetWorldTransform (Variables|Default|GetCamera) Actor false false))

(event Custom|ClientFB
  (params (Scenario :type ScenarioEnum%20Enum) (Command :type String) (Step :type Integer) (UserCount :type Integer))
  ;[1 0.065 0.065] Network code
  (CallFunction|SetInfoStep Scenario (UserInterface|GetUserWidgetObject (Variables|Default|GetInfoBox)) Step self)
  (CallFunction|ExecuteVRCommand Command Step Scenario UserCount (Variables|Default|GetCurrentSequence)))

(event Custom|CheckProgression
  (CallFunction|CheckProgression (Variables|Default|GetScenario) (Variables|Default|GetLectureStep) self))

(event Custom|SetStep
  (Variables|Default|SetLectureStep 0))

(event EventBeginPlay
  ;[1 0.4824 0.04706] BeginPlay
  (Development|PrintText (Default|UserInfotoString (Utilities|LiveInstance) (Variables|Default|GetUser)))
  (Networking|SwitchHasAuthority
    (:Authority
      (CallFunction|ClientInitialisation (Variables|/Game/Blueprints/LiveInstance.LiveInstance_C|GetCurrentScenario (Utilities|LiveInstance)))
      (CallFunction|ClientCreateCommands))))

(event Collision|EventActorBeginOverlap
  (params (OtherActor :type Actor%20Object%20Reference)))

(event EventHideInfo
  (bind _infobox (Variables|Default|GetInfoBox))
  (bind _returnvalue (UserInterface|GetUserWidgetObject _infobox))
  (if (Widget|IsVisible _returnvalue)
    (Widget|SetVisibility _returnvalue "Hidden")))

(event EventForceAdvance
  (bind _liveinstance (Utilities|LiveInstance))
  (bind _infobox (Variables|Default|GetInfoBox))
  (bind _lecturestep (Variables|Default|GetLectureStep))
  (bind (_returnvalue _font) (|GetInfoBoxtext _infobox))
  ;[1 1 1] ServerAdvanceStep
  (Variables|Default|SetCurrentCommand "Next")
  (CallFunction|ClientFB (Variables|/Game/Blueprints/LiveInstance.LiveInstance_C|GetCurrentScenario _liveinstance) (stale Custom|ServerAdvance _output_get) _lecturestep (Default|UserCount _liveinstance))
  (CallFunction|ClientSetDescription _returnvalue (.Size (Utilities|Struct|BreakSlateFontInfo _font)))
  (Math|Integer|IncrementInt _lecturestep))

(event EventTick
  (params (DeltaSeconds :type Float%20%28single-precision%29))
  ;[0 0.595 0.05287] Sync Transforms
  (if (Pawn|IsLocallyControlled)
    (CallFunction|ServerNotifyUpdate (.Id (Utilities|Struct|BreakUser (Variables|Default|GetUser))) (Transformation|GetWorldTransform (Variables|Default|GetCamera)) (Transformation|GetWorldTransform (Variables|Default|GetR_MotionController)) (Transformation|GetWorldTransform (Variables|Default|GetL_MotionController)))))

(event EventPossessed
  (params (NewController :type Controller%20Object%20Reference))
  (Variables|Default|SetIsPossessed true))

(event EventUnpossessed
  (params (OldController :type Controller%20Object%20Reference))
  (Development|PrintString (Utilities|String|Append (Utilities|GetObjectName OldController) " unpossessed.")))

(event EventShowAdvancewithDelay
  (params (WaitDelay :type Float%20%28single-precision%29))
  (bind _live_playercontroller (Utilities|LivePlayerController))
  (bind _radialmenu (Utilities|GetRadialMenuWidget))
  (bind _currenthoveredbutton (Variables|/Game/Blueprints/UserInterface/RadialMenu.RadialMenu_C|GetCurrentHoveredButton _radialmenu))
  (Utilities|IsValid _currenthoveredbutton
    (:Is%20Valid
      (if (not (Widget|IsVisible _currenthoveredbutton))
        (if (> WaitDelay 0.0)
          (Utilities|FlowControl|Delay WaitDelay)
          (Default|RumbleController _live_playercontroller 1.0 0.1 true)
          (else
            (Default|RumbleController _live_playercontroller 0.5 0.1 true)))
        (Widget|SetVisibility _currenthoveredbutton "Visible")))))

(event EventHideAdvance
  (bind _radialmenu (Utilities|GetRadialMenuWidget))
  (bind _currenthoveredbutton (Variables|/Game/Blueprints/UserInterface/RadialMenu.RadialMenu_C|GetCurrentHoveredButton _radialmenu))
  (if (not (Utilities|Enum|Equal(Enum) (.UserClass (Utilities|Struct|BreakUser (Variables|Default|GetUser))) "NewEnumerator2"))
    (Utilities|IsValid _currenthoveredbutton
      (:Is%20Valid
        (if (Widget|IsVisible _currenthoveredbutton)
          (Widget|SetVisibility _currenthoveredbutton "Hidden"))))))

(event EventShowInfowithDelay
  (params (WaitDelay :type Float%20%28single-precision%29) (Clip :type Sound%20Base%20Object%20Reference))
  (bind _live_playercontroller (Utilities|LivePlayerController))
  (bind _infobox (Variables|Default|GetInfoBox))
  (bind _returnvalue (UserInterface|GetUserWidgetObject _infobox))
  (if (Utilities|Enum|Equal(Enum) (.UserClass (Utilities|Struct|BreakUser (Variables|Default|GetUser))) "NewEnumerator2")
    (Default|RumbleController _live_playercontroller 0.5 0.1 true :!label _label)
    (Widget|SetVisibility _returnvalue "Visible" :!label _label_2)
    (Utilities|IsValid Clip
      (:Is%20Valid
        (Audio|PlaySound2D Clip)))
    (elif (not (Widget|IsVisible _returnvalue))
      (if (> WaitDelay 0.0)
        (Utilities|FlowControl|Delay WaitDelay)
        (Default|RumbleController _live_playercontroller 1.0 0.1 true)
        (goto _label_2)
        (else
          (goto _label))))))

(event Input|ActionEvents|InputActionNextMenuItem
  (params (Key :type Key%20Structure :default "AnyKey"))
  (bind _radialmenu (Utilities|GetRadialMenuWidget))
  ;[1 1 1] NextMenuItem
  (:Released
    (bind _count (Default|GetItemCount _radialmenu))
    (bind _result (Math|Integer|IncrementInt (Variables|Default|GetCursorIndex))
      (:%20%20
        (Default|MoveCursoratIndex _radialmenu _result _count (Variables|/Game/Blueprints/UserInterface/RadialMenu.RadialMenu_C|GetInitialAngle _radialmenu) (Variables|/Game/Blueprints/UserInterface/RadialMenu.RadialMenu_C|GetRadius _radialmenu) (Variables|/Game/Blueprints/UserInterface/RadialMenu.RadialMenu_C|GetCentre _radialmenu) (Variables|/Game/Blueprints/UserInterface/RadialMenu.RadialMenu_C|GetItemSize _radialmenu))))))

(event Input|ActionEvents|InputActionResetPosition
  (params (Key :type Key%20Structure :default "AnyKey"))
  (:Released
    (Class|HeadMountedDisplayFunctionLibrary|ResetOrientationandPosition 2.7e+02 "Position")))

(event Input|ActionEvents|InputActionExecuteMenuItem
  (params (Key :type Key%20Structure :default "AnyKey"))
  (bind _radialmenu (Utilities|GetRadialMenuWidget))
  ;[1 1 1] ExecuteMenuItem
  (:Released
    (if (Widget|IsVisible (Variables|/Game/Blueprints/UserInterface/RadialMenu.RadialMenu_C|GetCurrentHoveredButton _radialmenu))
      (Default|OnClick _radialmenu)
      (CallFunction|ServerAdvance (Variables|/Game/Blueprints/UserInterface/RadialMenu.RadialMenu_C|GetCurrentCommand _radialmenu)))))

(event Input|ActionEvents|InputActionResetOrientation
  (params (Key :type Key%20Structure :default "AnyKey"))
  (:Released
    (Class|HeadMountedDisplayFunctionLibrary|ResetOrientationandPosition 2.7e+02 "Orientation")))

(event Input|ActionEvents|InputActionPrevMenuItem
  (params (Key :type Key%20Structure :default "AnyKey"))
  (bind _radialmenu (Utilities|GetRadialMenuWidget))
  ;[1 1 1] PrevMenuItem
  (:Released
    (bind _result (Math|Integer|DecrementInt (Variables|Default|GetCursorIndex))
      (:%20%20
        (bind _count (Default|GetItemCount _radialmenu))
        (Default|MoveCursoratIndex _radialmenu _result _count (Variables|/Game/Blueprints/UserInterface/RadialMenu.RadialMenu_C|GetInitialAngle _radialmenu) (Variables|/Game/Blueprints/UserInterface/RadialMenu.RadialMenu_C|GetRadius _radialmenu) (Variables|/Game/Blueprints/UserInterface/RadialMenu.RadialMenu_C|GetCentre _radialmenu) (Variables|/Game/Blueprints/UserInterface/RadialMenu.RadialMenu_C|GetItemSize _radialmenu))))))

(event Input|AxisEvents|InputAxisMoveForward
  (params (AxisValue :type Float%20%28single-precision%29))
  ;[1 1 1] Keyboard Input
  (Pawn|Input|AddMovementInput (select (Class|HeadMountedDisplayFunctionLibrary|IsHeadMountedDisplayEnabled) (Math|Vector|GetForwardVector (Variables|Default|GetCamera)) (Transformation|GetActorForwardVector)) AxisValue false))

(event Input|AxisEvents|InputAxisMoveRight
  (params (AxisValue :type Float%20%28single-precision%29))
  ;[1 1 1] Keyboard Input
  (Pawn|Input|AddMovementInput (select (Class|HeadMountedDisplayFunctionLibrary|IsHeadMountedDisplayEnabled) (Math|Vector|GetRightVector (Variables|Default|GetCamera)) (Transformation|GetActorRightVector)) AxisValue false))

(event Input|KeyboardEvents|MotionControllerLeftTriggerAxis
  (params (AxisValue :type Float%20%28single-precision%29))
  ;[0.1137 0.349 1] Left Controller w/ Trigger Animation
  (bind _asvive_controller_ab (Utilities|Casting|CastToVive_Controller_AB (Components|SkeletalMesh|GetAnimInstance (Variables|Default|GetL_ViveController))))
  (Variables|/Game/Assets/Controller/Animations/Vive_Controller_AB.Vive_Controller_AB_C|SetTriggerAxisAmount _asvive_controller_ab AxisValue))

(event Input|KeyboardEvents|MotionControllerLeftThumbstickX
  (params (AxisValue :type Float%20%28single-precision%29))
  ;[0.1137 0.349 1] Left Trackpad Thumb Tracking
  (bind _output_get (Variables|Default|SetL%20ThumbX AxisValue))
  (Transformation|SetRelativeLocation (Variables|Default|GetL_TrackpadSphere) (Math|Vector|MakeVector (- (* (stale Input|KeyboardEvents|MotionControllerLeftThumbstickY _output_get) -1.7) 3.5) (* _output_get 1.7) 1.8) false false))

(event Input|KeyboardEvents|MotionControllerLeftThumbstickY
  (params (AxisValue :type Float%20%28single-precision%29))
  ;[0.1137 0.349 1] Left Trackpad Thumb Tracking
  (bind _output_get (Variables|Default|SetL%20ThumbY AxisValue))
  (Transformation|SetRelativeLocation (Variables|Default|GetL_TrackpadSphere) (Math|Vector|MakeVector (- (* _output_get -1.7) 3.5) (* (stale Input|KeyboardEvents|MotionControllerLeftThumbstickX _output_get) 1.7) 1.8) false false))

(event Input|KeyboardEvents|MotionControllerLeftThumbstick
  (params (Key :type Key%20Structure :default "AnyKey"))
  (bind _radialmenu (Utilities|GetRadialMenuWidget))
  ;[1 1 1] ExecuteMenuItem
  (:Released
    (if (Widget|IsVisible (Variables|/Game/Blueprints/UserInterface/RadialMenu.RadialMenu_C|GetCurrentHoveredButton _radialmenu))
      (Default|OnClick _radialmenu)
      (CallFunction|ServerAdvance (Variables|/Game/Blueprints/UserInterface/RadialMenu.RadialMenu_C|GetCurrentCommand _radialmenu)))))

(event Input|KeyboardEvents|MotionControllerLeftTrigger
  (params (Key :type Key%20Structure :default "AnyKey"))
  (bind _currentsequence (Variables|Default|GetCurrentSequence))
  (:Released
    (Utilities|IsValid _currentsequence
      (:Is%20Valid
        (Components|Timeline|SetPlaybackPosition _currentsequence 0.0)
        (Sequencer|Player|Play _currentsequence :!class /Script/MovieScene.MovieSceneSequencePlayer)))))

(fn ConstructionScript
  (Development|PrintString "Spawn"))

(fn ExecuteVRCommand
  (params (Command :type String))
  (switch string Command
    (:Next
      (switch Utilities|FlowControl|Switch|SwitchonUserClassEnum (.UserClass (Utilities|Struct|BreakUser (Variables|Default|GetUser)))
        (:NewEnumerator1
          (CallFunction|SetSelectionInfoStep (UserInterface|GetUserWidgetObject (Variables|Default|GetInfoBox)) (Variables|Default|GetLectureStep))
          (CallFunction|SelectionStepLocal (Variables|Default|GetLectureStep))
          (bind _sequencer (CallFunction|CreateSelectionAnimationStep (Variables|Default|GetLectureStep)))
          (Utilities|IsValid _sequencer
            (:Is%20Valid
              (Audio|Components|Audio|Play _sequencer))
            (:Is%20Not%20Valid
              _))
          (bind _result (Math|Integer|IncrementInt (Variables|Default|GetLectureStep))
            (:%20%20
              (Variables|Default|SetLectureStep (Math|Integer|Clamp(Integer) _result 1 10)))))))
    (:Previous
      (bind _result_2 (Math|Integer|DecrementInt (Variables|Default|GetLectureStep))) ; Not implemented
    )))

(fn OnRepIsPossessed
  (Development|SetHiddeninGame (Variables|Default|GetInfoBox) (not (Pawn|IsLocallyControlled)) false))

(fn CheckArrow
  ;[1 1 1] Check Arrow Rotation and Disable InfoBox
  (Utilities|FlowControl|Sequence
    (:then_0
      (bind _arrow (CallFunction|GetArrow))
      (bind _return_value (Default|CheckRotation _arrow)))
    (:then_1
      (if _return_value
        (CallFunction|HideInfo)
        (else
          (CallFunction|ShowInfowithDelay 0.0))))
    (:then_2
      (return _return_value))))

(fn GetAnimation
  (return (Variables|Default|GetCurrentSequence)))

(fn GetArrow
  (return (.AsArrow%20Actor (Utilities|Casting|CastToArrowActor (Variables|/Script/Engine.ChildActorComponent|GetChildActor (Variables|Default|GetArrowActor))))))

(fn GetCamera
  (return (Variables|Default|GetCamera)))

(fn GetInfoBox
  (return (Variables|Default|GetInfoBox)))

(fn GetMotionController
  (params (ControllerHand :type ViveControllerEnum%20Enum :default "NewEnumerator0"))
  (switch Utilities|FlowControl|Switch|SwitchonViveControllerEnum ControllerHand
    (:NewEnumerator0
      (return (Variables|Default|GetL_MotionController)))
    (:NewEnumerator1
      (return (Variables|Default|GetR_ViveController)))))

(fn GetRadialMenu
  (return (Variables|Default|GetRadialMenu)))

(fn GetTechniqueType
  (return "NewEnumerator3"))

(fn GetTrackpadPosition
  (params (Controller :type ViveControllerEnum%20Enum :default "NewEnumerator0"))
  (return (Math|Vector2D|MakeVector2D (Variables|Default|GetL%20ThumbX) (Variables|Default|GetL%20ThumbY))))

(fn GetUser
  (return (Variables|Default|GetUser)))

(fn GetWorldLocation
  (return (Transformation|GetWorldLocation (Variables|Default|GetCamera))))

(fn HasTrackpad
  (return true))

(fn IsLecturer
  (return (Utilities|Enum|Equal(Enum) (.UserClass (Utilities|Struct|BreakUser (Variables|Default|GetUser))) "NewEnumerator1")))

(fn RenameCommands
  (params (OldLabel :type String) (NewLabel :type String))
  (bind _radialmenu (Utilities|GetRadialMenuWidget))
  (bind _index (Default|FindCommand _radialmenu OldLabel))
  (if (!= _index -1)
    (bind _asradial_button (Utilities|Casting|CastToRadialButton (Class|PanelWidget|GetChildat (Variables|/Game/Blueprints/UserInterface/RadialMenu.RadialMenu_C|GetCanvasContainer _radialmenu) _index))
      (:then
        (Rendering|Components|TextRender|SetText (Variables|/Game/Blueprints/UserInterface/RadialButton.RadialButton_C|GetTextBlock_Label _asradial_button) (Utilities|Text|ToText(String) NewLabel))
        (return _index))
      (:CastFailed
        _)))
  (return -1))