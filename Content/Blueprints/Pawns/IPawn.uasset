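; IPawn is a Blueprint interface for pawns in what appears to be a VR guided lecture or training experience, declaring functions with no logic.
; It exposes getters for motion controllers, trackpad input, camera, user, world location, technique type, info box, radial menu, arrow and animation.
; Other functions declare step progression, arrow and lecturer checks, delayed showing and hiding of info and advance prompts, and command renaming.
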(fn GetMotionController
  (params (ControllerHand :type ViveControllerEnum%20Enum))
  (return 0))

(fn GetTrackpadPosition
  (params (Controller :type ViveControllerEnum%20Enum))
  (return ""))

(fn HasTrackpad
  (return false))

(fn RenameCommands
  (params (OldLabel :type String) (NewLabel :type String))
  (return 0))

(fn GetUser
  (return ""))

(fn GetInfoBox
  (return 0))

(fn GetRadialMenu
  (return 0))

(fn GetTechniqueType
  (return "NewEnumerator3"))

(fn GetWorldLocation
  (return "0, 0, 0"))

(fn GetCamera
  (return 0))

(fn GetArrow
  (return 0))

(fn NextStep
  (params (Delay :type Float%20%28single-precision%29)))

(fn CurrentStep)

(fn CheckArrow
  (return false))

(fn IsLecturer
  (return false))

(fn ShowInfowithDelay
  (params (WaitDelay :type Float%20%28single-precision%29) (Clip :type Sound%20Base%20Object%20Reference)))

(fn HideInfo)

(fn HideAdvance)

(fn ShowAdvancewithDelay
  (params (WaitDelay :type Float%20%28single-precision%29)))

(fn ForceAdvance)

(fn GetAnimation
  (return 0))