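; Function library that drives step-by-step VR lectures across Selection, Manipulation, Navigation and System scenarios.
; The Next command applies the step's logic and plays its animation sequence, both chosen by scenario and single- or multi-user count; the server also replaces the current sequence.
; Scenario switches also fill info boxes and run progression checks that toggle the pawn's advance prompt.
; Helpers handle tagged-actor visibility and role-based interaction technique switching through server requests.
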(fn SetAllActorsVisibility
  (params (Visible :type Boolean) (ActorTag :type Name))
  (bind _outactors (Actor|GetAllActorswithTag 0 ActorTag))
  (for _array_element _outactors
    (Rendering|SetActorHiddenInGame _array_element (not Visible))))

(fn ExecuteVRCommand
  (params (Command :type String) (LectureStep :type Integer) (Scenario :type ScenarioEnum%20Enum) (UserCount :type Integer) (CurrentSequence :type Level%20Sequence%20Player%20Object%20Reference%20%28by%20ref%29))
  (bind _output_get (LocalVariables|SetCurrentStep LectureStep))
  (Development|PrintString 0 (Utilities|String|Append "Step: " (Utilities|String|ToString(Integer) _output_get)))
  (switch string Command
    (:Next
      (CallFunction|LectureStep Scenario (LocalVariables|GetCurrentStep) UserCount)
      (CallFunction|PlayAnimation Scenario (LocalVariables|GetCurrentStep) UserCount CurrentSequence))))

(fn SelectionStepNetwork
  (params (LectureStep :type Integer))
  (switch int LectureStep
    (:0
      (Utilities|FlowControl|Sequence
        (:then_0
          (bind _outactors (Actor|GetAllActorswithInterface 0 "/Game/Blueprints/Pawns/IPawn.IPawn_C"))
          (for _array_element _outactors
            (for _array_element_2 (Actor|GetAllChildActors _array_element true)
              (bind _asarrow_actor (Utilities|Casting|CastToArrowActor _array_element_2))
              (Rendering|SetActorHiddenInGame _asarrow_actor true))))
        (:then_2
          (bind _found_pawns (CallFunction|GetAllPawnsbyUserClass "NewEnumerator2"))
          (for _array_element_3 _found_pawns
            (bind _infobox (Default|GetInfoBox _array_element_3))
            (Development|SetHiddeninGame _infobox true false)))))
    (:1)
    (:2
      (Utilities|FlowControl|Sequence
        (:then_0
          (bind _found_pawns_2 (CallFunction|GetAllPawnsbyUserClass "NewEnumerator1"))
          (Default|ServerRequestSwitch (.AsLive%20Player%20Controller (Utilities|Casting|CastToLivePlayerController (Pawn|GetController (.AsPawn (Utilities|Casting|CastToPawn (Utilities|Array|Get(acopy) _found_pawns_2)))))) "Ray"))))
    (:5)
    (:6)
    (:8
      (if (Networking|IsServer)
        (bind _found_pawns_3 (CallFunction|GetAllPawnsbyUserClass "NewEnumerator2"))
        (for _array_element_4 _found_pawns_3
          (Default|ServerRequestSwitch (.AsLive%20Player%20Controller (Utilities|Casting|CastToLivePlayerController (Pawn|GetController (.AsPawn (Utilities|Casting|CastToPawn _array_element_4))))) "Ray"))))))

(fn SetInfoStep
  (params (Scenario :type ScenarioEnum%20Enum) (Info%20Box :type Widget%20Object%20Reference) (LectureStep :type Integer) (Pawn :type I%20Pawn%20Interface))
  (switch Utilities|FlowControl|Switch|SwitchonScenarioEnum Scenario
    (:NewEnumerator5
      (Development|PrintString 0 (Utilities|String|Append "Info Step Error! " (Utilities|String|EnumtoString Scenario) (Utilities|String|ToString(Integer) LectureStep))))
    (:NewEnumerator1
      (CallFunction|SetSelectionInfoStep Info%20Box LectureStep Pawn))
    (:NewEnumerator3
      (CallFunction|SetManipulationInfoStep Info%20Box LectureStep Pawn))
    (:NewEnumerator4
      (CallFunction|SetNavigationInfoStep Info%20Box LectureStep Pawn))
    (:NewEnumerator6
      (CallFunction|SetSystemInfoStep Info%20Box LectureStep Pawn))))

(fn LectureStep
  (params (Scenario :type ScenarioEnum%20Enum) (Step :type Integer) (NumUsers :type Integer))
  (if (== NumUsers 1)
    (switch Utilities|FlowControl|Switch|SwitchonScenarioEnum Scenario
      (:NewEnumerator1
        (CallFunction|SelectionStepLocal Step))
      (:NewEnumerator3
        (CallFunction|ManipulationLocal Step))
      (:NewEnumerator4
        (CallFunction|NavigationLocal Step))
      (:NewEnumerator6
        (CallFunction|SystemStepLocal Step)))
    (else
      (switch Utilities|FlowControl|Switch|SwitchonScenarioEnum Scenario
        (:NewEnumerator1
          (CallFunction|SelectionStepMulti Step))
        (:NewEnumerator3
          (CallFunction|ManipulationMulti Step))
        (:NewEnumerator4
          (CallFunction|NavigationMulti Step))
        (:NewEnumerator6
          (CallFunction|SystemStepMulti Step))))))

(fn CreateAnimationStep
  (params (Scenario :type ScenarioEnum%20Enum) (Step :type Integer) (UserCount :type Integer))
  (if (== UserCount 1)
    (switch Utilities|FlowControl|Switch|SwitchonScenarioEnum Scenario
      (:NewEnumerator1
        (bind _sequencer (CallFunction|CreateSelectionAnimationStep Step))
        (return _sequencer))
      (:NewEnumerator3
        (bind _sequencer_2 (CallFunction|CreateManipulationAnimationStep Step))
        (return _sequencer_2))
      (:NewEnumerator4
        (bind _sequencer_3 (CallFunction|CreateNavigationAnimationStep Step))
        (return _sequencer_3))
      (:NewEnumerator6
        (bind _sequencer_4 (CallFunction|CreateSystemAnimationStep Step))
        (return _sequencer_4)))
    (else
      (switch Utilities|FlowControl|Switch|SwitchonScenarioEnum Scenario
        (:NewEnumerator1
          (bind _sequencer_5 (CallFunction|CreateSelectionAnimationMulti Step))
          (return _sequencer_5))
        (:NewEnumerator3
          (bind _sequencer_6 (CallFunction|CreateManipulationAnimationMulti Step))
          (return _sequencer_6))
        (:NewEnumerator4
          (bind _sequencer_7 (CallFunction|CreateNavigationAnimationMulti Step))
          (return _sequencer_7))
        (:NewEnumerator6
          (bind _sequencer_8 (CallFunction|CreateSystemAnimationStepMulti Step))
          (return _sequencer_8))))))

(fn GetPlayerController
  (params (UserClass :type UserClassEnum%20Enum))
  (bind _found_pawns (CallFunction|GetAllPawnsbyUserClass UserClass))
  (for _array_element _found_pawns
    (bind _user (Default|GetUser _array_element))
    (Development|PrintString 0 (Utilities|String|EnumtoString (.UserClass (Utilities|Struct|BreakUser _user))))
    (return (.AsLive%20Player%20Controller (Utilities|Casting|CastToLivePlayerController (Pawn|GetController (.AsPawn (Utilities|Casting|CastToPawn (Utilities|Array|Get(acopy) _found_pawns)))))))))

(fn CheckProgression
  (params (Scenario :type ScenarioEnum%20Enum) (Step :type Integer) (Pawn :type I%20Pawn%20Interface))
  (Utilities|FlowControl|Sequence
    (:then_0
      (switch Utilities|FlowControl|Switch|SwitchonScenarioEnum Scenario
        (:NewEnumerator1
          (bind (_returnvalue _waitdelay) (CallFunction|SelectionCheck Step Pawn))
          (LocalVariables|SetCanProgress _returnvalue)
          (LocalVariables|SetWaitDelay _waitdelay))
        (:NewEnumerator3
          (bind (_returnvalue_2 _waitdelay_2) (CallFunction|ManipulationCheck Step Pawn))
          (LocalVariables|SetCanProgress _returnvalue_2)
          (LocalVariables|SetWaitDelay _waitdelay_2))
        (:NewEnumerator4
          (bind (_returnvalue_3 _waitdelay_3) (CallFunction|NavigationCheck Step Pawn))
          (LocalVariables|SetCanProgress _returnvalue_3)
          (LocalVariables|SetWaitDelay _waitdelay_3))
        (:NewEnumerator6
          (bind (_returnvalue_4 _waitdelay_4) (CallFunction|SystemCheck Step Pawn))
          (LocalVariables|SetCanProgress _returnvalue_4)
          (LocalVariables|SetWaitDelay _waitdelay_4))))
    (:then_1
      (if (LocalVariables|GetCanProgress)
        (Default|ShowAdvancewithDelay Pawn (LocalVariables|GetWaitDelay))
        (else
          (Default|HideAdvance Pawn))))
    (:then_2
      (return (LocalVariables|GetCanProgress)))))

(fn PlayAnimation
  (params (Scenario :type ScenarioEnum%20Enum) (Step :type Integer) (UserCount :type Integer) (CurrentSequence :type Level%20Sequence%20Player%20Object%20Reference%20%28by%20ref%29))
  (bind _sequence_player (CallFunction|CreateAnimationStep Scenario Step UserCount))
  (Utilities|IsValid _sequence_player
    (:Is%20Valid
      (if (Networking|IsServer)
        (Sequencer|Player|Stop CurrentSequence :!class /Script/MovieScene.MovieSceneSequencePlayer)
        (|SetBy-RefVar CurrentSequence _sequence_player))
      (Audio|Components|Audio|Play _sequence_player))))

(fn SwitchTechniqueifRole
  (params (Technique :type String) (UserClass :type UserClassEnum%20Enum))
  (bind _returnvalue (Game|GetPlayerController 0))
  (bind _aslive_player_controller (Utilities|Casting|CastToLivePlayerController _returnvalue))
  (bind _user (Default|GetUser (.AsIPawn (Utilities|Casting|CastToIPawn (Pawn|GetControlledPawn _returnvalue)))))
  (if (Utilities|Enum|Equal(Enum) (.UserClass (Utilities|Struct|BreakUser _user)) UserClass)
    (Default|ServerRequestSwitch _aslive_player_controller Technique)))