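; LiveInstance is a game instance that handles hosting, joining and leaving multiplayer games, plus menu, lobby and loading-screen widgets.
; Host and join run "open" console commands for a listen-server lobby or direct IP, then pass the user to LobbyPlayerController.SessionJoined.
; Joining polls until that controller exists, then stores the user ID.
; Logoff destroys the session, helpers print logs and network errors, and session-based create/join paths are disconnected.
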(event Custom|ShowMainMenu
  ;[1 1 1] UI
  (bind _widget_out (CallFunction|CreateorAddWidgettoViewport (Variables|Widgets|GetStartScreen) "/Game/Blueprints/UserInterface/Network/StartScreen.StartScreen_C"))
  (Variables|Widgets|SetStartScreen _widget_out))

(event Custom|Join%20Server
  (params (User :type User%20Structure) (IP%20Address :type String))
  ;[1 1 1] Join Server Direct IP
  (CallFunction|ShowLoadingScreen)
  (Development|ExecuteConsoleCommand (Utilities|String|Append "open " IP%20Address))
  (bind _aslobby_player_controller (Utilities|Casting|CastToLobbyPlayerController (Game|GetPlayerController 0) :!label _label)
    (:then
      (Default|SessionJoined _aslobby_player_controller User)
      (Variables|Default|SetPersistentUserId (.Id (Utilities|Struct|BreakUser User))))
    (:CastFailed
      (CallFunction|LogMessage "Join" "Waiting...")
      (Utilities|FlowControl|Delay 0.3)
      (goto _label))))

(event Custom|HostServer
  (params (User :type User%20Structure))
  ;[1 1 1] Host Server
  (CallFunction|ShowLoadingScreen)
  (Development|ExecuteConsoleCommand "open  lobby?listen")
  (Utilities|FlowControl|Delay 0.01)
  (Default|SessionJoined (.AsLobby%20Player%20Controller (Utilities|Casting|CastToLobbyPlayerController (Game|GetPlayerController 0))) User))

(event Custom|Logoff
  (|DestroySession (Game|GetPlayerController 0)
    (:OnSuccess
      (CallFunction|LogMessage "LIVE" "Session destroyed."))
    (:OnFailure
      (CallFunction|LogMessage "LIVE" "Failed to destroy session."))))

(event Custom|ShowLoadingScreen
  ;[1 1 1] UI
  (bind _widget_out (CallFunction|CreateorAddWidgettoViewport (Variables|Widgets|GetLoadingScreen) "/Game/Blueprints/UserInterface/LoadingScreen.LoadingScreen_C"))
  (Variables|Widgets|SetLoadingScreen _widget_out))

(event Custom|ShowMiniLobby
  ;[1 1 1] UI
  (bind _widget_out (CallFunction|CreateorAddWidgettoViewport (Variables|Widgets|GetMiniLobby) "/Game/Blueprints/UserInterface/Network/MiniLobby.MiniLobby_C"))
  (Variables|Widgets|SetMiniLobby (.AsMini%20Lobby (Utilities|Casting|CastToMiniLobby _widget_out))))

(event EventHandleNetworkError
  (params (FailureType :type ENetworkFailure%20Enum :default "NetDriverAlreadyExists") (bIsServer :type Boolean))
  (CallFunction|LogMessage "" (Utilities|Text|ToText(String) (CallFunction|NetworkErrortoString FailureType))))

(event EventShutdown)

(fn NetworkErrortoString
  (params (FailureType :type ENetworkFailure%20Enum))
  (return (Utilities|String|ToString(Text) (Utilities|Text|FormatText "[NetworkError] {0}" (Utilities|Text|ToText(String) (Utilities|String|EnumtoString FailureType))))))

(fn LogMessage
  (params (Caller :type Text) (LogEntry :type Text))
  (Development|PrintText (Utilities|Text|FormatText "[LIVE]->{0} {1}" Caller LogEntry) true true "(R=0.000000,G=0.660000,B=1.000000,A=1.000000)" 4.0))

(fn UserInfotoString
  (params (User :type User%20Structure))
  (bind (_id _name _vrenabled _userclass) (Utilities|Struct|BreakUser User))
  (return (Utilities|Text|FormatText "{0} [{1}({2})]" (Utilities|Text|ToText(String) (Utilities|String|EnumtoString _userclass)) (Utilities|Text|ToText(String) _name) _id)))

(fn CreateorAddWidgettoViewport
  (params (Widget%20In :type User%20Widget%20Object%20Reference) (Widget%20Class :type User%20Widget%20Class%20Reference))
  (Utilities|IsValid Widget%20In
    (:Is%20Valid
      (LocalVariables|SetNew%20Widget Widget%20In))
    (:Is%20Not%20Valid
      (bind _returnvalue (UserInterface|CreateWidget Widget%20Class (Game|GetPlayerController 0)))
      (LocalVariables|SetNew%20Widget _returnvalue)))
  (UserInterface|Viewport|AddtoViewport (LocalVariables|GetNew%20Widget) 0)
  (return (LocalVariables|GetNew%20Widget)))

(fn UserCount
  (return (Utilities|Array|Length (Variables|Default|GetPersistentUserData))))